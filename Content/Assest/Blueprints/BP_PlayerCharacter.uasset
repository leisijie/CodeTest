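; Player character Blueprint that rides an attached car, spawned on BeginPlay, and can swap it for an enemy's car.
; Each tick it draws three laser beams around the aim position using a downward trace, and box-scans (with debug drawing) for enemy cars to store as Target.
; ChangeCar detaches the enemy and destroys the current car, then a timeline lerps the player to the new seat before attaching that car.
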(event `self.ReceiveBeginPlay`
  (`self.SpawnDefaultCar`))

(event `self.ReceiveTick`
  (params (DeltaSeconds :type "Float (single-precision)"))
  (`self.RotateAimLine`)
  (`self.FindCar` 0.0))

(event `BeginChangeCar`
  (bind _car (`self.Car`))
  (bind (_direction _newtrack_0) (`Timeline|ChanegCarTimeline` :!via `PlayFromStart`)
    (:`Update`
      (`self.K2_SetActorLocation` (`KismetMathLibrary.VLerp` (`self.K2_GetActorLocation`) (`SceneComponent.K2_GetComponentLocation` (`/Game/Assest/Blueprints/BP_Car.Seat` _car)) _newtrack_0)))
    (:`Finished`
      (`self.K2_AttachToActor` _car self "None" "KeepWorld" "KeepWorld" "KeepWorld" true))))

(fn `ChangeCar`
  (params (NewCar :type "/Game/Assest/Blueprints/BP_Car Object Reference"))
  (`/Engine/EditorBlueprintResources/StandardMacros.IsValid` NewCar
    (:`Is Valid`
      (bind _asbp_enemy (cast `/Game/Assest/Blueprints/BP_Enemy` (`self.GetAttachParentActor` NewCar))
        (:`then`
          (`self.K2_DetachFromActor` _asbp_enemy "KeepWorld" "KeepWorld" "KeepWorld")
          (`self.K2_DestroyActor` (`self.Car`))
          (set `self.Car` NewCar)
          (`self.BeginChangeCar`))
        (:`CastFailed`
          (`KismetSystemLibrary.PrintString` "Hello"))))))

(fn `FindCar`
  (params (Degree :type "Float (double-precision)"))
  (bind _boxextent (`self.BoxExtent`))
  (bind _returnvalue (+ (`self.BoxPos`) (`self.K2_GetActorLocation`)))
  (`KismetSystemLibrary.DrawDebugBox` _returnvalue (/ _boxextent 2.0) (struct :`R` 1.0 :`A` 1.0) (struct) 0.0 10.0)
  (bind (_outactors _returnvalue_2) (`KismetSystemLibrary.BoxOverlapActors` _returnvalue _boxextent (`|MakeArray` "ObjectTypeQuery7" :!type "EObjectTypeQuery Enum")))
  (if _returnvalue_2
    (for _array_element _outactors
      (bind _asbp_enemy (cast `/Game/Assest/Blueprints/BP_Enemy` _array_element))
      (set `self.Target` (`/Game/Assest/Blueprints/BP_Enemy.Car` _asbp_enemy)))))

(fn `RotateAimLine`
  (bind _laserbeam (`self.LaserBeam`))
  (bind _aimposition (`self.AimPosition`))
  (bind _laserbeamdown (`self.LaserBeamDown`))
  (bind _laserbeamground (`self.LaserBeamGround`))
  (bind _x (.x _aimposition))
  (bind _y (.y _aimposition))
  (`ParticleSystemComponent.SetBeamSourcePoint` _laserbeam 0 (`KismetMathLibrary.MakeVector` (.x (`self.K2_GetActorLocation`)) (.y (`self.K2_GetActorLocation`))) 0)
  (`ParticleSystemComponent.SetBeamTargetPoint` _laserbeam 0 (`KismetMathLibrary.MakeVector` (.x _aimposition) (.y _aimposition)) 0)
  (bind _outhit (`KismetSystemLibrary.LineTraceSingle` (`KismetMathLibrary.MakeVector` _x _y 500.0) (`KismetMathLibrary.MakeVector` _x _y -500.0) "TraceTypeQuery1"))
  (`ParticleSystemComponent.SetBeamSourcePoint` _laserbeamdown 0 _aimposition 0)
  (bind (_bblockinghit _binitialoverlap _time _distance _location _impactpoint) (`GameplayStatics.BreakHitResult` _outhit))
  (`ParticleSystemComponent.SetBeamTargetPoint` _laserbeamdown 0 _impactpoint 0)
  (`ParticleSystemComponent.SetBeamSourcePoint` _laserbeamground 0 (+ (0.0 -100.0 10.0) _impactpoint) 0)
  (`ParticleSystemComponent.SetBeamTargetPoint` _laserbeamground 0 (+ (0.0 100.0 10.0) _impactpoint) 0))

(fn `SpawnDefaultCar`
  (bind _returnvalue (`|SpawnActorFromClass` (`self.DefaultCar`) (`KismetMathLibrary.MakeTransform` (0.0 0.0 0.0)) "Undefined" "OverrideRootScale" self null))
  (bind _output_get (set `self.Car` _returnvalue))
  (`self.K2_AttachToActor` _output_get self "None" "KeepRelative" "KeepRelative" "KeepRelative" true)
  (`self.K2_SetActorRelativeLocation` _output_get (`KismetMathLibrary.NegateVector` (`SceneComponent.RelativeLocation` (`/Game/Assest/Blueprints/BP_Car.Seat` _output_get))) false false))

(fn `UserConstructionScript`)