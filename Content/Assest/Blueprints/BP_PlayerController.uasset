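; Player controller for a car-hopping shooter that moves the player character, aims and fires its gun, and triggers car changes.
; Tick offsets the character by axis input scaled by the current car's speed, without sweep.
; Normally it sets AimPosition by projecting the mouse ray onto the X-normal plane through the pawn.
; Holding Prepare instead feeds the mouse's angle around screen center to FindCar, and Jump then changes to the target car.
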(event `self.ReceiveBeginPlay`
  (bind _asbp_player_character (cast `/Game/Assest/Blueprints/BP_PlayerCharacter` (`GameplayStatics.GetPlayerPawn` 0)))
  (bind _output_get (set `self.MainCharacter` _asbp_player_character))
  (set `self.PlayerGun` (`self.GetComponentByClass` _output_get "/Game/Assest/Blueprints/BP_Gun.BP_Gun_C")))

(event `self.ReceiveTick`
  (params (DeltaSeconds :type "Float (single-precision)"))
  (`self.CharacterMove`)
  (if (`self.PrepareToChangeCar`)
    (`self.AimCar`)
    (else
      (`self.GunAim`))))

(event `InputAction|Jump`
  (params (Key :type "Key Structure"))
  (bind _maincharacter (`self.MainCharacter`))
  (:`Pressed`
    (if (`self.PrepareToChangeCar`)
      (`/Game/Assest/Blueprints/BP_PlayerCharacter.ChangeCar` _maincharacter (`/Game/Assest/Blueprints/BP_PlayerCharacter.Target` _maincharacter)))))

(event `InputAction|Prepare`
  (params (Key :type "Key Structure"))
  (:`Pressed`
    (set `self.PrepareToChangeCar` true))
  (:`Released`
    (set `self.PrepareToChangeCar` false)))

(event `InputAction|Fire`
  (params (Key :type "Key Structure"))
  (:`Pressed`
    (`/Game/Assest/Blueprints/BP_Gun.Fire` (`self.PlayerGun`))))

(event `InputAxis|Vertical`
  (params (AxisValue :type "Float (single-precision)"))
  (set `self.MoveVector` (`KismetMathLibrary.MakeVector2D` AxisValue (`.Y` (`KismetMathLibrary.BreakVector2D` (`self.MoveVector`))))))

(event `InputAxis|Horizontal`
  (params (AxisValue :type "Float (single-precision)"))
  (set `self.MoveVector` (`KismetMathLibrary.MakeVector2D` (`KismetMathLibrary.BreakVector2D` (`self.MoveVector`)) AxisValue)))

(fn `AimCar`
  (bind (_locationx _locationy) (`WidgetLayoutLibrary.GetMousePositionScaledByDPI` self))
  (bind _returnvalue (`KismetMathLibrary.Normal2D` (- (/ (`WidgetLayoutLibrary.GetViewportSize`) 2.0) (* (`KismetMathLibrary.MakeVector2D` _locationx _locationy) (`WidgetLayoutLibrary.GetViewportScale`)))))
  (bind _asbp_player_character (cast `/Game/Assest/Blueprints/BP_PlayerCharacter` (`GameplayStatics.GetPlayerPawn` 0)))
  (`/Game/Assest/Blueprints/BP_PlayerCharacter.FindCar` _asbp_player_character (+ (* (`KismetMathLibrary.DegAcos` (`KismetMathLibrary.DotProduct2D` (1.0 0.0) _returnvalue)) (`KismetMathLibrary.SignOfFloat` (`.Y` (`KismetMathLibrary.BreakVector2D` _returnvalue)))) 180.0)))

(fn `CharacterMove`
  (bind _asbp_player_character (cast `/Game/Assest/Blueprints/BP_PlayerCharacter` (`GameplayStatics.GetPlayerPawn` 0)))
  (`self.K2_AddActorWorldOffset` _asbp_player_character (* (`KismetMathLibrary.Conv_Vector2DToVector` (* (`self.MoveVector`) (`/Game/Assest/Blueprints/BP_Car.Speed` (`/Game/Assest/Blueprints/BP_PlayerCharacter.Car` _asbp_player_character)))) (`GameplayStatics.GetWorldDeltaSeconds`)) false false))

(fn `GunAim`
  (bind (_worldlocation _worlddirection) (`self.DeprojectMousePositionToWorld` self))
  (set `/Game/Assest/Blueprints/BP_PlayerCharacter.AimPosition` (+ _worldlocation (* _worlddirection (/ (`KismetMathLibrary.Dot_VectorVector` (- (`self.K2_GetActorLocation` (`self.K2_GetPawn` self)) (`PlayerCameraManager.GetCameraLocation` (`GameplayStatics.GetPlayerCameraManager` 0))) (1.0 0.0 0.0)) (`KismetMathLibrary.Dot_VectorVector` _worlddirection (1.0 0.0 0.0))))) (`self.MainCharacter`)))

(fn `UserConstructionScript`)