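; Building_A is a building actor that gets a brief physics-driven push when spawned and removes itself on contact with tagged objects.
; On BeginPlay it sets its static mesh's linear velocity from the Velocity variable, then zeroes it after a short delay.
; Overlapping an actor whose root component carries the "BYE" tag destroys the building after a delay.
; A Timeline that would move it by local offsets is unconnected and never runs.
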(event `self.ReceiveBeginPlay`
  (`PrimitiveComponent.SetPhysicsLinearVelocity` (`self.StaticMesh`) (`self.velocity`) false "None")
  (`KismetSystemLibrary.Delay` 2.0)
  (`PrimitiveComponent.SetPhysicsLinearVelocity` (`self.StaticMesh`) (0.0 0.0 0.0) false "None"))

(event `self.ReceiveActorBeginOverlap`
  (params (OtherActor :type "Actor Object Reference"))
  (if (`ActorComponent.ComponentHasTag` (`Actor.RootComponent` OtherActor) "BYE")
    (`KismetSystemLibrary.Delay` 1.0)
    (`self.K2_DestroyActor`)))

(fn `UserConstructionScript`)