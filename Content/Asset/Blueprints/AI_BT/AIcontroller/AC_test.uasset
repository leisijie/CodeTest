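; AC_test is a shared AI controller that picks a behavior tree for whichever enemy pawn it possesses.
; On possess, a Sequence tries a cast for each supported enemy class and runs that class's tree on a match.
; Some types share trees: BP_Enemy2 and BP_Enemy_Throw use BT_test, while BP_Enemy_Bomber and BP_Enemyshoot use BT_Enemy_Bomber.
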(event `self.ReceivePossess`
  (params (PossessedPawn :type "Pawn Object Reference"))
  (`|ExecutionSequence`
    (:`then_0`
      (cast `/Game/Asset/Blueprints/Enemy/BP_Enemy2` PossessedPawn)
      (`self.RunBehaviorTree` "/Game/Asset/Blueprints/AI_BT/BehaviorTreeAndBlackboard/BT_test.BT_test"))
    (:`then_1`
      (cast `/Game/Asset/Blueprints/Enemy/BP_Enemy3` PossessedPawn)
      (`self.RunBehaviorTree` "/Game/Asset/Blueprints/AI_BT/BehaviorTreeAndBlackboard/BT_Enemy3.BT_Enemy3"))
    (:`then_2`
      (cast `/Game/Asset/Blueprints/Enemy/BP_Enemy_Bomber` PossessedPawn)
      (`self.RunBehaviorTree` "/Game/Asset/Blueprints/AI_BT/BehaviorTreeAndBlackboard/BT_Enemy_Bomber.BT_Enemy_Bomber"))
    (:`then_3`
      (cast `/Game/Asset/Blueprints/Enemy/BP_Enemyshoot` PossessedPawn)
      (`self.RunBehaviorTree` "/Game/Asset/Blueprints/AI_BT/BehaviorTreeAndBlackboard/BT_Enemy_Bomber.BT_Enemy_Bomber"))
    (:`then_4`
      (cast `/Game/Asset/Blueprints/Enemy/BP_Enemy_Throw` PossessedPawn)
      (`self.RunBehaviorTree` "/Game/Asset/Blueprints/AI_BT/BehaviorTreeAndBlackboard/BT_test.BT_test"))
    (:`then_5`
      (cast `/Game/Asset/Blueprints/Enemy/BP_ShotGun` PossessedPawn)
      (`self.RunBehaviorTree` "/Game/Asset/Blueprints/AI_BT/BehaviorTreeAndBlackboard/BT_ShotGunAtk.BT_ShotGunAtk"))
    (:`then_6`
      (cast `/Game/Asset/Blueprints/Enemy/BP_MeleeEnemy` PossessedPawn)
      (`self.RunBehaviorTree` "/Game/Asset/Blueprints/AI_BT/BehaviorTreeAndBlackboard/BT_EnemyMeele.BT_EnemyMeele"))
    (:`then_7`
      (cast `/Game/Asset/Blueprints/Enemy/BP_EnemyRandom` PossessedPawn)
      (`self.RunBehaviorTree` "/Game/Asset/Blueprints/AI_BT/BehaviorTreeAndBlackboard/BP_Enemy_Random.BP_Enemy_Random"))
    (:`then_8`
      (cast `/Game/Asset/Blueprints/Enemy/BP_BombEnemy` PossessedPawn)
      (`self.RunBehaviorTree` "/Game/Asset/Blueprints/AI_BT/BehaviorTreeAndBlackboard/BT_Base.BT_Base"))))

(event `self.ReceiveTick`
  (params (DeltaSeconds :type "Float (single-precision)")))

(fn `UserConstructionScript`)