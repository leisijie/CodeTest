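; Behavior tree task that makes a BT_Enemy wander around its BeginLocation within MoveRadius.
; On execute it picks a random horizontal point in the outer band of that radius, though direction and travel length each evaluate their own random roll.
; Each tick drives the enemy's Car along that direction at its Speed, and a Delay of length over speed finishes the task successfully.
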(event `self.ReceiveExecuteAI`
  (params (OwnerController :type "AIController Object Reference") (ControlledPawn :type "Pawn Object Reference"))
  (bind _asbt_enemy (cast `/Game/Asset/Blueprints/AI_BT/BT_Enemy` ControlledPawn))
  (bind _returnvalue (- (+ (`/Game/Asset/Blueprints/Enemy/BP_Enemy.BeginLocation` _asbt_enemy) (* (* (`KismetMathLibrary.Conv_Vector2DToVector` (`KismetMathLibrary.Normal2D` (`KismetMathLibrary.Conv_VectorToVector2D` (`KismetMathLibrary.RandomUnitVector`)))) (+ (* (`KismetMathLibrary.RandomFloat`) 0.3) 0.7)) (`/Game/Asset/Blueprints/Enemy/BP_Enemy.MoveRadius` _asbt_enemy))) (`Actor.K2_GetActorLocation` _asbt_enemy)))
  (set `self.targetDir` (`KismetMathLibrary.Normal` _returnvalue))
  (set `self.length` (`KismetMathLibrary.VSize` _returnvalue)))

(event `self.ReceiveTickAI`
  (params (OwnerController :type "AIController Object Reference") (ControlledPawn :type "Pawn Object Reference") (DeltaSeconds :type "Float (single-precision)"))
  (bind _asbt_enemy (cast `/Game/Asset/Blueprints/AI_BT/BT_Enemy` ControlledPawn))
  (bind _speed (`/Game/Asset/Blueprints/Enemy/BP_Enemy.Speed` _asbt_enemy))
  (`/Game/Asset/Blueprints/Car/BP_Car.Drive` (`/Game/Asset/Blueprints/Enemy/BP_Enemy.Car` _asbt_enemy) (`KismetMathLibrary.Conv_VectorToVector2D` (* (`self.targetDir`) (* _speed DeltaSeconds))))
  (`KismetSystemLibrary.Delay` (/ (`self.length`) _speed))
  (`self.FinishExecute` true))

(event `self.ReceiveExecute`
  (params (OwnerActor :type "Actor Object Reference")))

(event `self.ReceiveAbort`
  (params (OwnerActor :type "Actor Object Reference")))