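; Behavior tree task that makes a BT_Enemy car flee to the map quadrant diagonally opposite the player.
; On execute it moves BeginLocation there from the player's coordinate signs, then derives direction and distance from separately rolled random points around it within MoveRadius.
; Each tick drives the Car at triple Speed along that direction, with a Delay of the estimated travel time before finishing as failed.
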(event `self.ReceiveExecuteAI`
  (params (OwnerController :type "AIController Object Reference") (ControlledPawn :type "Pawn Object Reference"))
  (bind _x (.x (`Actor.K2_GetActorLocation` (`GameplayStatics.GetPlayerPawn` 0))))
  (bind _y (.y (`Actor.K2_GetActorLocation` (`GameplayStatics.GetPlayerPawn` 0))))
  (bind _asbt_enemy (cast `/Game/Asset/Blueprints/AI_BT/BT_Enemy` ControlledPawn))
  (set `/Game/Asset/Blueprints/Enemy/BP_Enemy.BeginLocation` (`KismetMathLibrary.Conv_Vector2DToVector` (* (`KismetMathLibrary.MakeVector2D` (/ _x (`KismetMathLibrary.Abs` _x)) (/ _y (`KismetMathLibrary.Abs` _y))) (-750.0 -1500.0))) _asbt_enemy)
  (bind _returnvalue (- (+ (`/Game/Asset/Blueprints/Enemy/BP_Enemy.BeginLocation` _asbt_enemy) (* (* (`KismetMathLibrary.Conv_Vector2DToVector` (`KismetMathLibrary.Normal2D` (`KismetMathLibrary.Conv_VectorToVector2D` (`KismetMathLibrary.RandomUnitVector`)))) (+ (* (`KismetMathLibrary.RandomFloat`) 0.3) 0.7)) (`/Game/Asset/Blueprints/Enemy/BP_Enemy.MoveRadius` _asbt_enemy))) (`Actor.K2_GetActorLocation` _asbt_enemy)))
  (set `self.targetDir` (`KismetMathLibrary.Normal` _returnvalue))
  (set `self.length` (`KismetMathLibrary.VSize` _returnvalue)))

(event `self.ReceiveTickAI`
  (params (OwnerController :type "AIController Object Reference") (ControlledPawn :type "Pawn Object Reference") (DeltaSeconds :type "Float (single-precision)"))
  (bind _asbt_enemy (cast `/Game/Asset/Blueprints/AI_BT/BT_Enemy` ControlledPawn))
  (bind _returnvalue (* (`/Game/Asset/Blueprints/Enemy/BP_Enemy.Speed` _asbt_enemy) 3.0))
  (`/Game/Asset/Blueprints/Car/BP_Car.Drive` (`/Game/Asset/Blueprints/Enemy/BP_Enemy.Car` _asbt_enemy) (`KismetMathLibrary.Conv_VectorToVector2D` (* (`self.targetDir`) (* _returnvalue DeltaSeconds))))
  (`KismetSystemLibrary.Delay` (/ (`self.length`) _returnvalue))
  (`self.FinishExecute` false))

(event `self.ReceiveExecute`
  (params (OwnerActor :type "Actor Object Reference")))