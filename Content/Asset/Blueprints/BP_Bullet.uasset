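; Projectile actor that flies in a straight line and destroys itself when it overlaps a BP_Enemy or runs out of range.
; BeginPlay faces it along ForwardVector, then Tick moves it by Speed without sweeping and accumulates Distance until MaxDistance.
; Overlaps go to HitEnemy, which destroys only the bullet on an enemy cast, applying no damage, and prints the name of any other actor.
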(event `self.ReceiveBeginPlay`
  (`self.K2_SetActorRotation` (`KismetMathLibrary.Conv_VectorToRotator` (`self.ForwardVector`))))

(event `self.ReceiveActorBeginOverlap`
  (params (OtherActor :type "Actor Object Reference"))
  (`|ExecutionSequence`
    (:`then_0`
      (`self.HitEnemy` OtherActor))))

(event `self.ReceiveTick`
  (params (DeltaSeconds :type "Float (single-precision)"))
  (bind _returnvalue (* (`GameplayStatics.GetWorldDeltaSeconds`) (`self.Speed`)))
  (bind _output_get (set `self.Distance` (+ _returnvalue (`self.Distance`))))
  (if (> (`self.MaxDistance`) _output_get)
    (`self.K2_SetActorLocation` (+ (* (`self.ForwardVector`) _returnvalue) (`self.K2_GetActorLocation`)))
    (else
      (`self.K2_DestroyActor`))))

(fn `HitEnemy`
  (params (Actor :type "Actor Object Reference"))
  (cast `/Game/Asset/Blueprints/BP_Enemy` Actor
    (:`then`
      (`self.K2_DestroyActor`))
    (:`CastFailed`
      (`KismetSystemLibrary.PrintString` (`KismetSystemLibrary.GetObjectName` Actor)))))

(fn `UserConstructionScript`)