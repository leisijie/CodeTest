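; Player bullet projectile that flies along its forward vector at a set speed and damages enemy drivers of cars.
; BeginPlay sets the particle template and the Box physics velocity, and Tick destroys the bullet once its accumulated distance exceeds the maximum.
; Hit branches on the other actor's first tag: Enemy and Car resolve a BP_Car's driver to apply damage, then spawn an electrical impact.
; Any other hit just destroys the bullet.
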(event `self.ReceiveBeginPlay`
  (`ParticleSystemComponent.SetTemplate` (`self.ParticleSystem`) (`self.ParticleSys`))
  (`self.K2_SetActorRotation` (`KismetMathLibrary.Conv_VectorToRotator` (`self.ForwardVector`)))
  (`PrimitiveComponent.SetPhysicsLinearVelocity` (`self.Box`) (* (`self.ForwardVector`) (`self.Speed`)) false "None"))

(event `self.ReceiveHit`
  (params (MyComp :type "PrimitiveComponent Object Reference") (Other :type "Actor Object Reference") (OtherComp :type "PrimitiveComponent Object Reference") (bSelfMoved :type Boolean) (HitLocation :type "Vector Structure") (HitNormal :type "Vector Structure") (NormalImpulse :type "Vector Structure") (Hit :type "HitResult Structure (by ref)"))
  (bind _tags (`Actor.Tags` Other))
  (if (`KismetArrayLibrary.Array_IsValidIndex` _tags)
    (switch `name` (`|GetArrayItem` _tags)
      (:`Default`
        (`self.HitObstacle` :!label _label))
      (:`Enemy`
        (`self.HitEnemy` Other)
        (`GameplayStatics.SpawnEmitterAtLocation` "/Game/BallisticsVFX/Particles/Impacts/LegacyFX/Small-Medium-Large/Electrical/Electrical_impact_med.Electrical_impact_med" HitLocation :!label _label_2))
      (:`Car`
        (`self.HitEnemyCar` Other)
        (goto _label_2))
      (:`Obstacle`
        (goto _label)))
    (else
      (`self.HitObstacle`))))

(event `self.ReceiveTick`
  (params (DeltaSeconds :type "Float (single-precision)"))
  (bind _output_get (set `self.Distance` (+ (* DeltaSeconds (`self.Speed`)) (`self.Distance`))))
  (if (> _output_get (`self.MaxDistance`))
    (`self.K2_DestroyActor`)))

(fn `HitEnemy`
  (params (Actor :type "Actor Object Reference"))
  (bind _asbp_car (cast `/Game/Asset/Blueprints/Car/BP_Car` Actor))
  (bind _asbp_enemy (cast `/Game/Asset/Blueprints/Character/BP_Enemy` (`/Game/Asset/Blueprints/Car/BP_Car.Driver` _asbp_car)))
  (`/Game/Asset/Blueprints/Character/BP_Enemy.BeHit` _asbp_enemy (`self.Damage`))
  (`self.K2_DestroyActor`))

(fn `HitEnemyCar`
  (params (Car :type "Actor Object Reference"))
  (bind _asbp_car (cast `/Game/Asset/Blueprints/Car/BP_Car` Car))
  (`self.HitEnemy` (`self.GetAttachParentActor` _asbp_car)))

(fn `HitObstacle`
  (`self.K2_DestroyActor`))

(fn `UserConstructionScript`)