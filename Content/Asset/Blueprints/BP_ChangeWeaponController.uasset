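; BP_ChangeWeaponController is an input controller that drives the weapon change menu from the keyboard.
; The W, S, A and D keys each call Turn on MainWeaponMenu with a different direction enum value.
; Enter calls Select on the same menu to confirm the choice, and the Blueprint holds no other logic.
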(event `Key|W`
  (params (Key :type "Key Structure"))
  (:`Pressed`
    (`/Game/Asset/Widget/WeaponMenu.Turn` (`self.MainWeaponMenu`) "NewEnumerator0")))

(event `Key|S`
  (params (Key :type "Key Structure"))
  (:`Pressed`
    (`/Game/Asset/Widget/WeaponMenu.Turn` (`self.MainWeaponMenu`) "NewEnumerator1")))

(event `Key|A`
  (params (Key :type "Key Structure"))
  (:`Pressed`
    (`/Game/Asset/Widget/WeaponMenu.Turn` (`self.MainWeaponMenu`) "NewEnumerator2")))

(event `Key|D`
  (params (Key :type "Key Structure"))
  (:`Pressed`
    (`/Game/Asset/Widget/WeaponMenu.Turn` (`self.MainWeaponMenu`) "NewEnumerator3")))

(event `Key|Enter`
  (params (Key :type "Key Structure"))
  (:`Pressed`
    (`/Game/Asset/Widget/WeaponMenu.Select` (`self.MainWeaponMenu`))))

(fn `UserConstructionScript`)