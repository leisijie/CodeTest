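; Game state Blueprint that spawns the game's path actors and answers movement queries along their splines.
; On BeginPlay it spawns each path class listed in PathTable and stores its spline in a map keyed by class display name.
; CalculateDeltaLocation returns the world offset over a distance step, wrapping by spline length to loop.
; It also outputs a speed percent from the dot product of nearby tangents, which drops on bends.
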(event `self.ReceiveBeginPlay`
  (bind _pathtable (`self.PathTable`))
  (bind _outrownames (`DataTableFunctionLibrary.GetDataTableRowNames` _pathtable))
  (for _array_element _outrownames
    (bind _returnvalue (`|GetDataTableRow` _pathtable _array_element)
      (:`then`
        (bind _path (break `/Game/Asset/Blueprints/Struct/Path` _returnvalue))
        (bind _returnvalue_2 (`|SpawnActorFromClass` _path (`KismetMathLibrary.MakeTransform` (0.0 0.0 40.0)) "Undefined" "OverrideRootScale" self null))
        (`BlueprintMapLibrary.Map_Add` (`self.Paths`) (`KismetSystemLibrary.GetClassDisplayName` _path) (`/Game/Asset/Blueprints/Path/BP_PathBase.Spline` _returnvalue_2))))))

(fn `CalculateDeltaLocation`
  (params (PathClass :type "/Game/Asset/Blueprints/Path/BP_PathBase Class Reference") (Distance :type "Float (double-precision)") (DeltaDistance :type "Float (double-precision)"))
  (returns (DeltaPosition :type "Vector Structure") (SpeedPercent :type "Float (double-precision)"))
  (bind (_path _isfound) (`self.GetPath` PathClass))
  (if _isfound
    (return (- (`SplineComponent.GetLocationAtDistanceAlongSpline` _path (mod Distance (`SplineComponent.GetSplineLength` _path)) "World") (`SplineComponent.GetLocationAtDistanceAlongSpline` _path (mod (- Distance DeltaDistance) (`SplineComponent.GetSplineLength` _path)) "World")) (`KismetMathLibrary.Dot_VectorVector` (`KismetMathLibrary.Normal` (`SplineComponent.GetTangentAtDistanceAlongSpline` _path Distance "World")) (`KismetMathLibrary.Normal` (`SplineComponent.GetTangentAtDistanceAlongSpline` _path (+ Distance DeltaDistance) "World"))))))

(fn `UserConstructionScript`)