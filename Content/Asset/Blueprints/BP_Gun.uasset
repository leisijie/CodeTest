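; BP_Gun is the player character's gun, which spawns bullets toward the character's aim position.
; On BeginPlay it caches the relative location of the owning BP_PlayerCharacter's Arrow as the fire offset.
; Fire spawns a Bullet at the owner's location plus that unrotated offset, then sets its ForwardVector to the normalized direction from the character to AimPosition.
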(event `self.ReceiveBeginPlay`
  (bind _asbp_player_character (cast `/Game/Asset/Blueprints/BP_PlayerCharacter` (`self.GetOwner` self)))
  (set `self.FirePositionRelativeToActor` (`SceneComponent.RelativeLocation` (`/Game/Asset/Blueprints/BP_PlayerCharacter.Arrow` _asbp_player_character))))

(fn `Fire`
  (bind _returnvalue (`self.GetOwner` self))
  (bind _returnvalue_2 (`|SpawnActorFromClass` (`self.Bullet`) (`KismetMathLibrary.Conv_VectorToTransform` (+ (`Actor.K2_GetActorLocation` _returnvalue) (`self.FirePositionRelativeToActor`))) "Undefined" "OverrideRootScale" null null))
  (bind _asbp_player_character (cast `/Game/Asset/Blueprints/BP_PlayerCharacter` _returnvalue))
  (set `/Game/Asset/Blueprints/BP_Bullet.ForwardVector` (`KismetMathLibrary.Normal` (- (`/Game/Asset/Blueprints/BP_PlayerCharacter.AimPosition` _asbp_player_character) (`Actor.K2_GetActorLocation` _asbp_player_character))) _returnvalue_2))