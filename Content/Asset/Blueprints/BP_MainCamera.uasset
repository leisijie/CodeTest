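; Main camera that registers with BP_PlayerController and rotates between left and right limits from horizontal movement and mouse position.
; Each tick, it sums curve-shaped move influence and scaled mouse offset as the rotation lerp alpha.
; When movement passes a threshold and horizontal speed reaches zero, the CameraRecover timeline eases move influence toward its threshold value, rearming once back in range.
; It also prints move influence every frame.
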(event `self.ReceiveBeginPlay`
  (bind _asbp_player_controller (cast `/Game/Asset/Blueprints/BP_PlayerController` (`GameplayStatics.GetPlayerController` 0)))
  (set `/Game/Asset/Blueprints/BP_PlayerController.MainCamera` self _asbp_player_controller))

(event `self.ReceiveTick`
  (params (DeltaSeconds :type "Float (single-precision)"))
  (`self.CheckMovementRange`)
  (`self.CheckSpeedValue`)
  (bind _influence (`self.MoveInfluence`))
  (`KismetSystemLibrary.PrintString` (`KismetStringLibrary.Conv_DoubleToString` _influence))
  (bind _influence_2 (`self.MouseInfluence`))
  (`self.K2_SetActorRotation` (`KismetMathLibrary.RLerp` (`self.LeftRotation`) (`self.RightRotation`) (+ _influence_2 _influence) true)))

(event `BeginDash`
  (bind (_direction _newtrack_0) (`Timeline|CameraRecover` :!via `PlayFromStart`)
    (:`Update`
      (set `self.CameraRecoverInfluence` _newtrack_0))
    (:`Finished`
      (set `self.IsDashFinish` true))))

(fn `CheckMovementRange`
  (bind _output_get (set `self.IsOutRange` (>= (`KismetMathLibrary.Abs` (* (- (`self.HorizontalMovePercent`) 0.5) 2.0)) (`self.MovementThreshold`))))
  (if (not _output_get)
    (set `self.IsDashFinish` false)
    (set `self.IsOnDash` false)))

(fn `CheckSpeedValue`
  (set `self.IsSpeedZero` (`KismetMathLibrary.NearlyEqual_FloatFloat` (`self.HorizontalSpeed`))))

(fn `MouseInfluence`
  (returns (influence :type "Float (double-precision)"))
  (return (* (* (- (`self.HorizontalMousePercent`) 0.5) 2.0) (`self.MouseScale`))))

(fn `MoveInfluence`
  (returns (influence :type "Float (double-precision)"))
  (bind _rotatecurve (`self.RotateCurve`))
  (bind _returnvalue (* (- (`self.HorizontalMovePercent`) 0.5) 2.0))
  (bind _returnvalue_2 (`KismetMathLibrary.SignOfFloat` _returnvalue))
  (bind _returnvalue_3 (`KismetMathLibrary.FClamp` (+ 0.5 (* _returnvalue_2 (* (`CurveFloat.GetFloatValue` _rotatecurve (`KismetMathLibrary.Abs` _returnvalue)) 0.5)))))
  (if (`self.IsOutRange`)
    (if (`self.IsDashFinish`)
      (return (`KismetMathLibrary.Lerp` _returnvalue_3 (+ 0.5 (* (* (`CurveFloat.GetFloatValue` _rotatecurve (`self.MovementThreshold`)) 0.5) _returnvalue_2)) (`self.CameraRecoverInfluence`)))
      (elif (`self.IsOnDash`)
        (return (`KismetMathLibrary.Lerp` _returnvalue_3 (+ 0.5 (* (* (`CurveFloat.GetFloatValue` _rotatecurve (`self.MovementThreshold`)) 0.5) _returnvalue_2)) (`self.CameraRecoverInfluence`)))
        (elif (`self.IsSpeedZero`)
          (`self.BeginDash`)
          (set `self.IsOnDash` true)
          (return (`KismetMathLibrary.Lerp` _returnvalue_3 (+ 0.5 (* (* (`CurveFloat.GetFloatValue` _rotatecurve (`self.MovementThreshold`)) 0.5) _returnvalue_2)) (`self.CameraRecoverInfluence`)))
          (else
            _)))))
  (return _returnvalue_3))

(fn `UserConstructionScript`)