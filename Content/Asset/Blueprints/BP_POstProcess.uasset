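; Post-process actor that can apply a random weather look, apparently fog, when play begins.
; If RandomWeather is set, BeginPlay picks a random Foggroup entry and writes it as the post-process materials in the PostProcess1 component's settings.
; The target is found by a class lookup for BP_POstProcess rather than a self reference, so it may be another instance if several exist.
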(event `self.ReceiveBeginPlay`
  (bind _foggroup (`self.foggroup`))
  (if (`self.RandomWeather`)
    (bind _returnvalue (`GameplayStatics.GetActorOfClass` "BP_POstProcess_C"))
    (`/Engine/EditorBlueprintResources/StandardMacros.IsValid` _returnvalue
      (:`Is Valid`
        (setmembers `PostProcessSettings` :`StructRef` (`PostProcessComponent.Settings` (`/Game/Asset/Blueprints/BP_POstProcess.PostProcess1` _returnvalue)) :`WeightedBlendables` (`|GetArrayItem` _foggroup (`KismetMathLibrary.RandomInteger` (`KismetArrayLibrary.Array_Length` _foggroup))))))))

(fn `UserConstructionScript`)