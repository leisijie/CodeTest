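; BP_PlayerBullet is the player's projectile, launched along a forward vector by setting the linear velocity of its physics sphere.
; Tick adds up estimated travel from speed and delta time, destroying the bullet past a maximum distance.
; On hit, the other actor's first tag selects the response: enemies take damage through BeHit on BP_Enemy, while obstacles, untagged actors and other tags just destroy the bullet.
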(event `self.ReceiveBeginPlay`
  (`self.K2_SetActorRotation` (`KismetMathLibrary.Conv_VectorToRotator` (`self.ForwardVector`)))
  (`PrimitiveComponent.SetPhysicsLinearVelocity` (`self.Sphere2`) (* (`self.ForwardVector`) (`self.Speed`)) false "None"))

(event `self.ReceiveHit`
  (params (MyComp :type "PrimitiveComponent Object Reference") (Other :type "Actor Object Reference") (OtherComp :type "PrimitiveComponent Object Reference") (bSelfMoved :type Boolean) (HitLocation :type "Vector Structure") (HitNormal :type "Vector Structure") (NormalImpulse :type "Vector Structure") (Hit :type "HitResult Structure (by ref)"))
  (bind _tags (`Actor.Tags` Other))
  (if (`KismetArrayLibrary.Array_IsValidIndex` _tags)
    (switch `name` (`|GetArrayItem` _tags)
      (:`Default`
        (`self.HitObstacle` :!label _label))
      (:`Enemy`
        (`self.HitEnemy` Other))
      (:`Obstacle`
        (goto _label)))
    (else
      (`self.HitObstacle`))))

(event `self.ReceiveTick`
  (params (DeltaSeconds :type "Float (single-precision)"))
  (bind _output_get (set `self.Distance` (+ (* DeltaSeconds (`self.Speed`)) (`self.Distance`))))
  (if (> _output_get (`self.MaxDistance`))
    (`self.K2_DestroyActor`)))

(fn `HitEnemy`
  (params (Actor :type "Actor Object Reference"))
  (bind _asbp_enemy (cast `/Game/Asset/Blueprints/BP_Enemy` Actor))
  (`/Game/Asset/Blueprints/BP_Enemy.BeHit` _asbp_enemy (`self.Damage`))
  (`KismetSystemLibrary.PrintString` (`KismetSystemLibrary.GetObjectName` _asbp_enemy))
  (`self.K2_DestroyActor`))

(fn `HitObstacle`
  (`self.K2_DestroyActor`))

(fn `UserConstructionScript`)