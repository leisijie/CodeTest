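; Player character that rides an attached vehicle, aims with laser beams and can take over an enemy's car.
; It spawns the default car at BeginPlay, aligned by its seat, and hands its gun to the player controller.
; Each tick it updates three aim beams and box-scans the aimed side for an enemy car to target, drawing debug boxes.
; ChangeCar destroys the current car, then a timeline moves the player to the new seat before attaching that car.
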(event `self.ReceiveBeginPlay`
  (`self.SpawnDefaultCar`)
  (bind _asbp_player_controller (cast `/Game/Asset/Blueprints/BP_PlayerController` (`GameplayStatics.GetPlayerController` 0)))
  (set `/Game/Asset/Blueprints/BP_PlayerController.PlayerGun` (`self.BP_Gun`) _asbp_player_controller))

(event `self.ReceiveTick`
  (params (DeltaSeconds :type "Float (single-precision)"))
  (`self.RotateAimLine`)
  (`self.FindCar` 0.0))

(event `BeginChangeCar`
  (bind _car (`self.Car`))
  (bind (_direction _newtrack_0) (`Timeline|ChanegCarTimeline` :!via `PlayFromStart`)
    (:`Update`
      (`self.K2_SetActorLocation` (`KismetMathLibrary.VLerp` (`self.K2_GetActorLocation`) (`SceneComponent.K2_GetComponentLocation` (`/Game/Asset/Blueprints/BP_Car.Seat` _car)) _newtrack_0)))
    (:`Finished`
      (`self.K2_AttachToActor` _car self "None" "KeepWorld" "KeepWorld" "KeepWorld" true))))

(fn `ChangeCar`
  (params (NewCar :type "/Game/Asset/Blueprints/BP_Car Object Reference"))
  (`/Engine/EditorBlueprintResources/StandardMacros.IsValid` NewCar
    (:`Is Valid`
      (bind _asbp_enemy (cast `/Game/Asset/Blueprints/BP_Enemy` (`self.GetAttachParentActor` NewCar))
        (:`then`
          (`self.K2_DetachFromActor` _asbp_enemy "KeepWorld" "KeepWorld" "KeepWorld")
          (`self.K2_DestroyActor` (`self.Car`))
          (set `self.Car` NewCar)
          (`self.BeginChangeCar`))
        (:`CastFailed`
          (`KismetSystemLibrary.PrintString` "Hello"))))))

(fn `FindCar`
  (params (Degree :type "Float (double-precision)"))
  (bind _returnvalue (`self.K2_GetActorLocation`))
  (bind _boxpos (`self.BoxPos`))
  (bind _boxextent (`self.BoxExtent`))
  (bind _returnvalue_2 (/ _boxextent 2.0))
  (bind _returnvalue_3 (+ _boxpos _returnvalue))
  (if (>= (.x (`self.AimPosition`)) (.x _returnvalue))
    (`KismetSystemLibrary.DrawDebugBox` _returnvalue_3 _returnvalue_2 (struct :`R` 1.0 :`A` 1.0) (struct) 0.0 10.0)
    (bind (_outactors _returnvalue_4) (`KismetSystemLibrary.BoxOverlapActors` _returnvalue_3 _boxextent (`|MakeArray` "ObjectTypeQuery7" :!type "EObjectTypeQuery Enum")))
    (if _returnvalue_4
      (for _array_element _outactors
        (bind _asbp_enemy (cast `/Game/Asset/Blueprints/BP_Enemy` _array_element))
        (set `self.Target` (`/Game/Asset/Blueprints/BP_Enemy.Car` _asbp_enemy))))
    (else
      (bind _result (`/Engine/EditorBlueprintResources/StandardMacros.NegateFloat` (.x _boxpos))
        (:`  `
          (bind _returnvalue_5 (+ (`KismetMathLibrary.MakeVector` _result (.y _boxpos) (.z _boxpos)) _returnvalue))
          (`KismetSystemLibrary.DrawDebugBox` _returnvalue_5 _returnvalue_2 (struct :`R` 1.0 :`A` 1.0) (struct) 0.0 10.0)
          (bind (_outactors_2 _returnvalue_6) (`KismetSystemLibrary.BoxOverlapActors` _returnvalue_5 _boxextent (`|MakeArray` "ObjectTypeQuery7" :!type "EObjectTypeQuery Enum")))
          (if _returnvalue_6
            (for _array_element_2 _outactors_2
              (bind _asbp_enemy_2 (cast `/Game/Asset/Blueprints/BP_Enemy` _array_element_2))
              (set `self.Target` (`/Game/Asset/Blueprints/BP_Enemy.Car` _asbp_enemy_2)))))))))

(fn `RotateAimLine`
  (bind _laserbeam (`self.LaserBeam`))
  (bind _aimposition (`self.AimPosition`))
  (bind _laserbeamdown (`self.LaserBeamDown`))
  (bind _laserbeamground (`self.LaserBeamGround`))
  (bind _x (.x _aimposition))
  (bind _y (.y _aimposition))
  (`ParticleSystemComponent.SetBeamSourcePoint` _laserbeam 0 (`KismetMathLibrary.MakeVector` (.x (`self.K2_GetActorLocation`)) (.y (`self.K2_GetActorLocation`))) 0)
  (`ParticleSystemComponent.SetBeamTargetPoint` _laserbeam 0 (`KismetMathLibrary.MakeVector` (.x _aimposition) (.y _aimposition)) 0)
  (bind _outhit (`KismetSystemLibrary.LineTraceSingle` (`KismetMathLibrary.MakeVector` _x _y 500.0) (`KismetMathLibrary.MakeVector` _x _y -500.0) "TraceTypeQuery1"))
  (`ParticleSystemComponent.SetBeamSourcePoint` _laserbeamdown 0 _aimposition 0)
  (bind (_bblockinghit _binitialoverlap _time _distance _location _impactpoint) (`GameplayStatics.BreakHitResult` _outhit))
  (`ParticleSystemComponent.SetBeamTargetPoint` _laserbeamdown 0 _impactpoint 0)
  (`ParticleSystemComponent.SetBeamSourcePoint` _laserbeamground 0 (+ (0.0 -100.0 10.0) _impactpoint) 0)
  (`ParticleSystemComponent.SetBeamTargetPoint` _laserbeamground 0 (+ (0.0 100.0 10.0) _impactpoint) 0))

(fn `SpawnDefaultCar`
  (bind _returnvalue (`|SpawnActorFromClass` (`self.DefaultCar`) (`KismetMathLibrary.MakeTransform` (0.0 0.0 0.0)) "Undefined" "OverrideRootScale" self null))
  (bind _output_get (set `self.Car` _returnvalue))
  (`self.K2_AttachToActor` _output_get self "None" "KeepRelative" "KeepRelative" "KeepRelative" true)
  (`self.K2_SetActorRelativeLocation` _output_get (`KismetMathLibrary.NegateVector` (`SceneComponent.RelativeLocation` (`/Game/Asset/Blueprints/BP_Car.Seat` _output_get))) false false)
  (bind _asanim_b_moto (cast `/Game/Asset/Animation/MOTO/AnimB_Moto` (`SkeletalMeshComponent.GetAnimInstance` (`/Game/Asset/Blueprints/BP_Car.Motor` _returnvalue))))
  (set `/Game/Asset/Animation/MOTO/AnimB_Moto.IsPlayer` true _asanim_b_moto))

(fn `UserConstructionScript`)