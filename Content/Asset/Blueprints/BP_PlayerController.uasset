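; Player controller that drives the player's gun-mounted car, routing input to movement, weapons, UI and cameras.
; Tick moves the car within GameMode bounds, decays the accumulated input behind turn animation values and feeds camera parameters.
; Guns are mapped by direction and toggled between two slots, with a gated-delay macro pacing automatic fire.
; It also handles reloads, hold-to-upgrade spending cores, a gascan-gated LAGAAN launcher and static camera switching.
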(event `StartControll`
  (`self.EnableInput` self))

(event `self.ReceiveTick`
  (params (DeltaSeconds :type "Float (single-precision)"))
  (`self.MoveTime` DeltaSeconds)
  (`self.CharacterMove`)
  (`self.SetMainCameraPara`)
  (`self.SpeedAcGravity`)
  (`/Engine/EditorBlueprintResources/StandardMacros.DoOnce` false
    (:`Completed`
      (bind _returnvalue (`|CreateWidget` "/Game/Asset/Widget/BulletWidget.BulletWidget_C" self))
      (bind _output_get (set `self.BulletWidget` _returnvalue))
      (`UserWidget.AddToPlayerScreen` _output_get 0)
      (`/Game/Asset/Widget/BulletWidget.Init` _output_get (`self.MainCharacter`))
      (`self.InitGun&Widget`)
      (`self.DefaultGunAndWidget`))))

(event `StopControll`
  (`self.DisableInput` self))

(event `DirectionChanged`
  (`self.ChangeGunAndWidget`))

(event `self.ReceiveBeginPlay`
  (`|ExecutionSequence`
    (:`then_0`
      (bind _asbp_player_character (cast `/Game/Asset/Blueprints/Character/BP_PlayerCharacter` (`GameplayStatics.GetPlayerPawn` 0)))
      (set `self.MainCharacter` _asbp_player_character)
      (bind _asbp_game_mode (cast `/Game/Asset/Blueprints/GameMode/BP_GameMode` (`GameplayStatics.GetGameMode`)))
      (set `self.GameMode` _asbp_game_mode))))

(event `InputAction|Strat Switch`
  (params (Key :type "Key Structure"))
  (:`Pressed`
    (bind _counter (`/Engine/EditorBlueprintResources/StandardMacros.Do N` 2 :!label _label)
      (:`Exit`
        (`self.DetectDirection` _counter)))))

(event `Reset Timer`
  (goto _label :!via `Reset`))

(event `InputAction|Fire`
  (params (Key :type "Key Structure"))
  (bind _currentgun (`self.CurrentGun`))
  (bind _dir (`/Game/Asset/Blueprints/Gun/BP_GunBase.Dir` (`self.CurrentGun`)))
  (bind _cur_max (`/Game/Asset/Blueprints/Gun/BP_GunBase.Cur/Max` _currentgun))
  ;[1 1 1] Fire&Reload
  (:`Pressed`
    (if (`/Game/Asset/Blueprints/Gun/BP_GunBase.Can_FireCon` _currentgun)
      (`self.Fire_Con` (`/Game/Asset/Blueprints/Gun/BP_GunBase.FireRate` _currentgun) :!label _label_2
        (:`Fire`
          (if (not (`/Game/Asset/Blueprints/Gun/BP_GunBase.Overcharge` _currentgun))
            (`/Game/Asset/Blueprints/Gun/BP_GunBase.GunFire` _currentgun true :!label _label_3)
            (`/Game/Asset/Blueprints/Character/BP_PlayerCharacter.bulletGas` (`self.MainCharacter`) (`/Game/Asset/Blueprints/Gun/BP_GunBase.Gas` _currentgun))
            (`/Game/Asset/Widget/BulletWidget.Fire` (`self.BulletWidget`) _dir _cur_max)
            (`/Game/Asset/Blueprints/Character/BP_PlayerCharacter.Check Ammo` (`self.MainCharacter`) _cur_max _dir))))
      (else
        (goto _label_3))))
  (:`Released`
    (`|ExecutionSequence`
      (:`then_0`
        (goto _label_2 :!via `Off`))
      (:`then_1`
        (`/Game/Asset/Blueprints/Gun/BP_GunBase.FireOff` _currentgun)))))

(event `InputAction|Upgrade`
  (params (Key :type "Key Structure"))
  (bind _bulletwidget (`self.BulletWidget`))
  ;[1 1 1] Upgrade Your GUN
  (:`Pressed`
    (if (> (`self.Upgrade Core`) 0)
      (bind _returnvalue (`KismetSystemLibrary.K2_SetTimer` null "Upgrade Timer" 0.01 true))
      (`/Game/Asset/Widget/BulletWidget.upgrade Mode` _bulletwidget)))
  (:`Released`
    (`|ExecutionSequence`
      (:`then_0`
        (`/Game/Asset/Widget/BulletWidget.Upgrade OFF` _bulletwidget))
      (:`then_1`
        (`self.Upgrade CUT`)))))

(event `InputAction|Reload`
  (params (Key :type "Key Structure"))
  (bind _currentgun (`self.CurrentGun`))
  ;[1 1 1] Fire&Reload
  (:`Pressed`
    (`/Game/Asset/Blueprints/Gun/BP_GunBase.ReloadBullet` _currentgun :!label _label_4)
    (`/Game/Asset/Widget/BulletWidget.StartLoad` (`self.BulletWidget`) (`/Game/Asset/Blueprints/Gun/BP_GunBase.Dir` _currentgun))))

(event `Upgrade GUN`
  (bind _maincharacter (`self.MainCharacter`))
  ;[1 1 1] Upgrade Your GUN
  (if (> (`self.Upgrade Core`) 0)
    (set `self.Upgrade Check Timer` 0.0)
    (`/Game/Asset/Blueprints/Character/BP_PlayerCharacter.UpgradeGun` _maincharacter (`/Game/Asset/Blueprints/Gun/BP_GunBase.Dir` (`self.CurrentGun`)))
    (set `self.Upgrade Core` (- (`self.Upgrade Core`) 1))
    (`/Game/Asset/Widget/Main_Controller.Core Check` (`/Game/Asset/Blueprints/Character/BP_PlayerCharacter.HPWidget` _maincharacter))
    (else
      (`self.Upgrade CUT`))))

(event `Special Reload`
  ;[1 1 1] Fire&Reload
  (goto _label_4))

(event `Upgrade CUT`
  ;[1 1 1] Upgrade Your GUN
  (`KismetSystemLibrary.K2_ClearAndInvalidateTimerHandle` (stale `InputAction|Upgrade` _returnvalue))
  (set `self.Upgrade Check Timer` 0.0)
  (`ProgressBar.SetPercent` (`/Game/Asset/Widget/BulletWidget.UPgradeProgress` (`self.BulletWidget`)) 0.0))

(event `InputAction|lagaanLunch`
  (params (Key :type "Key Structure"))
  ;[1 1 1] UseLAGGAN
  (:`Pressed`
    (bind _lagaanluncher (`self.GetLAGAANLuncher`)
      (:`Out`
        (`/Game/Asset/Blueprints/Follower/LAGAANLuncher.Aim` _lagaanluncher))))
  (:`Released`
    (bind _lagaanluncher_2 (`self.GetLAGAANLuncher`)
      (:`Out`
        (if (`self.DoYouHaveGascan`)
          (`/Game/Asset/Blueprints/Follower/LAGAANLuncher.Start` _lagaanluncher_2))))))

(event `Get Core`
  (params (CorAmount :type Integer))
  ;[1 1 1] Upgrade Your GUN
  ;;[1 1 1] Get Core
  (set `self.Upgrade Core` (+ (`self.Upgrade Core`) CorAmount))
  (`/Game/Asset/Widget/Main_Controller.Core Check` (`/Game/Asset/Blueprints/Character/BP_PlayerCharacter.HPWidget` (`self.MainCharacter`))))

(event `InputAxis|Vertical`
  (params (AxisValue :type "Float (single-precision)"))
  (bind (_x _y) (`KismetMathLibrary.BreakVector2D` (`self.SpeedAccumulation`)))
  ;[1 1 1] LeftAxis
  (set `self.MoveVector` (`KismetMathLibrary.MakeVector2D` AxisValue (`.Y` (`KismetMathLibrary.BreakVector2D` (`self.MoveVector`)))))
  (set `self.SpeedAccumulation` (`KismetMathLibrary.MakeVector2D` _x (+ (* (* AxisValue (`self.Strength`)) (`GameplayStatics.GetWorldDeltaSeconds`)) _y))))

(event `InputAxis|Horizontal`
  (params (AxisValue :type "Float (single-precision)"))
  (bind (_x _y) (`KismetMathLibrary.BreakVector2D` (`self.SpeedAccumulation`)))
  ;[1 1 1] LeftAxis
  (set `self.MoveVector` (`KismetMathLibrary.MakeVector2D` (`KismetMathLibrary.BreakVector2D` (`self.MoveVector`)) AxisValue))
  (set `self.SpeedAccumulation` (`KismetMathLibrary.MakeVector2D` (+ _x (* (`GameplayStatics.GetWorldDeltaSeconds`) (* (`self.Strength`) AxisValue))) _y)))

(event `InputAxis|Weapon Wheel Forward`
  (params (AxisValue :type "Float (single-precision)"))
  ;[1 1 1] RightAxis
  (set `self.RightWheelValue` (`KismetMathLibrary.MakeVector2D` AxisValue (stale `InputAxis|Weapon Wheel Side` AxisValue)) :!label _label_5)
  (bind (_direction _angel_yaw_) (`self.Gun_Rotation`))
  (`/Game/Asset/Blueprints/Car/BP_Car.Gun Rotation` (`/Game/Asset/Blueprints/Character/BP_PlayerCharacter.Car` (`self.MainCharacter`)) _direction _angel_yaw_))

(event `InputAxis|Weapon Wheel Side`
  (params (AxisValue :type "Float (single-precision)"))
  ;[1 1 1] RightAxis
  (goto _label_5))

(event `InputAction|SwitchCineModel`
  (params (Key :type "Key Structure"))
  (bind _staticcamera (`self.StaticCamera`))
  ;[1 1 1] SwitchCineModel
  (:`Pressed`
    (`/Engine/EditorBlueprintResources/StandardMacros.FlipFlop`
      (:`A`
        (`self.SetViewTargetWithBlend` _staticcamera 1.0 "VTBlend_Linear" 1.0 true)
        (`KismetSystemLibrary.PrintString` (`KismetSystemLibrary.GetDisplayName` _staticcamera)))
      (:`B`
        (`self.SetViewTargetWithBlend` (`self.MainCamera`) 1.0 "VTBlend_Linear" 1.0 true)))))

(event `PrepareCamera`
  (params (NewParam :type "/Game/Asset/Blueprints/BP_MainCamera Object Reference"))
  (bind _maincamera (`self.MainCamera`))
  ;[1 1 1] PrepareCamera
  (`/Engine/EditorBlueprintResources/StandardMacros.DoOnce` false
    (:`Completed`
      (set `self.MainCamera` NewParam)
      (bind _returnvalue (`|SpawnActorFromClass` "/Game/Asset/Blueprints/BP_MainCamera.BP_MainCamera_C" (`KismetMathLibrary.MakeTransform` (`self.K2_GetActorLocation` _maincamera) (`self.K2_GetActorRotation` _maincamera)) "Undefined" "OverrideRootScale" null null))
      (bind _output_get (set `self.StaticCamera` _returnvalue))
      (`/Game/Asset/Blueprints/BP_MainCamera.SwitchCineModel` _output_get))))

(fn `CalRealMoveVector`
  (params (MoveVector :type "Vector2D Structure") (MaxMoveRange :type "Vector2D Structure"))
  (returns (RealMoveVector :type "Vector2D Structure"))
  (locals (DeltaX :type "Float (double-precision)") (DeltaY :type "Float (double-precision)"))
  (bind (_x _y) (`KismetMathLibrary.BreakVector2D` MaxMoveRange))
  (bind (_x_2 _y_2) (`KismetMathLibrary.BreakVector2D` MoveVector))
  (bind (_x_3 _y_3) (`KismetMathLibrary.BreakVector2D` (`KismetMathLibrary.Negated2D` MaxMoveRange)))
  (bind (_x_4 _y_4) (`KismetMathLibrary.BreakVector2D` (+ MoveVector (`KismetMathLibrary.Conv_VectorToVector2D` (`self.K2_GetActorLocation` (`self.MainCharacter`))))))
  ;[1 1 1] 如果X到达边界，则deltaX设为0（y同理）
  (if (>= _x _x_4)
    (if (>= _x_4 _x_3)
      (set `local.DeltaX` _x_2)
      (else
        (set `local.DeltaX` 0.0 :!label _label)))
    (else
      (goto _label)))
  ;[1 1 1] Y
  (if (>= _y _y_4)
    (if (>= _y_4 _y_3)
      (set `local.DeltaY` _y_2)
      (else
        (set `local.DeltaY` 0.0)))
    (`KismetSystemLibrary.DrawDebugBox` (0.0 550.0 0.0) (`KismetMathLibrary.Conv_Vector2DToVector` (0.0 0.0)) (struct :`R` 0.243041 :`G` 0.191743 :`B` 0.85 :`A` 1.0) (struct) 0.0 10.0)
    (return (`KismetMathLibrary.MakeVector2D` (`local.DeltaX`) (`local.DeltaY`)))))

(fn `ChangeGunAndWidget`
  (bind _firedirection (`self.FireDirection`))
  (set `self.CurrentGun` (`BlueprintMapLibrary.Map_Find` (`self.GunMap`) _firedirection))
  (`/Game/Asset/Widget/BulletWidget.Switch` (`self.BulletWidget`) _firedirection (`self.PreviousFireDirection`)))

(fn `CharacterMove`
  (locals (DeltaX :type "Float (double-precision)") (DeltaY :type "Float (double-precision)"))
  (bind _maincharacter (`self.MainCharacter`))
  (bind _maincamera (`self.MainCamera`))
  (bind (_x _y) (`KismetMathLibrary.BreakVector2D` (`self.MoveVector`)))
  (bind (_x_2 _y_2) (`KismetMathLibrary.BreakVector2D` (`self.SpeedAccumulation`)))
  (bind (_x_3 _y_3) (`KismetMathLibrary.BreakVector2D` (`KismetMathLibrary.Negated2D` (`/Game/Asset/Blueprints/GameMode/BP_GameMode.MaxMoveRangeExtent` (`self.GameMode`)))))
  (set `self.AnimMoveVaribles` (`KismetMathLibrary.MakeVector2D` (* (`KismetMathLibrary.SignOfFloat` _y_2) (`CurveFloat.GetFloatValue` (`self.AnimTurnCurve`) (`KismetMathLibrary.Abs` _y_2))) (* (`CurveFloat.GetFloatValue` (`self.AnimTurnCurve`) (`KismetMathLibrary.Abs` _x_2)) (`KismetMathLibrary.SignOfFloat` _x_2))))
  (bind _realmovevector (`self.CalRealMoveVector` (`KismetMathLibrary.Conv_VectorToVector2D` (* (`KismetMathLibrary.Conv_Vector2DToVector` (`KismetMathLibrary.MakeVector2D` (* _x (`self.VerticalSpeed`)) (* _y (`CurveFloat.GetFloatValue` (`self.HorizontalSpeedCurve`) (`self.HorizontalMoveTimer`))))) (`GameplayStatics.GetWorldDeltaSeconds`))) (`/Game/Asset/Blueprints/GameMode/BP_GameMode.MaxMoveRangeExtent` (`self.GameMode`))))
  (set `/Game/Asset/Blueprints/BP_MainCamera.HorizontalSpeed` (`KismetMathLibrary.BreakVector2D` _realmovevector) (`self.MainCamera`))
  (`/Game/Asset/Blueprints/Car/BP_Car.Drive` (`/Game/Asset/Blueprints/Character/BP_PlayerCharacter.Car` _maincharacter) _realmovevector)
  (set `/Game/Asset/Blueprints/BP_MainCamera.HorizontalMovePercent` (`self.MovePercent` (.y (`self.K2_GetActorLocation` _maincharacter)) _y_3) _maincamera)
  (set `/Game/Asset/Blueprints/BP_MainCamera.VerticalMovePercent` (`self.MovePercent` (.x (`self.K2_GetActorLocation` _maincharacter)) _x_3) _maincamera))

(fn `DefaultGunAndWidget`
  (set `self.CurrentGun` (`BlueprintMapLibrary.Map_Find` (`self.GunMap`) (`self.FireDirection`))))

(fn `DetectDirection`
  (params (Time :type Integer))
  (locals (X :type "Float (double-precision)") (Y :type "Float (double-precision)"))
  (bind _previousfiredirection (`self.PreviousFireDirection`))
  (bind _firedirection (`self.FireDirection`))
  (switch `int` Time
    (:`1`
      (set `self.FireDirection` "NewEnumerator2")
      (if (`|EnumInequality` _firedirection _previousfiredirection) :!label _label
        (`self.DirectionChanged`)
        (`/Game/Asset/Blueprints/Character/BP_PlayerCharacter.Switch` (`self.MainCharacter`) _firedirection _previousfiredirection (`self.CurrentGun`))
        (set `self.PreviousFireDirection` _firedirection)))
    (:`2`
      (`|ExecutionSequence`
        (:`then_0`
          (set `self.FireDirection` "NewEnumerator3")
          (goto _label))
        (:`then_1`
          (`self.Reset Timer`))))))

(fn `Gun_Rotation`
  (returns (Direction :type "Vector Structure") (`Angel（Yaw）` :type "Float (double-precision)"))
  (bind _rightwheelvalue (`self.RightWheelValue`))
  (bind (_x _y) (`KismetMathLibrary.BreakVector2D` _rightwheelvalue))
  (return (`KismetMathLibrary.Conv_Vector2DToVector` _rightwheelvalue) (`KismetMathLibrary.DegAtan2` _y _x)))

(fn `InitGun&Widget`
  (for _array_element (`/Game/Asset/Blueprints/Car/BP_Car.Guns` (`/Game/Asset/Blueprints/Character/BP_PlayerCharacter.Car` (`self.MainCharacter`)))
    (`BlueprintMapLibrary.Map_Add` (`self.GunMap`) (`/Game/Asset/Blueprints/Gun/BP_GunBase.Dir` _array_element) _array_element)))

(fn `KeepCameraAndCharacter`
  (bind _maincamera (`self.MainCamera`))
  (bind _staticcamera (`self.StaticCamera`))
  (bind _z (.z (`self.K2_GetActorLocation` _maincamera)))
  (`self.K2_SetActorLocation` _maincamera (`KismetMathLibrary.MakeVector` (.x (`self.K2_GetActorLocation` _maincamera)) (.y (`self.K2_GetActorLocation` (`self.MainCharacter`))) _z) false false)
  (`self.K2_SetActorLocation` _staticcamera (`KismetMathLibrary.MakeVector` (.x (`self.K2_GetActorLocation` _staticcamera)) (.y (`self.K2_GetActorLocation` _staticcamera)) _z) false false))

(fn `MousePositionInScreen`
  (returns (MousePositionInScreen :type "Vector2D Structure"))
  (bind (_sizex _sizey) (`self.GetViewportSize` self))
  (bind (_locationx _locationy) (`WidgetLayoutLibrary.GetMousePositionScaledByDPI` self))
  (return (/ (* (`KismetMathLibrary.MakeVector2D` _locationx _locationy) (`WidgetLayoutLibrary.GetViewportScale`)) (`KismetMathLibrary.MakeVector2D` (`KismetMathLibrary.Conv_IntToDouble` _sizex) (`KismetMathLibrary.Conv_IntToDouble` _sizey)))))

(fn `MoveTime`
  (params (DeltaTime :type "Float (double-precision)"))
  (locals (DeltaHorizontal :type "Float (double-precision)") (DeltaVertical :type "Float (double-precision)"))
  (bind (_x _y) (`KismetMathLibrary.BreakVector2D` (`self.MoveVector`)))
  (if (`KismetMathLibrary.NearlyEqual_FloatFloat` _y)
    (set `self.HorizontalMoveTimer` 0.0)
    (else
      (set `self.HorizontalMoveTimer` (+ DeltaTime (`self.HorizontalMoveTimer`)))))
  (if (`KismetMathLibrary.NearlyEqual_FloatFloat` _x)
    (set `self.VerticalMoveTimer` 0.0)
    (else
      (set `self.VerticalMoveTimer` (+ DeltaTime (`self.VerticalMoveTimer`))))))

(fn `ReplaceGunAndWidget`
  (params (NewGun :type "/Game/Asset/Blueprints/Gun/BP_GunBase Object Reference"))
  (bind _dir (`/Game/Asset/Blueprints/Gun/BP_GunBase.Dir` NewGun))
  (`BlueprintMapLibrary.Map_Remove` (`self.GunMap`) _dir)
  (`BlueprintMapLibrary.Map_Add` (`self.GunMap`) _dir NewGun)
  (`self.ChangeGunAndWidget`))

(fn `SetMainCameraPara`
  (bind _mousepositioninscreen (`self.MousePositionInScreen`))
  (set `/Game/Asset/Blueprints/BP_MainCamera.HorizontalMousePercent` (`KismetMathLibrary.BreakVector2D` _mousepositioninscreen) (`self.MainCamera`)))

(fn `SpeedAcGravity`
  (bind _returnvalue (`GameplayStatics.GetWorldDeltaSeconds`))
  (bind _falltime (`self.FallTime`))
  (bind (_x _y) (`KismetMathLibrary.BreakVector2D` (`self.SpeedAccumulation`)))
  (set `self.SpeedAccumulation` (`KismetMathLibrary.MakeVector2D` (- _x (* (`KismetMathLibrary.SignOfFloat` _x) (* (/ (`KismetMathLibrary.Abs` _x) _falltime) _returnvalue))) (- _y (* (* _returnvalue (/ (`KismetMathLibrary.Abs` _y) _falltime)) (`KismetMathLibrary.SignOfFloat` _y))))))

(fn `Upgrade Timer`
  (bind _upgrade_check_timer (`self.Upgrade Check Timer`))
  (bind _upgrade_timermax (`self.Upgrade TimerMAX`))
  (bind _upgradeprogress (`/Game/Asset/Widget/BulletWidget.UPgradeProgress` (`self.BulletWidget`)))
  (if (> (`self.Upgrade Core`) 0)
    (bind _output_get (set `self.Upgrade Check Timer` (+ _upgrade_check_timer 2.0)))
    (`ProgressBar.SetPercent` _upgradeprogress (/ _output_get _upgrade_timermax))
    (if (== _upgrade_check_timer _upgrade_timermax)
      (`self.Upgrade GUN`)
      (`ProgressBar.SetPercent` _upgradeprogress 0.0))
    (else
      (`self.Upgrade CUT`))))

(fn `UserConstructionScript`)