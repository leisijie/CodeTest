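; BP_Sensor is a scene-component sensor that line-traces along its local down axis and reports hit results on demand.
; GetResult calls UpdataData, which traces on the Camera channel over a length based on relative Z height, with debug drawing.
; Each call stores the new hit but returns the previously stored one, giving a one-call delay.
; When the current trace misses, it prints a warning instead.
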(fn `GetResult`
  (returns (Result :type "HitResult Structure"))
  (bind _lastframedata (`self.UpdataData`))
  (return _lastframedata))

(fn `UpdataData`
  (returns (LastFrameData :type "HitResult Structure"))
  (locals (OutputData :type "HitResult Structure"))
  (bind _returnvalue (`self.K2_GetComponentLocation`))
  (set `local.OutputData` (`self.LastFrameData`))
  (bind (_outhit _returnvalue_2) (`KismetSystemLibrary.LineTraceSingle` :`Start` _returnvalue :`End` (+ _returnvalue (* (`KismetMathLibrary.TransformDirection` (`self.K2_GetComponentToWorld`) (0.0 0.0 -1.0)) (+ (.z (`self.RelativeLocation`)) 100.0))) :`TraceChannel` "TraceTypeQuery2" :`DrawDebugType` "ForOneFrame" :`TraceHitColor` (struct :`R` 1.0 :`G` 0.05706 :`B` 0.898401 :`A` 1.0)))
  (set `self.LastFrameData` _outhit)
  (if _returnvalue_2
    (return (`local.OutputData`))
    (else
      (`KismetSystemLibrary.PrintString` "NoSensorValue"))))