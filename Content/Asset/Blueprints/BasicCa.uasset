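; BasicCa is an actor that moves along the BP_Path_A path at a speed scaled by path feedback.
; Each tick it advances its travelled distance and asks BP_GameState for the position delta and a new speed percentage.
; It applies the delta as an unswept world offset, while the returned percentage scales the next tick's step.
; BeginPlay stores the starting location, which this graph never reads.
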(event `self.ReceiveBeginPlay`
  (set `self.OriginalPoint` (`SceneComponent.K2_GetComponentLocation` (`self.DefaultSceneRoot`))))

(event `self.ReceiveTick`
  (params (DeltaSeconds :type "Float (single-precision)"))
  (bind _returnvalue (* (* DeltaSeconds (`self.Speed`)) (`self.SpeedPercent`)))
  (bind _asbp_game_state (cast `/Game/Asset/Blueprints/BP_GameState` (`GameplayStatics.GetGameState`)))
  (bind _output_get (set `self.Distance` (+ _returnvalue (`self.Distance`))))
  (bind (_deltaposition _speedpercent) (`/Game/Asset/Blueprints/BP_GameState.CalculateDeltaLocation` _asbp_game_state "/Game/Asset/Blueprints/Path/BP_Path_A.BP_Path_A_C" _output_get _returnvalue))
  (set `self.SpeedPercent` _speedpercent)
  (`SceneComponent.K2_AddWorldOffset` (`self.DefaultSceneRoot`) _deltaposition false false))

(fn `UserConstructionScript`)