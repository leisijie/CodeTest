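; Building_Generator_2 is a spawner that endlessly creates building actors at the transform of its Arrow component.
; On BeginPlay, if the Building reference is valid, it stores the first level actor of that class as ThisBuilding.
; It spawns a new actor of ThisBuilding's class, waits SpaceTime through a Delay, then loops back to spawn again, with no stop condition.
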(event `self.ReceiveBeginPlay`
  (bind _building (`self.building`))
  (`/Engine/EditorBlueprintResources/StandardMacros.IsValid` _building
    (:`Is Valid`
      (bind _outactors (`GameplayStatics.GetAllActorsOfClass` (`GameplayStatics.GetObjectClass` _building)))
      (set `self.this_building` (`|GetArrayItem` _outactors))
      (`|SpawnActorFromClass` (`GameplayStatics.GetObjectClass` (`self.this_building`)) (`SceneComponent.K2_GetComponentToWorld` (`self.Arrow`)) "Undefined" "OverrideRootScale" null null :!label _label)
      (`KismetSystemLibrary.Delay` (`self.Space_time`))
      (goto _label))))

(fn `UserConstructionScript`)