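; Enemy Boomer explosion "bullet" that deals area damage as soon as it spawns.
; BeginPlay runs a sphere overlap over DamageRadius on one custom object type and sends BeExploded with Damage to each hit's parent actor, implying child-actor hitboxes.
; The actor destroys itself when its particle system finishes.
; A construction-script debug sphere and printed victim names serve as debug output.
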(event `self.ReceiveBeginPlay`
  (`parent.ReceiveBeginPlay`)
  (`self.Explosion`))

(event `self.ParticleSystem.OnSystemFinished`
  (params (PSystem :type "ParticleSystemComponent Object Reference"))
  (`self.K2_DestroyActor`))

(fn `Explosion`
  (bind _outactors (`KismetSystemLibrary.SphereOverlapActors` (`self.K2_GetActorLocation`) (`self.DamageRadius`) (`|MakeArray` "ObjectTypeQuery13" :!type "EObjectTypeQuery Enum")))
  (for _array_element _outactors
    (bind _returnvalue (`self.GetParentActor` _array_element))
    (message `/Game/Asset/Blueprints/IF_Explosion.BeExploded` _returnvalue (`self.Damage`))
    (`KismetSystemLibrary.PrintString` (`KismetSystemLibrary.GetDisplayName` _returnvalue))))

(fn `UserConstructionScript`
  (`parent.UserConstructionScript`)
  (`KismetSystemLibrary.DrawDebugSphere` (`self.K2_GetActorLocation`) (`self.DamageRadius`) 12 (struct :`R` 0.367851 :`G` 0.208099 :`B` 0.729167 :`A` 1.0) 0.1 10.0))