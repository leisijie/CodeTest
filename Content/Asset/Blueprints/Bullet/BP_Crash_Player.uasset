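; BP_Crash_Player is a one-shot crash hit that damages enemies overlapping its Cube, apparently on the player's behalf.
; On BeginPlay it runs a component overlap query on a custom object type and casts each result's parent actor to BP_Enemy.
; Matching enemies receive BeHit damage and a large energy-shield impact effect spawns at its particle component.
; The actor destroys itself immediately, whether or not anything is hit.
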(event `self.ReceiveBeginPlay`
  (bind _cube (`self.Cube`))
  (`parent.ReceiveBeginPlay`)
  (`|ExecutionSequence`
    (:`then_1`
      (bind (_outactors _returnvalue) (`KismetSystemLibrary.ComponentOverlapActors` _cube (`SceneComponent.K2_GetComponentToWorld` _cube) (`|MakeArray` "ObjectTypeQuery12" :!type "EObjectTypeQuery Enum")))
      (if _returnvalue
        (for _array_element _outactors
          (bind _asbp_enemy (cast `/Game/Asset/Blueprints/Enemy/BP_Enemy` (`self.GetParentActor` _array_element))
            (:`then`
              (`/Game/Asset/Blueprints/Enemy/BP_Enemy.BeHit` _asbp_enemy 5)
              (`GameplayStatics.SpawnEmitterAtLocation` "/Game/BallisticsVFX/Particles/Impacts/LegacyFX/Small-Medium-Large/EnergyShield/EnergyShield_impact_Large.EnergyShield_impact_Large" (`SceneComponent.K2_GetComponentLocation` (`self.ParticleSystem`)) (struct) (2.0 2.0 2.0))
              (`self.K2_DestroyActor`))
            (:`CastFailed`
              (`self.K2_DestroyActor` :!label _label)))))
      (goto _label))))

(fn `UserConstructionScript`
  (`parent.UserConstructionScript`))