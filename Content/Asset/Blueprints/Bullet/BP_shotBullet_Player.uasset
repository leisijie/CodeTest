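; Player shot bullet that damages enemies in a growing or shrinking area during its half-second lifetime.
; A timeline started on BeginPlay scales the static mesh in X and Y, leaving Z fixed.
; Each timeline update overlap-tests the mesh against one object type and calls BeHit on the BP_Enemy parent of overlapped actors.
; No hit tracking exists, so an enemy can be hit on successive updates.
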(event `self.ReceiveBeginPlay`
  (bind _staticmesh (`self.StaticMesh`))
  (`parent.ReceiveBeginPlay`)
  (`|ExecutionSequence`
    (:`then_0`
      (`KismetSystemLibrary.Delay` 0.5)
      (`self.K2_DestroyActor`))
    (:`then_1`
      (bind (_direction _newtrack_0) (`Timeline|Timeline_0`)
        (:`Update`
          (`SceneComponent.SetWorldScale3D` (`self.StaticMesh`) (`KismetMathLibrary.MakeVector` (* (.x (`self.scale`)) _newtrack_0) (* (.y (`self.scale`)) _newtrack_0) (.z (`self.scale`))))
          (bind (_outactors _returnvalue) (`KismetSystemLibrary.ComponentOverlapActors` _staticmesh (`SceneComponent.K2_GetComponentToWorld` _staticmesh) (`|MakeArray` "ObjectTypeQuery14" :!type "EObjectTypeQuery Enum")))
          (if _returnvalue
            (for _array_element _outactors
              (bind _asbp_enemy (cast `/Game/Asset/Blueprints/Enemy/BP_Enemy` (`self.GetParentActor` _array_element)))
              (`/Game/Asset/Blueprints/Enemy/BP_Enemy.BeHit` _asbp_enemy 2))))))))

(fn `UserConstructionScript`
  (`parent.UserConstructionScript`))