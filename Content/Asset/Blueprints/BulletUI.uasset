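; BulletUI is an ammo indicator that shows remaining bullets and reload progress through a dynamic image material's "Depth" parameter.
; UseBullet subtracts the per-shot cost, refreshes the fill and reports whether ammo equals zero.
; ReloadStart dims the image and runs a looping timer to animate the fill, until a one-shot timer restores ammo and opacity.
; Upgrade overwrites the ammo and reload settings.
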(event `ReloadStart`
  (`KismetSystemLibrary.K2_SetTimer` null "Loading" 0.0167 true)
  (`KismetSystemLibrary.K2_SetTimerDelegate` (delegate `ReloadEnd`) (`self.ReloadDuration`))
  (`Image.SetOpacity` (`self.Image`) 0.5))

(event `ReloadEnd`
  (`KismetSystemLibrary.K2_ClearTimer` null "Loading")
  (set `self.CurrentAmmo` (`self.MaxAmmo`))
  (set `self.Timer` 0.0)
  (`self.UpdateImagePercent` (`self.AmmoPercent`))
  (`Image.SetOpacity` (`self.Image`) 1.0))

(fn `Loading`
  (bind _output_get (set `self.Timer` (+ 0.0167 (`self.Timer`))))
  (`self.UpdateImagePercent` (`KismetMathLibrary.FClamp` (/ _output_get (`self.ReloadDuration`)))))

(fn `UpdateImagePercent`
  (params (Percent :type "Float (double-precision)"))
  (bind _returnvalue (`Image.GetDynamicMaterial` (`self.Image`)))
  (`MaterialInstanceDynamic.SetScalarParameterValue` _returnvalue "Depth" Percent))

(fn `Upgrade`
  (params (MaxAmmo :type Integer) (CurrentAmmo :type Integer) (BulletCountToUse :type Integer) (ReloadDuration :type "Float (double-precision)"))
  (set `self.MaxAmmo` MaxAmmo)
  (set `self.CurrentAmmo` CurrentAmmo)
  (set `self.BulletCountToUse` BulletCountToUse)
  (set `self.ReloadDuration` ReloadDuration))

(fn `UseBullet`
  (returns (`RunOut?` :type Boolean))
  (set `self.CurrentAmmo` (- (`self.CurrentAmmo`) (`self.BulletCountToUse`)))
  (`self.UpdateImagePercent` (`self.AmmoPercent`))
  (return (== (`self.CurrentAmmo`) 0)))