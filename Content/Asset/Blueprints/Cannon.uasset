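; Cannon Blueprint that slowly turns its Cannon component to track the first player's pawn.
; Each Tick it takes the yaw of the direction from the cannon to the player, offsets it by -90 degrees and eases toward it with RInterpTo.
; Only yaw follows the player, as the target pitch and roll are zero.
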(event `self.ReceiveTick`
  (params (DeltaSeconds :type "Float (single-precision)"))
  (`SceneComponent.K2_SetWorldRotation` (`self.Cannon`) (`KismetMathLibrary.RInterpTo` (`SceneComponent.K2_GetComponentRotation` (`self.Cannon`)) (`KismetMathLibrary.MakeRotator` 0.0 0.0 (- (.yaw (`KismetMathLibrary.Conv_VectorToRotator` (- (`self.K2_GetActorLocation` (`GameplayStatics.GetPlayerPawn` 0)) (`SceneComponent.K2_GetComponentLocation` (`self.Cannon`))))) 90.0)) DeltaSeconds 1.0) false false))

(fn `UserConstructionScript`)