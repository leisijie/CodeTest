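; BP_GunBase is the base gun actor that fires a set of bullet generators, meant to be mounted on a BP_Car.
; Its construction script gathers all its BP_BulletGenerator components and, when its parent actor is a BP_Car, adds itself to that car's Guns array.
; Fire passes the BePlayer flag to every gathered generator; the event graph holds no active logic.
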(fn `Fire`
  (params (BePlayer :type Boolean))
  (for _array_element (`self.Generators`)
    (`/Game/Asset/Blueprints/Component/BP_BulletGenerator.Fire` _array_element BePlayer)))

(fn `UserConstructionScript`
  (set `self.Generators` (`self.K2_GetComponentsByClass` "/Game/Asset/Blueprints/Component/BP_BulletGenerator.BP_BulletGenerator_C"))
  (bind _asbp_car (cast `/Game/Asset/Blueprints/Car/BP_Car` (`self.GetParentActor`)))
  (`KismetArrayLibrary.Array_Add` (`/Game/Asset/Blueprints/Car/BP_Car.Guns` _asbp_car) self))