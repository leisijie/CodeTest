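; BP_Car is a car actor with a rotatable gun that moves within the game mode's play bounds.
; Drive clamps the requested move to MaxMoveRangeExtent, then applies X and Y as separate swept offsets.
; Each tick, AdjustRotation snaps only the car's height to the Sensor's result location, despite its name.
; GunRotation points GunCenter along a given direction, and Box hits spawn a CarCrush particle above the impact point.
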(event `self.ReceiveBeginPlay`
  (bind _asbp_game_mode (cast `/Game/Asset/Blueprints/GameMode/BP_GameMode` (`GameplayStatics.GetGameMode`)))
  (set `self.GameMode` _asbp_game_mode))

(event `self.ReceiveTick`
  (params (DeltaSeconds :type "Float (single-precision)"))
  (`self.AdjustRotation`))

(event `self.Box.OnComponentHit`
  (params (HitComponent :type "PrimitiveComponent Object Reference") (OtherActor :type "Actor Object Reference") (OtherComp :type "PrimitiveComponent Object Reference") (NormalImpulse :type "Vector Structure") (Hit :type "HitResult Structure (by ref)"))
  (`GameplayStatics.SpawnEmitterAtLocation` "/Game/Asset/Particles/CarCrush.CarCrush" (`KismetMathLibrary.MakeVector` (.x (`.ImpactPoint` (`GameplayStatics.BreakHitResult` Hit))) (.y (`.ImpactPoint` (`GameplayStatics.BreakHitResult` Hit))) (+ (.z (`.ImpactPoint` (`GameplayStatics.BreakHitResult` Hit))) 100.0))))

(event `Gun Rotation`
  (params (Direction :type "Vector Structure") (Angle :type "Float (double-precision)"))
  (`SceneComponent.K2_SetWorldRotation` (`self.GunCenter`) (`KismetMathLibrary.Conv_VectorToRotator` Direction) false false))

(fn `AdjustRotation`
  (locals (Degree :type "Float (double-precision)"))
  (bind _result (`/Game/Asset/Blueprints/Component/BP_Sensor.GetResult` (`self.Sensor`)))
  (`self.K2_SetActorLocation` (`KismetMathLibrary.MakeVector` (.x (`self.K2_GetActorLocation`)) (.y (`self.K2_GetActorLocation`)) (.z (`.Location` (`GameplayStatics.BreakHitResult` _result))))))

(fn `Drive`
  (params (RealMoveVector :type "Vector2D Structure"))
  (locals (X :type "Float (double-precision)") (Y :type "Float (double-precision)"))
  (bind (_x _y) (`KismetMathLibrary.BreakVector2D` RealMoveVector))
  (bind _x_2 (.x (`self.K2_GetActorLocation`)))
  (bind _y_2 (.y (`self.K2_GetActorLocation`)))
  (bind (_x_3 _y_3) (`KismetMathLibrary.BreakVector2D` (`/Game/Asset/Blueprints/GameMode/BP_GameMode.MaxMoveRangeExtent` (`self.GameMode`))))
  (if (> (`KismetMathLibrary.Abs` (+ _x_2 _x)) _x_3)
    (set `local.X` (* (`KismetMathLibrary.SignOfFloat` _x_2) (- _x_3 (`KismetMathLibrary.Abs` _x_2))))
    (else
      (set `local.X` _x)))
  (if (> (`KismetMathLibrary.Abs` (+ _y _y_2)) _y_3)
    (set `local.Y` (* (- _y_3 (`KismetMathLibrary.Abs` _y_2)) (`KismetMathLibrary.SignOfFloat` _y_2)))
    (else
      (set `local.Y` _y)))
  (`self.K2_AddActorWorldOffset` (`KismetMathLibrary.MakeVector` (`local.X`)) true)
  (`self.K2_AddActorWorldOffset` (`KismetMathLibrary.MakeVector` 0.0 (`local.Y`)) true))

(fn `UserConstructionScript`)