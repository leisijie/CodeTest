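; BP_Car_JustTrain is a train car Blueprint whose overrides are mostly empty, with blank DESTROY and GunInit.
; Its construction script only calls the parent.
; EachGunSet casts a child actor to BP_GunBase, enables player interpolation, disables destruction and appends it to a gun array, but its calls in GunInit are disconnected.
; CheckGuns removes array entries matching an unset value while iterating.
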(event `DESTROY`
  (params (InputPin :type "PrimitiveComponent Object Reference")))

(fn `CheckGuns`
  (params (Array :type "Array of /Game/Asset/Blueprints/Gun/BP_GunBase Object Reference"))
  (for (_array_element _array_index) Array
    (if (== _array_element null)
      (`KismetArrayLibrary.Array_Remove` Array _array_index))))

(fn `EachGunSet`
  (params (TargetArray :type "Array of /Game/Asset/Blueprints/Gun/BP_GunBase Object Reference (by ref)") (Object :type "Object Object Reference"))
  (bind _asbp_gun_base (cast `/Game/Asset/Blueprints/Gun/BP_GunBase` Object))
  (set `/Game/Asset/Blueprints/Gun/BP_GunBase.CanInterptoPlayer` true _asbp_gun_base)
  (set `/Game/Asset/Blueprints/Gun/BP_GunBase.CanDestroy` false _asbp_gun_base)
  (`KismetArrayLibrary.Array_Add` TargetArray _asbp_gun_base))

(fn `GunInit`)

(fn `UserConstructionScript`
  (`parent.UserConstructionScript`))