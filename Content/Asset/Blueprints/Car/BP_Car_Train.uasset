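; BP_Car_Train is a train vehicle carrying child-actor guns, with destructible parts and a full death sequence.
; On BeginPlay, GunInit sorts the weapons into five gun arrays, enabling each gun's interp-to-player flag and clearing its destroy flag.
; DESTROY blasts a given component away with physics and burst emitters, deletes it after a delay, then prunes empty gun entries.
; DeathCar applies a similar, larger blast to the Box before destroying the actor.
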(event `self.ReceiveBeginPlay`
  (`|ExecutionSequence`
    (:`then_0`
      (`parent.ReceiveBeginPlay`))
    (:`then_1`
      (`self.GunInit`))))

(event `self.ReceiveTick`
  (params (DeltaSeconds :type "Float (single-precision)"))
  (`parent.ReceiveTick` DeltaSeconds))

(event `DESTROY`
  (params (InputPin :type "PrimitiveComponent Object Reference"))
  (`|ExecutionSequence`
    (:`then_0`
      (`PrimitiveComponent.SetCollisionObjectType` InputPin "ECC_Visibility")
      (`PrimitiveComponent.SetSimulatePhysics` InputPin true)
      (`PrimitiveComponent.SetPhysicsLinearVelocity` InputPin (`KismetMathLibrary.MakeVector` 0.0 -10000.0) true "None")
      (`PrimitiveComponent.SetPhysicsAngularVelocityInDegrees` InputPin (`KismetMathLibrary.MakeVector` 0.0) true "None")
      (bind _returnvalue (`GameplayStatics.SpawnEmitterAttached` "/Game/BallisticsVFX/Burst_smoke.Burst_smoke" InputPin "None" (0.0 0.0 0.0) (struct) (5.0 5.0 5.0)))
      (bind _returnvalue_2 (`GameplayStatics.SpawnEmitterAttached` "/Game/BallisticsVFX/FXProps/Canister1/Particles/Burst.Burst" InputPin "None" (0.0 0.0 100.0) (struct) (10.0 10.0 10.0)))
      (`KismetSystemLibrary.Delay` 2.0)
      (`ActorComponent.K2_DestroyComponent` InputPin)
      (`ActorComponent.K2_DestroyComponent` _returnvalue_2)
      (`ActorComponent.K2_DestroyComponent` _returnvalue)
      (`self.CheckGuns` (`self.3-1guns`))
      (`self.CheckGuns` (`self.2-1guns`))
      (`self.CheckGuns` (`self.2-2guns`))
      (`self.CheckGuns` (`self.1-1guns`))
      (`self.CheckGuns` (`self.1-2guns`)))))

(event `self.DeathCar`
  (bind _box (`self.Box`))
  (`|ExecutionSequence`
    (:`then_0`
      (`PrimitiveComponent.SetCollisionObjectType` _box "ECC_Visibility")
      (`PrimitiveComponent.SetSimulatePhysics` _box true)
      (`PrimitiveComponent.SetPhysicsLinearVelocity` _box (`KismetMathLibrary.MakeVector` 0.0 -10000.0) true "None")
      (`PrimitiveComponent.SetPhysicsAngularVelocityInDegrees` _box (`KismetMathLibrary.MakeVector` 0.0) true "None")
      (bind _returnvalue (`GameplayStatics.SpawnEmitterAttached` "/Game/BallisticsVFX/Burst_smoke.Burst_smoke" _box "None" (0.0 0.0 0.0) (struct) (10.0 10.0 10.0)))
      (bind _returnvalue_2 (`GameplayStatics.SpawnEmitterAttached` "/Game/BallisticsVFX/FXProps/Canister1/Particles/Burst.Burst" _box "None" (0.0 0.0 0.0) (struct) (100.0 100.0 100.0)))
      (`KismetSystemLibrary.Delay` 3.0)
      (`ActorComponent.K2_DestroyComponent` _returnvalue)
      (`ActorComponent.K2_DestroyComponent` _returnvalue_2)
      (`self.K2_DestroyActor`))))

(fn `CheckGuns`
  (params (Array :type "Array of /Game/Asset/Blueprints/Gun/BP_GunBase Object Reference"))
  (for (_array_element _array_index) Array
    (if (== _array_element null)
      (`KismetArrayLibrary.Array_Remove` Array _array_index))))

(fn `EachGunSet`
  (params (TargetArray :type "Array of /Game/Asset/Blueprints/Gun/BP_GunBase Object Reference (by ref)") (Object :type "Object Object Reference"))
  (bind _asbp_gun_base (cast `/Game/Asset/Blueprints/Gun/BP_GunBase` Object))
  (set `/Game/Asset/Blueprints/Gun/BP_GunBase.CanInterptoPlayer` true _asbp_gun_base)
  (set `/Game/Asset/Blueprints/Gun/BP_GunBase.CanDestroy` false _asbp_gun_base)
  (`KismetArrayLibrary.Array_Add` TargetArray _asbp_gun_base))

(fn `GunInit`
  (`self.EachGunSet` (`self.3-1guns`) (`ChildActorComponent.ChildActor` (`self.Weapon`)))
  (`self.EachGunSet` (`self.3-1guns`) (`ChildActorComponent.ChildActor` (`self.Weapon1`)))
  (`self.EachGunSet` (`self.2-1guns`) (`ChildActorComponent.ChildActor` (`self.Weapon6`)))
  (`self.EachGunSet` (`self.2-1guns`) (`ChildActorComponent.ChildActor` (`self.Weapon3`)))
  (`self.EachGunSet` (`self.2-2guns`) (`ChildActorComponent.ChildActor` (`self.Weapon4`)))
  (`self.EachGunSet` (`self.2-2guns`) (`ChildActorComponent.ChildActor` (`self.Weapon5`)))
  (`self.EachGunSet` (`self.1-1guns`) (`ChildActorComponent.ChildActor` (`self.Weapon7`)))
  (`self.EachGunSet` (`self.1-1guns`) (`ChildActorComponent.ChildActor` (`self.Weapon9`)))
  (`self.EachGunSet` (`self.1-2guns`) (`ChildActorComponent.ChildActor` (`self.Weapon10`))))

(fn `UserConstructionScript`
  (`parent.UserConstructionScript`))