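; BP_Flight_test is a test Blueprint meant to fire a salvo of six missiles.
; Six near-identical fire graphs each spawn a Missile at a StaticMesh world transform, then wait briefly before returning.
; They are chained through their Completed outputs, but nothing triggers the chain.
; BeginPlay only runs a delay that leads nowhere, so no missiles spawn as wired.
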(event `self.ReceiveBeginPlay`
  (`KismetSystemLibrary.Delay` 7.0))

(fn `UserConstructionScript`)