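; Super is an actor in the Car folder that automatically fires BP_Bullet_Throw_SHIP projectiles in repeating bursts.
; After a startup delay on BeginPlay, a looped chain of Delay nodes spawns pairs of bullets in quick succession with a longer pause between pairs, with no exit condition.
; Each bullet spawns at the root component's current world location, without inheriting its rotation.
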(event `self.ReceiveTick`
  (params (DeltaSeconds :type "Float (single-precision)")))

(event `self.ReceiveBeginPlay`
  (`KismetSystemLibrary.Delay` 5.0)
  (`|SpawnActorFromClass` "/Game/Asset/Blueprints/EnemyBullet/BP_Bullet_Throw_SHIP.BP_Bullet_Throw_SHIP_C" (`KismetMathLibrary.Conv_VectorToTransform` (`SceneComponent.K2_GetComponentLocation` (`self.DefaultSceneRoot`))) "Undefined" "OverrideRootScale" null (0.0 1.0 0.0) null (struct) null :!label _label)
  (`KismetSystemLibrary.Delay` 0.2)
  (`|SpawnActorFromClass` "/Game/Asset/Blueprints/EnemyBullet/BP_Bullet_Throw_SHIP.BP_Bullet_Throw_SHIP_C" (`KismetMathLibrary.Conv_VectorToTransform` (`SceneComponent.K2_GetComponentLocation` (`self.DefaultSceneRoot`))) "Undefined" "OverrideRootScale" null (0.0 1.0 0.0) null (struct) null)
  (`KismetSystemLibrary.Delay` 0.8)
  (goto _label))

(fn `UserConstructionScript`)