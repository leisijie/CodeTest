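; Car platform actor that slides a skeletal mesh between Begin, Ready and End marker components, starting at Begin.
; GetREady snaps the mesh to End, moves it to Ready and sets the ready flag, while Start moves it to End on a timeline chosen by that flag.
; Leaving the Move volume with Show set replays Begin to End.
; Timelines lerp from the current location each update, so motion is non-linear.
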(event `self.ReceiveBeginPlay`
  (`SceneComponent.K2_SetWorldLocation` (`self.SkeletalMesh`) (`SceneComponent.K2_GetComponentLocation` (`self.Begin`)) false false))

(event `Start`
  (bind _skeletalmesh (`self.SkeletalMesh`))
  (bind _skeletalmesh_2 (`self.SkeletalMesh`))
  (if (`self.Ready?`)
    (bind (_direction _time) (`Timeline|Timeline_2` :!via `PlayFromStart`)
      (:`Update`
        (`SceneComponent.K2_SetWorldLocation` _skeletalmesh_2 (`KismetMathLibrary.VLerp` (`SceneComponent.K2_GetComponentLocation` _skeletalmesh_2) (`SceneComponent.K2_GetComponentLocation` (`self.End`)) _time) false false)))
    (else
      (bind (_direction_2 _time_2) (`Timeline|Timeline_0` :`NewTime` 0.0 :!via `PlayFromStart`)
        (:`Update`
          (`SceneComponent.K2_SetWorldLocation` _skeletalmesh (`KismetMathLibrary.VLerp` (`SceneComponent.K2_GetComponentLocation` _skeletalmesh) (`SceneComponent.K2_GetComponentLocation` (`self.End`)) _time_2) false false))))))

(event `GetREady`
  (bind _skeletalmesh (`self.SkeletalMesh`))
  (`SceneComponent.K2_SetWorldLocation` (`self.SkeletalMesh`) (`SceneComponent.K2_GetComponentLocation` (`self.End`)) false false)
  (bind (_direction _time) (`Timeline|Timeline_1` :!via `PlayFromStart`)
    (:`Update`
      (`SceneComponent.K2_SetWorldLocation` _skeletalmesh (`KismetMathLibrary.VLerp` (`SceneComponent.K2_GetComponentLocation` _skeletalmesh) (`SceneComponent.K2_GetComponentLocation` (`self.Ready`)) _time) false false))
    (:`Finished`
      (set `self.Ready?` true))))

(event `self.move.OnComponentEndOverlap`
  (params (OverlappedComponent :type "PrimitiveComponent Object Reference") (OtherActor :type "Actor Object Reference") (OtherComp :type "PrimitiveComponent Object Reference") (OtherBodyIndex :type Integer))
  (bind _skeletalmesh (`self.SkeletalMesh`))
  (if (`self.Show?`)
    (`SceneComponent.K2_SetWorldLocation` (`self.SkeletalMesh`) (`SceneComponent.K2_GetComponentLocation` (`self.Begin`)) false false)
    (bind (_direction _time) (`Timeline|Timeline_3` :!via `PlayFromStart`)
      (:`Update`
        (`SceneComponent.K2_SetWorldLocation` _skeletalmesh (`KismetMathLibrary.VLerp` (`SceneComponent.K2_GetComponentLocation` _skeletalmesh) (`SceneComponent.K2_GetComponentLocation` (`self.End`)) _time) false false)))))

(fn `UserConstructionScript`)