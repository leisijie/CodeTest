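; Enemy Blueprint that continuously fires short bursts of BP_Bullet_Enemy from its Arrow component, starting at BeginPlay.
; Each bullet takes the Arrow's transform and forward vector plus a tail particle system.
; A custom for-loop macro with Next and Break inputs lets a Delay space shots within each burst.
; On completion, a longer pause leads into the Shoot event, which re-enters the loop to repeat the burst.
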(event `self.ReceiveBeginPlay`
  (bind _arrow (`self.Arrow`))
  (`parent.ReceiveBeginPlay`)
  (`self.NewMacro_0` 0 4 :!label _label
    (:`Loop`
      (`|SpawnActorFromClass` "/Game/Asset/Blueprints/BP_Bullet_Enemy.BP_Bullet_Enemy_C" (`SceneComponent.K2_GetComponentToWorld` _arrow) "Undefined" "OverrideRootScale" null (`SceneComponent.GetForwardVector` _arrow) "/Game/Asset/Particles/PS_bullettail.PS_bullettail" null)
      (`KismetSystemLibrary.Delay` 0.1)
      (goto _label :!via `Next`))
    (:`Complete`
      (`KismetSystemLibrary.Delay` 1.0)
      (`self.Shoot`))))

(event `Shoot`
  (goto _label))

(fn `UserConstructionScript`
  (`parent.UserConstructionScript`))