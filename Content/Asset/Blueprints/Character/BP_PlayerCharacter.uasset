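; Player character that drives a BP_Car or BP_Moto, taking damage and forwarding HP and ammo events to its HUD and bullet-notice widgets.
; On BeginPlay it detaches the child-actor vehicle, attaches itself to it, sets gun collision, then installs data-table starting guns.
; A looping delay macro charges LAGAAN power into gas cans, which ready the launcher on Tick.
; Gun upgrades and swaps are passed to the player controller.
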(event `BeHit`
  (params (Damage :type Integer))
  ;[1 1 1] HIT
  (set `self.HP` (- (`self.HP`) Damage))
  (`/Game/Asset/Widget/Main_Controller.Been Hit` (`self.HPWidget`) Damage))

(event `self.ReceiveBeginPlay`
  (`|ExecutionSequence`
    (:`then_0`
      ;[1 1 1] Init
      (`self.InitCar`)
      (`self.InitGunCollision`)
      (set `self.HP` (`self.Max HP`))
      (`self.InitUI`))
    (:`then_1`
      (`self.AddGas`))
    (:`then_2`
      (`KismetSystemLibrary.Delay` 0.1)
      (`self.SwitchGunOpen`))))

(event `AddGas`
  (bind _maxgascan (`self.maxgascan`))
  (bind _maxgascan_2 (`self.maxgascan`))
  (`|ExecutionSequence`
    (:`then_0`
      ;[1 1 1] Add Gas
      (`self.Continue` 0.05 :!label _label
        (:`Out`
          (bind _output_get (set `self.LAGAANPower` (+ (`self.LAGAANPower`) 10.0)))
          (`/Game/Asset/Widget/Main_Controller.Gascheck` (`self.HPWidget`))
          (if (>= _output_get (`self.maxLagaanpower`))
            (set `self.LAGAANPower` 0.0)
            (bind _output_get_2 (set `self.Gascan` (+ (`self.Gascan`) 1)))
            (if (>= _output_get_2 _maxgascan)
              (set `self.Gascan` _maxgascan)
              (`/Game/Asset/Widget/Main_Controller.Gascheck` (`self.HPWidget`))
              (`|ExecutionSequence`
                (:`then_0`
                  (goto _label :!via `TurnOff`))
                (:`then_1`
                  (goto _label_2 :!via `Close`))))))))
    (:`then_1`
      (goto _label_2 :!via `Open`))))

(event `bulletGas`
  (params (BulletGas :type "Float (double-precision)"))
  (bind _maxgascan (`self.maxgascan`))
  (`/Engine/EditorBlueprintResources/StandardMacros.Gate` true :!label _label_2
    (:`Exit`
      (bind _output_get (set `self.LAGAANPower` (+ (`self.LAGAANPower`) BulletGas)))
      (`/Game/Asset/Widget/Main_Controller.Gascheck` (`self.HPWidget`))
      (if (>= _output_get (`self.maxLagaanpower`))
        (set `self.LAGAANPower` 0.0)
        (bind _output_get_2 (set `self.Gascan` (+ (`self.Gascan`) 1)))
        (if (>= _output_get_2 _maxgascan)
          (set `self.Gascan` _maxgascan)
          (`/Game/Asset/Widget/Main_Controller.Gascheck` (`self.HPWidget`))
          (`|ExecutionSequence`
            (:`then_0`
              (goto _label :!via `TurnOff`))
            (:`then_1`
              (goto _label_2 :!via `Close`))))))))

(event `self.ReceiveTick`
  (params (DeltaSeconds :type "Float (single-precision)"))
  (bind _aslagaanluncher (cast `/Game/Asset/Blueprints/Follower/LAGAANLuncher` (`ChildActorComponent.ChildActor` (`/Game/Asset/Blueprints/Car/BP_Car.LAGAAN` (`self.Car`)))))
  (if (> (`self.Gascan`) 0)
    (set `/Game/Asset/Blueprints/Follower/LAGAANLuncher.Ready?` true _aslagaanluncher)
    (else
      (set `/Game/Asset/Blueprints/Follower/LAGAANLuncher.Ready?` false _aslagaanluncher))))

(event `/Game/Asset/Blueprints/IF_Explosion.BeExploded`
  (params (Damage :type Integer))
  (`self.BeHit` Damage))

(event `Switch`
  (params (`Cur Dir` :type "/Game/Asset/Blueprints/Enum/Enum_GunDirection Enum" :default "NewEnumerator0") (`Pre Dir` :type "/Game/Asset/Blueprints/Enum/Enum_GunDirection Enum" :default "NewEnumerator0") (Gun :type "/Game/Asset/Blueprints/Gun/BP_GunBase Object Reference"))
  ;[1 1 1] UI
  (`/Game/Asset/Widget/BulletNotice.Switch Start` (`self.Notice`) `Cur Dir` `Pre Dir` Gun))

(event `Check Ammo`
  (params (`Cur/Max` :type "Float (double-precision)") (Dir :type "/Game/Asset/Blueprints/Enum/Enum_GunDirection Enum" :default "NewEnumerator0"))
  ;[1 1 1] UI
  (`/Game/Asset/Widget/BulletNotice.Use Ammo` (`self.Notice`) `Cur/Max` Dir))

(event `Restore`
  (params (Dir :type "/Game/Asset/Blueprints/Enum/Enum_GunDirection Enum" :default "NewEnumerator0") (Delay :type "Float (double-precision)"))
  ;[1 1 1] UI
  (`/Game/Asset/Widget/BulletNotice.Restore` (`self.Notice`) Dir Delay))

(fn `AddLAGGANPower`
  (params (Gas :type "Float (double-precision)"))
  (`/Engine/EditorBlueprintResources/StandardMacros.Gate` true :!label _label
    (:`Exit`
      (bind _output_get (set `self.LAGAANPower` (+ Gas (`self.LAGAANPower`))))
      (if (> _output_get (`self.maxLagaanpower`))
        (set `self.LAGAANPower` 0.0)
        (bind _output_get_2 (set `self.Gascan` (+ (`self.Gascan`) 1)))
        (if (== _output_get_2 (`self.maxgascan`))
          (goto _label :!via `Close`))))))

(fn `InitCar`
  (bind _childactor (`ChildActorComponent.ChildActor` (`self.ChildActor`)))
  (bind _asbp_car (cast `/Game/Asset/Blueprints/Car/BP_Car` _childactor))
  (set `/Game/Asset/Blueprints/Car/BP_Car.Driver` self _asbp_car)
  (set `self.Car` _asbp_car)
  (`KismetArrayLibrary.Array_Set` (`Actor.Tags` _asbp_car) 0 "Player")
  (`self.K2_DetachFromActor` _childactor "KeepWorld" "KeepWorld" "KeepWorld")
  (`self.K2_AttachToActor` self _childactor "None" "KeepWorld" "KeepRelative" "KeepWorld" true)
  (bind _asbp_moto (cast `/Game/Asset/Blueprints/Car/BP_Moto` _childactor))
  (bind _output_get (set `self.Car` _asbp_moto))
  (bind _asanim_b_moto (cast `/Game/Asset/Animation/MOTO/AnimB_Moto` (`SkeletalMeshComponent.GetAnimInstance` (`/Game/Asset/Blueprints/Car/BP_Car.Motor` _output_get))))
  (set `/Game/Asset/Animation/MOTO/AnimB_Moto.IsPlayer` true _asanim_b_moto))

(fn `InitGunCollision`
  (for _array_element (`/Game/Asset/Blueprints/Car/BP_Car.Guns` (`self.Car`))
    (`self.SetGunCollision` _array_element)))

(fn `InitUI`
  (bind _returnvalue (`GameplayStatics.GetPlayerController` 0))
  (bind _returnvalue_2 (`|CreateWidget` (`self.HPWidgetClass`) _returnvalue))
  (bind _output_get (set `self.HPWidget` _returnvalue_2))
  (set `/Game/Asset/Widget/Main_Controller.Owner` self _output_get)
  (`UserWidget.AddToPlayerScreen` _output_get 0)
  (bind _returnvalue_3 (`|CreateWidget` "/Game/Asset/Widget/BulletNotice.BulletNotice_C" _returnvalue))
  (bind _output_get_2 (set `self.Notice` _returnvalue_3))
  (`WidgetComponent.SetWidget` (`self.Widget`) _output_get_2))

(fn `SetGunCollision`
  (params (Gun :type "/Game/Asset/Blueprints/Gun/BP_GunBase Object Reference"))
  (`PrimitiveComponent.SetCollisionProfileName` (`/Game/Asset/Blueprints/Gun/BP_GunBase.GunMesh` Gun) "PlayerGun"))

(fn `SwitchGunOpen`
  (locals (Left :type "/Game/Asset/Blueprints/Gun/BP_GunBase Class Reference") (Right :type "/Game/Asset/Blueprints/Gun/BP_GunBase Class Reference"))
  (bind _returnvalue (`|GetDataTableRow` "/Game/Asset/Blueprints/DataTable/Start_Test_DataTable.Start_Test_DataTable" "Basic")
    (:`then`
      (bind ((`left_Gun_8_8504590D4C6B68D0FD1EE2AE241163E5` _left_gun) (`Right_Gun_9_B06B7106460D62073B5FFFAF95632C1C` _right_gun) (`Weapon_Trinket_14_48F9F69A423A8F1DEBDF898066BD4706` _weapon_trinket)) (break `/Game/Asset/Blueprints/GoodToGoTable` _returnvalue))
      (bind _structout (setmembers `/Game/Asset/Blueprints/GoodToGoTable` :`StructRef` (`self.TrinketStor`) :`Weapon_Trinket` _weapon_trinket))
      (set `self.TrinketStor` _structout)
      (`|ExecutionSequence`
        (:`then_0`
          (bind _returnvalue_2 (`|GetDataTableRow` "/Game/Asset/Blueprints/DataTable/WeaponTable.WeaponTable" _left_gun)
            (:`then`
              (set `local.Left` (`.WeaponClass_17_32FEF60C48EEA0C93F3519AD3CBF7A61` (break `/Game/Asset/Blueprints/Struct/WeaponIconAndClass` _returnvalue_2))))))
        (:`then_1`
          (bind _returnvalue_3 (`|GetDataTableRow` "/Game/Asset/Blueprints/DataTable/WeaponTable.WeaponTable" _right_gun)
            (:`then`
              (set `local.Right` (`.WeaponClass_17_32FEF60C48EEA0C93F3519AD3CBF7A61` (break `/Game/Asset/Blueprints/Struct/WeaponIconAndClass` _returnvalue_3))))))
        (:`then_2`
          (for _array_element (`/Game/Asset/Blueprints/Car/BP_Car.Guns` (`self.Car`))
            (if (`|EnumEquality` (`/Game/Asset/Blueprints/Gun/BP_GunBase.Dir` _array_element) "NewEnumerator3")
              (break)))
          (`self.Set StartGun` _array_element "NewEnumerator3" (`local.Right`)
            (:`Out`
              (for _array_element_2 (`/Game/Asset/Blueprints/Car/BP_Car.Guns` (`self.Car`))
                (if (`|EnumEquality` (`/Game/Asset/Blueprints/Gun/BP_GunBase.Dir` _array_element_2) "NewEnumerator2")
                  (break)))
              (`self.Set StartGun` _array_element_2 "NewEnumerator2" (`local.Left`)))))))))

(fn `UpgradeGun`
  (params (GunDirection :type "/Game/Asset/Blueprints/Enum/Enum_GunDirection Enum" :default "NewEnumerator0"))
  (locals (ChangedGun :type "/Game/Asset/Blueprints/Gun/BP_GunBase Object Reference"))
  (for _array_element (`/Game/Asset/Blueprints/Car/BP_Car.Guns` (`self.Car`))
    (if (`|EnumEquality` (`/Game/Asset/Blueprints/Gun/BP_GunBase.Dir` _array_element) GunDirection)
      (set `local.ChangedGun` _array_element)
      (break)))
  (bind _gunparent (`/Game/Asset/Blueprints/Gun/BP_GunBase.Upgrade` (`local.ChangedGun`)))
  (if (`KismetSystemLibrary.IsValid` _gunparent)
    (bind _asbp_hyper_gun_base (cast `/Game/Asset/Blueprints/Gun/BP_HyperGunBase` (`ChildActorComponent.ChildActor` _gunparent)))
    (set `/Game/Asset/Blueprints/Gun/BP_GunBase.Dir` GunDirection _asbp_hyper_gun_base)
    (bind _asbp_player_controller (cast `/Game/Asset/Blueprints/BP_PlayerController` (`GameplayStatics.GetPlayerController` 0)))
    (`/Game/Asset/Blueprints/BP_PlayerController.ReplaceGunAndWidget` _asbp_player_controller _asbp_hyper_gun_base)))

(fn `UserConstructionScript`)