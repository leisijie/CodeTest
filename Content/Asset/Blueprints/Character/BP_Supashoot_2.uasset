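; Enemy shooter that fires repeating bursts of BP_Bullet_Enemy and grows more aggressive as its Health drops.
; BeginPlay starts a self-repeating Shoot cycle that picks one, two or four arrow muzzles by Health, spacing shots with a custom latent loop macro.
; Tick watches separate Health thresholds, each firing once to play explosion effects, hide mesh parts and set the pause between bursts.
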(event `self.ReceiveBeginPlay`
  (bind _arrow (`self.Arrow`))
  (bind _arrow_2 (`self.Arrow`))
  (bind _arrow_3 (`self.Arrow`))
  (bind _arrow3 (`self.Arrow3`))
  (bind _arrow3_2 (`self.Arrow3`))
  (bind _arrow2 (`self.Arrow2`))
  (bind _arrow1 (`self.Arrow1`))
  (`parent.ReceiveBeginPlay`)
  (if (> (`KismetMathLibrary.Conv_IntToDouble` (`self.Health`)) 400.0) :!label _label
    (`self.NewMacro_0` 0 4 :!label _label_2
      (:`Loop`
        (`|SpawnActorFromClass` "/Game/Asset/Blueprints/Bullet/BP_Bullet_Enemy.BP_Bullet_Enemy_C" (`SceneComponent.K2_GetComponentToWorld` _arrow) "Undefined" "OverrideRootScale" null (`SceneComponent.GetForwardVector` _arrow) "/Game/Asset/Particles/PS_bullettail.PS_bullettail" null)
        (`KismetSystemLibrary.Delay` 0.1)
        (goto _label_2 :!via `Next`))
      (:`Complete`
        (`KismetSystemLibrary.Delay` (`self.Delaytime`))
        (`self.Shoot`)))
    (elif (> (`KismetMathLibrary.Conv_IntToDouble` (`self.Health`)) 200.0)
      (`|ExecutionSequence`
        (:`then_0`
          (`self.NewMacro_0` 0 4 :!label _label_3
            (:`Loop`
              (`|SpawnActorFromClass` "/Game/Asset/Blueprints/Bullet/BP_Bullet_Enemy.BP_Bullet_Enemy_C" (`SceneComponent.K2_GetComponentToWorld` _arrow_2) "Undefined" "OverrideRootScale" null (`SceneComponent.GetForwardVector` _arrow_2) "/Game/Asset/Particles/PS_bullettail.PS_bullettail" null)
              (`KismetSystemLibrary.Delay` 0.1)
              (goto _label_3 :!via `Next`))
            (:`Complete`
              (`KismetSystemLibrary.Delay` (`self.Delaytime`))
              (`self.Shoot`))))
        (:`then_1`
          (`self.NewMacro_0` 0 4 :!label _label_4
            (:`Loop`
              (`|SpawnActorFromClass` "/Game/Asset/Blueprints/Bullet/BP_Bullet_Enemy.BP_Bullet_Enemy_C" (`SceneComponent.K2_GetComponentToWorld` _arrow3) "Undefined" "OverrideRootScale" null (`SceneComponent.GetForwardVector` _arrow3) "/Game/Asset/Particles/PS_bullettail.PS_bullettail" null)
              (`KismetSystemLibrary.Delay` 0.1)
              (goto _label_4 :!via `Next`))
            (:`Complete`
              (`KismetSystemLibrary.Delay` (`self.Delaytime`))
              (`self.Shoot`)))))
      (else
        (`|ExecutionSequence`
          (:`then_0`
            (`self.NewMacro_0` 0 4 :!label _label_5
              (:`Loop`
                (`|SpawnActorFromClass` "/Game/Asset/Blueprints/Bullet/BP_Bullet_Enemy.BP_Bullet_Enemy_C" (`SceneComponent.K2_GetComponentToWorld` _arrow_3) "Undefined" "OverrideRootScale" null (`SceneComponent.GetForwardVector` _arrow_3) "/Game/Asset/Particles/PS_bullettail.PS_bullettail" null)
                (`KismetSystemLibrary.Delay` 0.1)
                (goto _label_5 :!via `Next`))
              (:`Complete`
                (`KismetSystemLibrary.Delay` (`self.Delaytime`))
                (`self.Shoot`))))
          (:`then_1`
            (`self.NewMacro_0` 0 4 :!label _label_6
              (:`Loop`
                (`|SpawnActorFromClass` "/Game/Asset/Blueprints/Bullet/BP_Bullet_Enemy.BP_Bullet_Enemy_C" (`SceneComponent.K2_GetComponentToWorld` _arrow3_2) "Undefined" "OverrideRootScale" null (`SceneComponent.GetForwardVector` _arrow3_2) "/Game/Asset/Particles/PS_bullettail.PS_bullettail" null)
                (`KismetSystemLibrary.Delay` 0.1)
                (goto _label_6 :!via `Next`))
              (:`Complete`
                (`KismetSystemLibrary.Delay` (`self.Delaytime`))
                (`self.Shoot`))))
          (:`then_2`
            (`self.NewMacro_0` 0 4 :!label _label_7
              (:`Loop`
                (`|SpawnActorFromClass` "/Game/Asset/Blueprints/Bullet/BP_Bullet_Enemy.BP_Bullet_Enemy_C" (`SceneComponent.K2_GetComponentToWorld` _arrow2) "Undefined" "OverrideRootScale" null (`SceneComponent.GetForwardVector` _arrow2) "/Game/Asset/Particles/PS_bullettail.PS_bullettail" null)
                (`KismetSystemLibrary.Delay` 0.1)
                (goto _label_7 :!via `Next`))
              (:`Complete`
                (`KismetSystemLibrary.Delay` (`self.Delaytime`))
                (`self.Shoot`))))
          (:`then_3`
            (`self.NewMacro_0` 0 4 :!label _label_8
              (:`Loop`
                (`|SpawnActorFromClass` "/Game/Asset/Blueprints/Bullet/BP_Bullet_Enemy.BP_Bullet_Enemy_C" (`SceneComponent.K2_GetComponentToWorld` _arrow1) "Undefined" "OverrideRootScale" null (`SceneComponent.GetForwardVector` _arrow1) "/Game/Asset/Particles/PS_bullettail.PS_bullettail" null)
                (`KismetSystemLibrary.Delay` 0.1)
                (goto _label_8 :!via `Next`))
              (:`Complete`
                (`KismetSystemLibrary.Delay` (`self.Delaytime`))
                (`self.Shoot`)))))))))

(event `Shoot`
  (goto _label))

(event `self.ReceiveTick`
  (params (DeltaSeconds :type "Float (single-precision)"))
  (bind _returnvalue (`SceneComponent.K2_GetComponentLocation` (`self.Arrow`)))
  (bind _returnvalue_2 (`SceneComponent.K2_GetComponentLocation` (`self.Arrow`)))
  (`parent.ReceiveTick` DeltaSeconds)
  (if (> (`KismetMathLibrary.Conv_IntToDouble` (`self.Health`)) 600.0)
    _
    (elif (> (`KismetMathLibrary.Conv_IntToDouble` (`self.Health`)) 300.0)
      (`/Engine/EditorBlueprintResources/StandardMacros.DoOnce` false
        (:`Completed`
          (`GameplayStatics.SpawnEmitterAtLocation` "/Game/BallisticsVFX/Particles/Explosive/Explosion_Frag_small.Explosion_Frag_small" _returnvalue_2)
          (`GameplayStatics.SpawnEmitterAtLocation` "/Game/Asset/Particles/Jump.Jump" _returnvalue_2)
          (set `self.Delaytime` 0.5)
          (`SceneComponent.SetVisibility` (`self.StaticMesh3`) false false)))
      (else
        (`/Engine/EditorBlueprintResources/StandardMacros.DoOnce` false
          (:`Completed`
            (`GameplayStatics.SpawnEmitterAtLocation` "/Game/BallisticsVFX/Particles/Explosive/Explosion_Frag_small.Explosion_Frag_small" _returnvalue)
            (`GameplayStatics.SpawnEmitterAtLocation` "/Game/Asset/Particles/Jump.Jump" _returnvalue)
            (set `self.Delaytime` 0.2)
            (`SceneComponent.SetVisibility` (`self.StaticMesh2`) false false)
            (`SceneComponent.SetVisibility` (`self.StaticMesh1`) false false)))))))

(fn `UserConstructionScript`
  (`parent.UserConstructionScript`))