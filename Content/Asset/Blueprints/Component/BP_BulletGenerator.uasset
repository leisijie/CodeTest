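; BP_BulletGenerator is a component that spawns player or enemy bullets at its own world transform.
; Fire picks the bullet class from a BePlayer flag, passes in the component's local +Y axis as forward vector plus a particle system, and returns the bullet.
; Only player shots also spawn a gun effect emitter.
; UseNothing spawns just a half-scale smoke emitter, with no bullet.
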(fn `Fire`
  (params (BePlayer :type Boolean))
  (returns (Bullet :type "/Game/Asset/Blueprints/Playerbullet/BP_Bullet_Player Object Reference"))
  (bind _bulletparticle (`self.BulletParticle`))
  (bind _returnvalue (`KismetMathLibrary.MakeTransform` (.location (`self.K2_GetComponentToWorld`)) (.rotation (`self.K2_GetComponentToWorld`))))
  (bind _returnvalue_2 (`KismetMathLibrary.TransformDirection` _returnvalue (`KismetMathLibrary.MakeVector` 0.0 1.0)))
  (if BePlayer
    (bind _returnvalue_3 (`|SpawnActorFromClass` (`self.Player BUllet Type`) _returnvalue "Undefined" "OverrideRootScale" null _returnvalue_2 _bulletparticle null))
    (`GameplayStatics.SpawnEmitterAtLocation` (`self.Gunsffect`) (.location _returnvalue) (struct :`Roll` 90.0) (.scale _returnvalue))
    (return _returnvalue_3)
    (else
      (bind _returnvalue_4 (`|SpawnActorFromClass` (`self.EnemyBulletType`) _returnvalue "Undefined" "OverrideRootScale" null _returnvalue_2 _bulletparticle null))
      (return _returnvalue_4))))

(fn `Use Nothing`
  (`GameplayStatics.SpawnEmitterAtLocation` "/Game/BallisticsVFX/Particles/Mothing_but_smoke.Mothing_but_smoke" (.location (`KismetMathLibrary.MakeTransform` (.location (`self.K2_GetComponentToWorld`)) (.rotation (`self.K2_GetComponentToWorld`)))) (.rotation (`KismetMathLibrary.MakeTransform` (.location (`self.K2_GetComponentToWorld`)) (.rotation (`self.K2_GetComponentToWorld`)))) (0.5 0.5 0.5)))