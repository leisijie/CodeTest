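; BP_Gun is a component that fires player or enemy bullets from its owning actor.
; On BeginPlay it caches the Arrow's relative location as the muzzle offset, only if the owner is a BP_PlayerCharacter.
; Fire uses a Player flag to pick the bullet class, spawning it at owner location plus that unrotated offset and passing AimDirection as its forward vector.
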(event `self.ReceiveBeginPlay`
  (bind _asbp_player_character (cast `/Game/Asset/Blueprints/Character/BP_PlayerCharacter` (`self.GetOwner` self)))
  (set `self.FirePositionRelativeToActor` (`SceneComponent.RelativeLocation` (`/Game/Asset/Blueprints/Character/BP_PlayerCharacter.Arrow` _asbp_player_character))))

(fn `Fire`
  (params (Player :type Boolean) (AimDirection :type "Vector Structure"))
  (if Player
    (`|SpawnActorFromClass` "/Game/Asset/Blueprints/BP_Bullet_Player.BP_Bullet_Player_C" (`KismetMathLibrary.Conv_VectorToTransform` (+ (`Actor.K2_GetActorLocation` (`self.GetOwner` self)) (`self.FirePositionRelativeToActor`))) "Undefined" "OverrideRootScale" null AimDirection null)
    (else
      (`|SpawnActorFromClass` "/Game/Asset/Blueprints/BP_Bullet_Enemy.BP_Bullet_Enemy_C" (`KismetMathLibrary.Conv_VectorToTransform` (+ (`Actor.K2_GetActorLocation` (`self.GetOwner` self)) (`self.FirePositionRelativeToActor`))) "Undefined" "OverrideRootScale" null AimDirection null))))