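; BP_Sensor is a scene component that probes for whatever lies below it and supplies the hit result on demand.
; GetResult calls UpdataData, which draws a debug line and traces a custom channel along local down, reaching twice the component's relative Z.
; Each call stores the new hit but outputs the previous call's stored one, returning explicitly only when the current trace hits.
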(fn `GetResult`
  (returns (Result :type "HitResult Structure"))
  (bind _lastframedata (`self.UpdataData`))
  (return _lastframedata))

(fn `UpdataData`
  (returns (LastFrameData :type "HitResult Structure"))
  (locals (OutputData :type "HitResult Structure"))
  (bind _returnvalue (`self.K2_GetComponentLocation`))
  (bind _returnvalue_2 (+ _returnvalue (* (`KismetMathLibrary.TransformDirection` (`self.K2_GetComponentToWorld`) (0.0 0.0 -1.0)) (* (.z (`self.RelativeLocation`)) 2.0))))
  (set `local.OutputData` (`self.LastFrameData`))
  (`KismetSystemLibrary.DrawDebugLine` _returnvalue _returnvalue_2 (struct :`R` 0.318721 :`G` 0.10496 :`B` 0.9625 :`A` 1.0) 0.0 10.0)
  (bind (_outhit _returnvalue_3) (`KismetSystemLibrary.LineTraceSingle` _returnvalue _returnvalue_2 "TraceTypeQuery3"))
  (set `self.LastFrameData` _outhit)
  (if _returnvalue_3
    (return (`local.OutputData`))))