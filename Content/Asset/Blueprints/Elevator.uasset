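; Elevator actor that moves its ELE component between the UP and DOWN marker positions when something overlaps UP1.
; On overlap it chooses the direction from ELE's height relative to DOWN, then a DoOnce starts a looping timer running Move.
; Move offsets ELE vertically by a fixed step, snaps it to the target marker on arrival and clears the timer.
; Ending the overlap resets the DoOnce and prints a debug string.
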(event `self.UP1.OnComponentBeginOverlap`
  (params (OverlappedComponent :type "PrimitiveComponent Object Reference") (OtherActor :type "Actor Object Reference") (OtherComp :type "PrimitiveComponent Object Reference") (OtherBodyIndex :type Integer) (bFromSweep :type Boolean) (SweepResult :type "HitResult Structure (by ref)"))
  (if (> (.z (`SceneComponent.K2_GetComponentLocation` (`self.ELE`))) (.z (`SceneComponent.K2_GetComponentLocation` (`self.DOWN`))))
    (set `self.Goup` false)
    (else
      (set `self.Goup` true)))
  (`/Engine/EditorBlueprintResources/StandardMacros.DoOnce` false :!label _label
    (:`Completed`
      (bind _returnvalue (`KismetSystemLibrary.K2_SetTimer` null "move" 0.0157 true)))))

(event `Stop`
  (`KismetSystemLibrary.K2_ClearAndInvalidateTimerHandle` (stale `self.UP1.OnComponentBeginOverlap` _returnvalue)))

(event `self.UP1.OnComponentEndOverlap`
  (params (OverlappedComponent :type "PrimitiveComponent Object Reference") (OtherActor :type "Actor Object Reference") (OtherComp :type "PrimitiveComponent Object Reference") (OtherBodyIndex :type Integer))
  (`KismetSystemLibrary.PrintString` "Hello")
  (goto _label :!via `Reset`))

(fn `move`
  (bind _ele (`self.ELE`))
  (bind _z (.z (`SceneComponent.K2_GetComponentLocation` (`self.UP`))))
  (bind _z_2 (.z (`SceneComponent.K2_GetComponentLocation` (`self.DOWN`))))
  (bind _z_3 (.z (`SceneComponent.K2_GetComponentLocation` _ele)))
  (if (`self.Goup`)
    (`SceneComponent.K2_AddLocalOffset` (`self.ELE`) (0.0 0.0 5.0) false false)
    (if (>= _z_3 _z)
      (`SceneComponent.K2_SetWorldLocation` _ele (`KismetMathLibrary.MakeVector` (.x (`SceneComponent.K2_GetComponentLocation` (`self.UP`))) (.y (`SceneComponent.K2_GetComponentLocation` (`self.UP`))) _z) false false)
      (`self.Stop` :!label _label))
    (else
      (`SceneComponent.K2_AddLocalOffset` (`self.ELE`) (0.0 0.0 -5.0) false false)
      (if (<= _z_3 _z_2)
        (`SceneComponent.K2_SetWorldLocation` _ele (`KismetMathLibrary.MakeVector` (.x (`SceneComponent.K2_GetComponentLocation` (`self.DOWN`))) (.y (`SceneComponent.K2_GetComponentLocation` (`self.DOWN`))) _z_2) false false)
        (goto _label)))))

(fn `UserConstructionScript`)