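; Elevator actor that detects a pawn above it, disables that pawn's input and starts descending.
; From BeginPlay, a looping timer runs Detect, box-tracing for Pawns upward from the static mesh with debug drawing on.
; A hit clears the detection timer and starts a second looping timer that nudges the mesh along local negative Z, with no stop condition.
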(event `self.ReceiveBeginPlay`
  (`self.Start Detect`))

(event `Start Detect`
  (bind _returnvalue (`KismetSystemLibrary.K2_SetTimer` null "Detect" 0.02 true)))

(event `Start Move`
  (`KismetSystemLibrary.K2_ClearAndInvalidateTimerHandle` (stale `Start Detect` _returnvalue))
  (`KismetSystemLibrary.K2_SetTimer` null "Move" 0.017 true))

(fn `Detect`
  (bind _returnvalue (`SceneComponent.K2_GetComponentLocation` (`self.StaticMesh`)))
  (bind (_outhit _returnvalue_2) (`KismetSystemLibrary.BoxTraceSingleForObjects` :`Start` _returnvalue :`End` (`KismetMathLibrary.MakeVector` (.x _returnvalue) (.y _returnvalue) (+ (.z _returnvalue) 1000.0)) :`HalfSize` (150.0 150.0 150.0) :`ObjectTypes` (`|MakeArray` "ObjectTypeQuery3" :!type "EObjectTypeQuery Enum") :`DrawDebugType` "ForDuration" :`DrawTime` 1.0))
  (if _returnvalue_2
    (`self.DisableInput` (`.HitActor` (`GameplayStatics.BreakHitResult` _outhit)) (`GameplayStatics.GetPlayerController` 0))
    (`self.Start Move`)))

(fn `Move`
  (`SceneComponent.K2_AddLocalOffset` (`self.StaticMesh`) (0.0 0.0 -2.0) false false))

(fn `UserConstructionScript`)