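; Train boss that shuttles along the Y axis and loses carriages as its health drops through three stages.
; A looping timer moves the BP_Car_Train child actor toward a point oscillating around BeginPos.
; CheckHealth destroys a box at each health threshold, shifts BeginPos along Y and switches the Train_Controller AI to its next phase.
; Named attack events pass the train's per-stage gun arrays to AttackInputGuns.
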(event `YouDang`
  (bind _train (`self.Train`))
  (bind _beginpos (`self.BeginPos`))
  (bind _returnvalue (`self.K2_GetActorLocation` _train))
  (`|ExecutionSequence`
    (:`then_0`
      (`self.K2_SetActorLocation` _train (+ (* (`KismetMathLibrary.Normal` (- (`KismetMathLibrary.VLerp` (+ _beginpos (0.0 1000.0 0.0)) (+ _beginpos (0.0 -1000.0 0.0)) (`self.MovePos`)) _returnvalue)) (* (`GameplayStatics.GetWorldDeltaSeconds`) 1000.0)) _returnvalue) false false)
      (set `self.MovePos` (`KismetMathLibrary.FClamp` (+ (`self.MovePos`) (* 0.016 (`self.SpeedTrain`))))))
    (:`then_1`
      (if (== (`self.MovePos`) 0.0)
        (set `self.SpeedTrain` 0.3)
        (elif (== (`self.MovePos`) 1.0)
          (set `self.SpeedTrain` -0.3))))))

(event `self.ReceiveBeginPlay`
  (`|ExecutionSequence`
    (:`then_0`
      (`parent.ReceiveBeginPlay`))
    (:`then_1`
      (`self.initTrain`))
    (:`then_2`
      (set `self.BeginPos` (`self.K2_GetActorLocation`)))
    (:`then_3`
      (`KismetSystemLibrary.K2_SetTimerDelegate` (delegate `YouDang`) 0.016 true))))

(event `3-1Atk`
  (`self.Attack_InputGuns` 0.0 0.0 (`/Game/Asset/Blueprints/Car/BP_Car_Train.3-1guns` (`self.Train`))))

(event `2-1Atk`
  (`self.Attack_InputGuns` 0.0 0.0 (`/Game/Asset/Blueprints/Car/BP_Car_Train.2-1guns` (`self.Train`))))

(event `2-2Atk`
  (`self.Attack_InputGuns` 0.0 0.0 (`/Game/Asset/Blueprints/Car/BP_Car_Train.2-2guns` (`self.Train`))))

(event `1-1Atk`
  (`self.Attack_InputGuns` 0.0 0.0 (`/Game/Asset/Blueprints/Car/BP_Car_Train.1-1guns` (`self.Train`))))

(event `1-2Atk`
  (`self.Attack_InputGuns` 0.0 0.0 (`/Game/Asset/Blueprints/Car/BP_Car_Train.1-2guns` (`self.Train`))))

(event `cancel_train_weapon`
  (params (Item :type "/Game/Asset/Blueprints/Gun/BP_GunBase Object Reference (by ref)"))
  (`KismetArrayLibrary.Array_RemoveItem` (`/Game/Asset/Blueprints/Car/BP_Car_Train.3-1guns` (`self.Train`)) Item))

(fn `CheckHealth`
  (bind _train (`self.Train`))
  (bind _train_2 (`self.Train`))
  (`|ExecutionSequence`
    (:`then_0`
      (`parent.CheckHealth`))
    (:`then_1`
      (if (and (< (`self.Health`) (`KismetMathLibrary.FTrunc` (* (`self.MaxHealth`) 0.8))) (== (`self.PlayerStage`) 3))
        (`/Game/Asset/Blueprints/Car/BP_Car_Train.DESTROY` _train (`/Game/Asset/Blueprints/Car/BP_Car_Train.Box3` _train))
        (set `self.BeginPos` (`KismetMathLibrary.MakeVector` (.x (`self.BeginPos`)) (- (.y (`self.BeginPos`)) 8500.0) (.z (`self.BeginPos`))))
        (set `self.PlayerStage` 2)
        (bind _astrain_controller (cast `/Game/Asset/Blueprints/AI_BT/AIcontroller/Train_Controller` (`AIBlueprintHelperLibrary.GetAIController` self)))
        (`/Game/Asset/Blueprints/AI_BT/AIcontroller/Train_Controller.TOSecend` _astrain_controller)))
    (:`then_2`
      (if (and (< (`self.Health`) (`KismetMathLibrary.FTrunc` (* (`self.MaxHealth`) 0.4))) (== (`self.PlayerStage`) 2))
        (`/Engine/EditorBlueprintResources/StandardMacros.DoOnce` false
          (:`Completed`
            (`/Game/Asset/Blueprints/Car/BP_Car_Train.DESTROY` _train_2 (`/Game/Asset/Blueprints/Car/BP_Car_Train.Box2` _train_2))
            (set `self.BeginPos` (`KismetMathLibrary.MakeVector` (.x (`self.BeginPos`)) (- (.y (`self.BeginPos`)) 8500.0) (.z (`self.BeginPos`))))
            (set `self.PlayerStage` 1)
            (bind _astrain_controller_2 (cast `/Game/Asset/Blueprints/AI_BT/AIcontroller/Train_Controller` (`AIBlueprintHelperLibrary.GetAIController` self)))
            (`/Game/Asset/Blueprints/AI_BT/AIcontroller/Train_Controller.TOFirst` _astrain_controller_2)))))))

(fn `initTrain`
  (bind _asbp_car_train (cast `/Game/Asset/Blueprints/Car/BP_Car_Train` (`ChildActorComponent.ChildActor` (`self.CarActor`))))
  (set `self.Train` _asbp_car_train))

(fn `UserConstructionScript`
  (`parent.UserConstructionScript`))