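; Enemy that drives a BP_Car child actor, fires its guns and can be destroyed by player bullets.
; Setup detaches the car and attaches the enemy to it; with MoveAlongPath set, timers drive it along a GameState-calculated path and fire periodically.
; Hits update health, the HP widget and the weak flag.
; Death destroys car and enemy, updates LevelCounter, and plays explosions, camera shake and force feedback.
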(event `self.ReceiveBeginPlay`
  (`self.InitCar`)
  (`self.InitHealth`)
  (`self.InitUI`)
  (`self.InitGunCollision`)
  (if (`self.MoveAlongPath`)
    (`self.StartMove`)
    (`KismetSystemLibrary.K2_SetTimer` null "Attack" (`self.ColdTime`) true)))

(event `StartMove`
  (bind _asbp_game_state (cast `/Game/Asset/Blueprints/BP_GameState` (`GameplayStatics.GetGameState`)))
  (set `self.GameState` _asbp_game_state)
  (set `self.OringinalPos` (`self.K2_GetActorLocation`))
  (`KismetSystemLibrary.K2_SetTimerDelegate` (delegate `Moving`) 0.017 true))

(event `Moving`
  (bind _returnvalue (* (* 0.017 (`self.Speed`)) (`self.SpeedPercent`)))
  (bind _output_get (set `self.Distance` (+ (`self.Distance`) _returnvalue)))
  (bind (_deltaposition _speedpercent) (`/Game/Asset/Blueprints/BP_GameState.CalculateDeltaLocation` (`self.GameState`) (`self.PathClass`) _output_get _returnvalue))
  (set `self.SpeedPercent` _speedpercent)
  (`/Game/Asset/Blueprints/Car/BP_Car.Drive` (`self.Car`) (`KismetMathLibrary.Conv_VectorToVector2D` _deltaposition)))

(event `BeHit`
  (params (Damage :type "Float (double-precision)"))
  (`self.BeHitByPlayerBullet` Damage))

(fn `Attack`
  (for _array_element (`/Game/Asset/Blueprints/Car/BP_Car.Guns` (`self.Car`))
    (`/Game/Asset/Blueprints/Gun/BP_GunBase.Fire` _array_element false)))

(fn `BeHitByPlayerBullet`
  (params (Damage :type "Float (double-precision)"))
  (set `self.Health` (- (`self.Health`) Damage))
  (`/Game/Asset/Widget/Enemy_HP.Been Hit` (`self.HPsystem`) Damage)
  (`self.CheckHealth`))

(fn `CheckHealth`
  ;[1 1 1] CheckIsDead
  (if (<= (`self.Health`) 0.0)
    (`self.DeadWithCar`)
    (else
      ;[1 1 1] CheckIsWeak
      (`self.CheckWeak`))))

(fn `CheckWeak`
  (set `self.BeWeak` (<= (`self.Health`) (`self.WeakThreshold`))))

(fn `DeadWithCar`
  (bind _returnvalue (`self.K2_GetActorLocation`))
  (bind _car (`self.Car`))
  (bind _levelcounter (`self.LevelCounter`))
  (if (`KismetSystemLibrary.IsValid` _car)
    (`self.K2_DestroyActor` _car)
    (`/Engine/EditorBlueprintResources/StandardMacros.IsValid` _levelcounter
      (:`Is Valid`
        (`/Game/Asset/Blueprints/Level_Counter.DeleteActor` _levelcounter self :!label _label))
      (:`Is Not Valid`
        _))
    (else
      (goto _label)))
  (`|ExecutionSequence`
    (:`then_0`
      (`GameplayStatics.SpawnEmitterAtLocation` "/Game/BallisticsVFX/Particles/Impacts/LegacyFX/Small-Medium-Large/EnergyShield/EnergyShield_impact_Large.EnergyShield_impact_Large" _returnvalue (struct :`Roll` -90.0) (6.0 6.0 6.0)))
    (:`then_1`
      (`GameplayStatics.SpawnEmitterAtLocation` "/Game/BallisticsVFX/Particles/Explosive/Explosion_Frag_small.Explosion_Frag_small" _returnvalue (struct) (2.0 2.0 2.0))
      (`GameplayStatics.SpawnEmitterAtLocation` "/Game/Asset/Particles/Jump.Jump" _returnvalue)
      (`self.K2_DestroyActor`))
    (:`then_2`
      (`GameplayStatics.PlayWorldCameraShake` "/Game/Asset/Shake/Shake_Des.Shake_Des_C" (`PlayerCameraManager.GetCameraLocation` (`GameplayStatics.GetPlayerCameraManager` 0)) 10.0 50.0 1.0 true)
      (`PlayerController.K2_ClientPlayForceFeedback` (`GameplayStatics.GetPlayerController` 0) "/Game/Asset/Shake/Shak_Dest.Shak_Dest" "None" false false false))))

(fn `HitFlash`)

(fn `InitCar`
  (bind _childactor (`ChildActorComponent.ChildActor` (`self.CarActor`)))
  (`self.K2_DetachFromActor` _childactor "KeepWorld" "KeepWorld" "KeepWorld")
  (`self.K2_AttachToActor` self _childactor "None" "KeepWorld" "KeepWorld" "KeepWorld" true)
  (bind _asbp_car (cast `/Game/Asset/Blueprints/Car/BP_Car` _childactor))
  (set `/Game/Asset/Blueprints/Car/BP_Car.Driver` self _asbp_car)
  (set `self.Car` _asbp_car)
  (`KismetArrayLibrary.Array_Set` (`Actor.Tags` _asbp_car) 0 "Enemy"))

(fn `InitGunCollision`
  (for _array_element (`/Game/Asset/Blueprints/Car/BP_Car.Guns` (`self.Car`))
    (`self.SetGunCollision` _array_element)))

(fn `InitHealth`
  (set `self.Health` (`self.MaxHealth`)))

(fn `InitUI`
  (bind _asenemy_hp (cast `/Game/Asset/Widget/Enemy_HP` (`WidgetComponent.GetUserWidgetObject` (`self.Widget`))))
  (set `/Game/Asset/Widget/Enemy_HP.Owner` self _asenemy_hp)
  (set `self.HPsystem` _asenemy_hp))

(fn `SetGunCollision`
  (params (Gun :type "/Game/Asset/Blueprints/Gun/BP_GunBase Object Reference"))
  (`PrimitiveComponent.SetCollisionProfileName` (`/Game/Asset/Blueprints/Gun/BP_GunBase.GunMesh` Gun) "EnemyGun"))

(fn `Shock`)

(fn `UserConstructionScript`)