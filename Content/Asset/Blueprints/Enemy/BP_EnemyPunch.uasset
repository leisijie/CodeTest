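; Enemy punch attack Blueprint that moves a Car actor through jump, aim, punch and return motions.
; Each motion sets the Car's location from a start position and a TimeFlow input: a curve-shaped jump, X tracking of the player, a Y-axis punch and a return to a fixed Y.
; Attack defers to the parent, and PlaySound spawns attached sounds for jump and punch.
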(fn `AimTarget`
  (params (BeginPos :type "Vector Structure") (TimeFlow :type "Float (double-precision)"))
  (bind _x (.x BeginPos))
  (`self.K2_SetActorLocation` (`self.Car`) (`KismetMathLibrary.MakeVector` (+ _x (* (- (.x (`self.K2_GetActorLocation` (`GameplayStatics.GetPlayerPawn` 0))) _x) TimeFlow)) (.y BeginPos) (.z BeginPos)) false false))

(fn `Attack`
  (params (`Z (Yaw)` :type "Float (double-precision)") (`Y (Pitch)` :type "Float (double-precision)"))
  (`parent.Attack` 0.0 0.0))

(fn `Jump`
  (params (TimeFlow :type "Float (double-precision)") (beginPos :type "Vector Structure"))
  (`self.K2_SetActorLocation` (`self.Car`) (`KismetMathLibrary.MakeVector` (.x beginPos) (+ (* TimeFlow (`self.jumpLength`)) (.y beginPos)) (+ (* (`self.jumpHight`) (`CurveFloat.GetFloatValue` (`self.jumpYcurve`) TimeFlow)) (.z beginPos))) false false))

(fn `PlaySound`
  (params (Input :type String))
  (bind _defaultsceneroot (`self.DefaultSceneRoot`))
  (switch `string` Input
    (:`Jump`
      (`GameplayStatics.SpawnSoundAttached` "/Game/Asset/Audio/Combat/喷气.喷气" _defaultsceneroot "None" (0.0 0.0 0.0) (struct) "KeepRelativeOffset" false 0.3 1.0 0.0 "/Game/Asset/Audio/FireAttenuation.FireAttenuation" null))
    (:`Punch`
      (`GameplayStatics.SpawnSoundAttached` "/Game/Asset/Audio/Combat/冲击.冲击" _defaultsceneroot "None" (0.0 0.0 0.0) (struct) "KeepRelativeOffset" false 0.3 1.0 0.0 "/Game/Asset/Audio/FireAttenuation.FireAttenuation" null))))

(fn `Punch`
  (params (beginPos :type "Vector Structure") (TimeFlow :type "Float (double-precision)"))
  (`self.K2_SetActorLocation` (`self.Car`) (`KismetMathLibrary.MakeVector` (.x beginPos) (+ (.y beginPos) (* TimeFlow (`self.pubchLength`))) (.z beginPos)) false false))

(fn `returnPosition`
  (params (beginPos :type "Vector Structure") (timeFlow :type "Float (double-precision)"))
  (bind _y (.y beginPos))
  (`self.K2_SetActorLocation` (`self.Car`) (`KismetMathLibrary.MakeVector` (.x beginPos) (- _y (* (+ _y 3000.0) timeFlow)) (.z beginPos)) false false))

(fn `UserConstructionScript`
  (`parent.UserConstructionScript`))