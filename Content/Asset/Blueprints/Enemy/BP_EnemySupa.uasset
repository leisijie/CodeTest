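; BP_EnemySupa is an enemy that fires repeated bursts of BP_Bullet_Enemy projectiles with a tail particle, starting at BeginPlay.
; Bullets spawn at the Arrow component's transform and travel data comes from its forward vector.
; A custom loop macro with Next and Break inputs lets a Delay space the shots; on completion, a longer Delay calls Shoot to restart the burst.
; Tick, overlap and construction only forward to the parent.
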(event `self.ReceiveBeginPlay`
  (bind _arrow (`self.Arrow`))
  (`parent.ReceiveBeginPlay`)
  (`self.NewMacro_0` 0 4 :!label _label
    (:`Loop`
      (`|SpawnActorFromClass` "/Game/Asset/Blueprints/EnemyBullet/BP_Bullet_Enemy.BP_Bullet_Enemy_C" (`SceneComponent.K2_GetComponentToWorld` _arrow) "Undefined" "OverrideRootScale" null (`SceneComponent.GetForwardVector` _arrow) "/Game/Asset/Particles/PS_bullettail.PS_bullettail" (struct) null)
      (`KismetSystemLibrary.Delay` 0.5)
      (goto _label :!via `Next`))
    (:`Complete`
      (`KismetSystemLibrary.Delay` 1.0)
      (`self.Shoot`))))

(event `self.ReceiveActorBeginOverlap`
  (params (OtherActor :type "Actor Object Reference"))
  (`parent.ReceiveActorBeginOverlap` OtherActor))

(event `Shoot`
  (goto _label))

(event `self.ReceiveTick`
  (params (DeltaSeconds :type "Float (single-precision)"))
  (`parent.ReceiveTick` DeltaSeconds))

(fn `UserConstructionScript`
  (`parent.UserConstructionScript`))