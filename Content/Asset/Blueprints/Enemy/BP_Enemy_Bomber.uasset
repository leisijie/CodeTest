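; Suicide bomber enemy that drives its Car toward the player, then attacks and destroys itself after a delay.
; Looping timers replace Tick: a fast one steers toward a target location, and a slower one refreshes that target from the player's position, so pursuit lags.
; When BeInRange reports true, movement stops and the delayed explosion starts.
; The construction script draws a debug sphere showing CheckRange.
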(event `self.ReceiveBeginPlay`
  (`parent.ReceiveBeginPlay`)
  (bind _asbp_player_character (cast `/Game/Asset/Blueprints/Character/BP_PlayerCharacter` (`GameplayStatics.GetPlayerPawn` 0)))
  (set `self.Player` _asbp_player_character)
  (`KismetSystemLibrary.K2_SetTimer` null "FollowPlayer" 0.017 true)
  (`KismetSystemLibrary.K2_SetTimer` null "UpdateMoveDirection" 2.0 true))

(event `PrepareToExplod`
  (`KismetSystemLibrary.K2_ClearTimer` null "FollowPlayer")
  (`KismetSystemLibrary.Delay` (`self.WaitTime`))
  (`self.Attack` 0.0)
  (`self.K2_DestroyActor`))

(fn `FollowPlayer`
  (locals (MoveVector :type "Vector2D Structure"))
  (bind _returnvalue (`self.K2_GetActorLocation`))
  (bind _targetlocation (`self.TargetLocation`))
  (if (<= (`KismetMathLibrary.Vector_Distance` _targetlocation _returnvalue) 0.01)
    (set `local.MoveVector` (0.0 0.0))
    (else
      (set `local.MoveVector` (* (`KismetMathLibrary.Normal2D` (`KismetMathLibrary.Conv_VectorToVector2D` (- _targetlocation _returnvalue))) (* (`self.Speed`) 0.017)))))
  (`/Game/Asset/Blueprints/Car/BP_Car.Drive` (`self.Car`) (`local.MoveVector`) false)
  (if (`self.BeInRange`)
    (`self.PrepareToExplod`)))

(fn `UpdateMoveDirection`
  (set `self.TargetLocation` (`self.K2_GetActorLocation` (`self.Player`))))

(fn `UserConstructionScript`
  (`parent.UserConstructionScript`)
  (`KismetSystemLibrary.DrawDebugSphere` (`self.K2_GetActorLocation`) (`self.CheckRange`) 12 (struct :`R` 0.508333 :`A` 1.0) 10.0 10.0))