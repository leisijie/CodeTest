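; Big enemy Blueprint that provides two melee and two ranged attack events, with no trigger for them in this graph.
; A box component tracks player overlap, which gates j1 and j2 as they damage the controller's MainCharacter through BeHit.
; y3 spawns one elongated bullet with a stab-shot particle at a scene point.
; y4 spawns a three-bullet angled spread from a second point, passing each bullet its direction.
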(event `j1`
  (`|ExecutionSequence`
    (:`then_0`
      (if (`self.overlap`)
        (bind _asbp_player_controller (cast `/Game/Asset/Blueprints/BP_PlayerController` (`GameplayStatics.GetPlayerController` 0)))
        (`/Game/Asset/Blueprints/Character/BP_PlayerCharacter.BeHit` (`/Game/Asset/Blueprints/BP_PlayerController.MainCharacter` _asbp_player_controller) (`self.Damage_j1`))))))

(event `j2`
  (if (`self.overlap`)
    (bind _asbp_player_controller (cast `/Game/Asset/Blueprints/BP_PlayerController` (`GameplayStatics.GetPlayerController` 0)))
    (`/Game/Asset/Blueprints/Character/BP_PlayerCharacter.BeHit` (`/Game/Asset/Blueprints/BP_PlayerController.MainCharacter` _asbp_player_controller) (`self.Damage_j2`))))

(event `self.Box.OnComponentBeginOverlap`
  (params (OverlappedComponent :type "PrimitiveComponent Object Reference") (OtherActor :type "Actor Object Reference") (OtherComp :type "PrimitiveComponent Object Reference") (OtherBodyIndex :type Integer) (bFromSweep :type Boolean) (SweepResult :type "HitResult Structure (by ref)"))
  (cast `/Game/Asset/Blueprints/Character/BP_PlayerCharacter` OtherActor)
  (set `self.overlap` true))

(event `y3`
  (bind _scene (`self.Scene`))
  (`|SpawnActorFromClass` "/Game/Asset/Blueprints/EnemyBullet/BP_Bullet_Enemy1.BP_Bullet_Enemy1_C" (`KismetMathLibrary.MakeTransform` (`SceneComponent.K2_GetComponentLocation` _scene) (`SceneComponent.K2_GetComponentRotation` _scene) (2.0 8.0 8.0)) "Undefined" "OverrideRootScale" null (0.0 1.0 0.0) "/Game/AdvancedMagicFX13/Particles/P_ky_stabShot1.P_ky_stabShot1" (struct) null))

(event `self.Box.OnComponentEndOverlap`
  (params (OverlappedComponent :type "PrimitiveComponent Object Reference") (OtherActor :type "Actor Object Reference") (OtherComp :type "PrimitiveComponent Object Reference") (OtherBodyIndex :type Integer))
  (cast `/Game/Asset/Blueprints/Character/BP_PlayerCharacter` OtherActor)
  (set `self.overlap` false))

(event `y4`
  (for _index (range -1 2)
    (`|SpawnActorFromClass` "/Game/Asset/Blueprints/EnemyBullet/BP_Bullet_Enemy.BP_Bullet_Enemy_C" (`KismetMathLibrary.MakeTransform` (.location (`SceneComponent.K2_GetComponentToWorld` (`self.Scene1`))) (.rotation (`SceneComponent.K2_GetComponentToWorld` (`self.Scene1`))) (4.0 4.0 4.0)) "Undefined" "OverrideRootScale" null (`KismetMathLibrary.GetUpVector` (`KismetMathLibrary.MakeRotator` (`KismetMathLibrary.Conv_IntToDouble` (* _index 30)) -90.0 90.0)) null (struct) null)))

(fn `UserConstructionScript`
  (`parent.UserConstructionScript`))