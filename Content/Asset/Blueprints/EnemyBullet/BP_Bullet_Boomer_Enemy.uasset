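; BP_Bullet_Boomer_Enemy is the Boomer enemy's bullet, an instant area-damage explosion rather than a travelling projectile.
; On BeginPlay it calls the parent, runs Explosion and immediately destroys itself.
; Explosion sphere-overlaps one custom object type within DamageRadius and sends a BeExploded message with Damage to each hit actor's parent actor.
; A particle-finished event also destroys the actor, and a debug sphere draw is left unconnected.
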(event `self.ReceiveBeginPlay`
  (`parent.ReceiveBeginPlay`)
  (`self.Explosion`)
  (`self.K2_DestroyActor`))

(event `self.ParticleSystem.OnSystemFinished`
  (params (PSystem :type "ParticleSystemComponent Object Reference"))
  (`self.K2_DestroyActor`))

(fn `Explosion`
  (bind _outactors (`KismetSystemLibrary.SphereOverlapActors` (`self.K2_GetActorLocation`) (`self.DamageRadius`) (`|MakeArray` "ObjectTypeQuery13" :!type "EObjectTypeQuery Enum")))
  (for _array_element _outactors
    (message `/Game/Asset/Blueprints/IF_Explosion.BeExploded` (`self.GetParentActor` _array_element) (`self.Damage`))))

(fn `UserConstructionScript`
  (`parent.UserConstructionScript`))