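; Enemy bullet that damages the player on impact and reacts to what it strikes.
; The Hit event switches on the other actor's first tag, sending untagged, obstacle and unknown hits to HitObstacle, which is not defined here.
; Player hits call BeHit through player controller 0's MainCharacter and destroy the bullet.
; Player and enemy hits spawn an impact emitter and short-lived scorch decal, with no damage to enemies.
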(event `self.ReceiveHit`
  (params (MyComp :type "PrimitiveComponent Object Reference") (Other :type "Actor Object Reference") (OtherComp :type "PrimitiveComponent Object Reference") (bSelfMoved :type Boolean) (HitLocation :type "Vector Structure") (HitNormal :type "Vector Structure") (NormalImpulse :type "Vector Structure") (Hit :type "HitResult Structure (by ref)"))
  (bind _tags (`Actor.Tags` Other))
  (if (`KismetArrayLibrary.Array_IsValidIndex` _tags)
    (switch `name` (`|GetArrayItem` _tags)
      (:`Default`
        (`self.HitObstacle` :!label _label))
      (:`Player`
        (`self.HitPlayer`)
        (`GameplayStatics.SpawnEmitterAtLocation` (`self.hitEffect`) HitLocation (struct) (3.0 3.0 3.0) :!label _label_2)
        (`GameplayStatics.SpawnDecalAttached` "/Game/BallisticsVFX/Decals/Decals_Scorch.Decals_Scorch" (30.0 50.0 50.0) OtherComp "None" HitLocation (struct :`Yaw` 90.0) "KeepWorldPosition" 0.3))
      (:`Enemy`
        (goto _label_2))
      (:`Obstacle`
        (goto _label)))
    (else
      (`self.HitObstacle`))))

(fn `HitPlayer`
  (bind _asbp_player_controller (cast `/Game/Asset/Blueprints/BP_PlayerController` (`GameplayStatics.GetPlayerController` 0)))
  (`/Game/Asset/Blueprints/Character/BP_PlayerCharacter.BeHit` (`/Game/Asset/Blueprints/BP_PlayerController.MainCharacter` _asbp_player_controller) (`self.Damage`))
  (`self.K2_DestroyActor`))

(fn `UserConstructionScript`
  (`parent.UserConstructionScript`))