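; Enemy bomb projectile that arcs and bounces off a fixed floor height, then charges along negative Y.
; A looping timer offsets the Box by horizontal and vertical speed without sweep, applying Jiasudu as vertical acceleration and flipping vertical speed upward at low height.
; After a short delay, a one-shot sets a fast negative horizontal speed and starts a second timer that keeps accelerating it.
; Overlap handling defers to the parent, and the random horizontal value goes unused here.
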(event `self.ReceiveBeginPlay`
  (`parent.ReceiveBeginPlay`)
  (`|ExecutionSequence`
    (:`then_0`
      (`KismetSystemLibrary.K2_SetTimerDelegate` (delegate `tan`) (`self.timer`) true))
    (:`then_1`
      (set `self.horizontalRandom` (`KismetMathLibrary.RandomFloatInRange` -500.0 500.0)))))

(event `tan`
  (`|ExecutionSequence`
    (:`then_0`
      (`SceneComponent.K2_AddWorldOffset` (`self.Box`) (`KismetMathLibrary.MakeVector` 0.0 (* (`self.horizontalspeed`) (`self.timer`)) (* (`self.verticalSpeed`) (`self.timer`))) false false))
    (:`then_1`
      (set `self.verticalSpeed` (+ (`self.verticalSpeed`) (* (`self.timer`) (`self.jiasudu`))))
      (`KismetSystemLibrary.Delay` 0.4)
      (`/Engine/EditorBlueprintResources/StandardMacros.DoOnce` false
        (:`Completed`
          (`|ExecutionSequence`
            (:`then_0`
              (set `self.horizontalspeed` -4000.0))
            (:`then_1`
              (`KismetSystemLibrary.K2_SetTimerDelegate` (delegate `CustomEvent_0`) (`self.timer`) true))))))
    (:`then_2`
      (if (< (.z (`self.K2_GetActorLocation` self)) 100.0)
        (set `self.verticalSpeed` (* (`KismetMathLibrary.Abs` (`self.verticalSpeed`)) 1.0))))))

(event `CustomEvent_0`
  (set `self.horizontalspeed` (- (`self.horizontalspeed`) (* (`self.timer`) 10000.0))))

(event `self.ReceiveActorBeginOverlap`
  (params (OtherActor :type "Actor Object Reference"))
  (`parent.ReceiveActorBeginOverlap` OtherActor))

(event `self.ReceiveTick`
  (params (DeltaSeconds :type "Float (single-precision)")))

(fn `UserConstructionScript`
  (`parent.UserConstructionScript`))