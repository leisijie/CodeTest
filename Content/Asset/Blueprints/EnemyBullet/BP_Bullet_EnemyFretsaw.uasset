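; Enemy fretsaw projectile that drops toward the ground while rapidly accelerating along its local X axis.
; BeginPlay starts a looping timer on the Saw event, which offsets Box without sweep using a DeltaTime captured once, after the timer is set.
; Gravity is integrated manually until actor height falls below 100, where vertical speed is zeroed once.
; A Box spin node exists but is unconnected.
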(event `self.ReceiveBeginPlay`
  (`|ExecutionSequence`
    (:`then_0`
      (`parent.ReceiveBeginPlay`))
    (:`then_1`
      (`KismetSystemLibrary.K2_SetTimerDelegate` (delegate `saw`) (`self.deltaTime`) true))
    (:`then_2`
      (set `self.deltaTime` (`GameplayStatics.GetWorldDeltaSeconds`)))))

(event `saw`
  (bind _deltatime (`self.deltaTime`))
  (`|ExecutionSequence`
    (:`then_0`
      (`SceneComponent.K2_AddLocalOffset` (`self.Box`) (`KismetMathLibrary.MakeVector` (* (`self.ySpeed`) _deltatime) 0.0 (* (`self.verticalSpeed`) _deltatime)) false false))
    (:`then_1`
      (set `self.ySpeed` (+ (`self.ySpeed`) (* 40000.0 (`self.deltaTime`)))))
    (:`then_2`
      (if (< (.z (`self.K2_GetActorLocation` self)) 100.0)
        (`/Engine/EditorBlueprintResources/StandardMacros.DoOnce` false
          (:`Completed`
            (set `self.verticalSpeed` 0.0)))
        (else
          (set `self.verticalSpeed` (+ (`self.verticalSpeed`) (* (`self.deltaTime`) -3000.0))))))))

(fn `UserConstructionScript`
  (`parent.UserConstructionScript`))