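; BP_Bullet_Throw is a lobbed enemy projectile that arcs to where the player stood when it spawned.
; On BeginPlay it stores that position, spawns a Target actor there and plays an electrical effect at its origin.
; A timeline lerps ground position and drives height with a separate curve, without sweeping.
; On finish it spawns BP_Bullet_Boomer_Enemy with a damage radius, plays an explosion, then destroys the target and itself.
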(event `self.ReceiveBeginPlay`
  (bind _actor_location (`self.Actor Location`))
  (bind _output_get (set `self.StorePlayer Location` (`self.K2_GetActorLocation` (`GameplayStatics.GetPlayerPawn` 0))))
  (bind _output_get_2 (set `self.Actor Location` (`self.K2_GetActorLocation` self)))
  (bind _returnvalue (`|SpawnActorFromClass` "/Game/Asset/Blueprints/Target.Target_C" (`KismetMathLibrary.Conv_VectorToTransform` _output_get) "Undefined" "OverrideRootScale" null null))
  (set `self.Target` _returnvalue)
  (`GameplayStatics.SpawnEmitterAtLocation` "/Game/BallisticsVFX/Particles/Impacts/LegacyFX/Small-Medium-Large/Electrical/Electrical_impact_med.Electrical_impact_med" _output_get_2 (struct) (2.0 2.0 5.0))
  (bind (_direction _ground _hori) (`Timeline|Timeline_0`)
    (:`Update`
      (bind _x (.x (`KismetMathLibrary.VLerp` _actor_location (`self.StorePlayer Location`) _ground)))
      (bind _y (.y (`KismetMathLibrary.VLerp` _actor_location (`self.StorePlayer Location`) _ground)))
      (bind _returnvalue_2 (`KismetMathLibrary.MakeVector` _x _y (+ (* _hori (+ (.z _actor_location) 1000.0)) 300.0)))
      (`self.K2_SetActorLocation` _returnvalue_2))
    (:`Finished`
      (`|SpawnActorFromClass` "/Game/Asset/Blueprints/EnemyBullet/BP_Bullet_Boomer_Enemy.BP_Bullet_Boomer_Enemy_C" (`KismetMathLibrary.Conv_VectorToTransform` _returnvalue_2) "Undefined" "OverrideRootScale" null 400.0 (0.0 1.0 0.0) null (struct) null)
      (`GameplayStatics.SpawnEmitterAtLocation` "/Game/BallisticsVFX/Particles/Explosive/Explosion_Frag_small.Explosion_Frag_small" (`KismetMathLibrary.MakeVector` _x _y) (struct) (2.0 2.0 2.0))
      (`self.K2_DestroyActor` (`self.Target`))
      (`self.K2_DestroyActor`))))

(fn `UserConstructionScript`
  (`parent.UserConstructionScript`))