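; Environment switch effect actor that slides through the level and can change the post-process look.
; Go starts a looping ~60 Hz timer that calls Move to offset the actor, then clears it and destroys the actor after DeathTime.
; With ChangeFogEffect set, it also shows a Vignette_Once widget, then a second later replaces BP_POstProcess's post-process materials.
; The Trigger overlap and End events have no effect.
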(event `Go`
  (bind _returnvalue (`KismetSystemLibrary.K2_SetTimer` null "Move" 0.0167 true))
  (`|ExecutionSequence`
    (:`then_0`
      (`KismetSystemLibrary.Delay` (`self.DeathTime`))
      (`KismetSystemLibrary.K2_ClearAndInvalidateTimerHandle` _returnvalue)
      (`self.K2_DestroyActor`))
    (:`then_1`
      (if (`self.Change Fog Effect?`)
        (bind _returnvalue_2 (`|CreateWidget` "/Game/Asset/Widget/Vignette_Once.Vignette_Once_C" (`GameplayStatics.GetPlayerController` 0)))
        (`UserWidget.AddToPlayerScreen` _returnvalue_2 0)
        (`KismetSystemLibrary.Delay` 1.0)
        (bind _returnvalue_3 (`GameplayStatics.GetActorOfClass` "/Game/Asset/Blueprints/BP_POstProcess.BP_POstProcess_C"))
        (`/Engine/EditorBlueprintResources/StandardMacros.IsValid` _returnvalue_3
          (:`Is Valid`
            (setmembers `PostProcessSettings` :`StructRef` (`PostProcessComponent.Settings` (`/Game/Asset/Blueprints/BP_POstProcess.PostProcess1` _returnvalue_3)) :`WeightedBlendables` (`self.PPM_Ma`))))))))

(event `self.Trigger.OnComponentBeginOverlap`
  (params (OverlappedComponent :type "PrimitiveComponent Object Reference") (OtherActor :type "Actor Object Reference") (OtherComp :type "PrimitiveComponent Object Reference") (OtherBodyIndex :type Integer) (bFromSweep :type Boolean) (SweepResult :type "HitResult Structure (by ref)"))
  (`/Engine/EditorBlueprintResources/StandardMacros.DoOnce` false))

(event `End`)

(fn `Move`
  (`self.K2_AddActorWorldOffset` (`self.Add Location`)))

(fn `UserConstructionScript`)