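; Spline-based moving environment line that registers with LevelCounter and circulates scenery actors to simulate a scrolling environment.
; The construction script spaces child actors evenly along the spline, storing each one's normalized time.
; GO reveals them last-to-first with delays, starts a looping timer that moves them by curve, and spawns a TransformActor for main roads.
; BYEBYE stops the timer, then scrolls the whole actor along -Y until delayed destruction.
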(event `self.ReceiveBeginPlay`
  (bind _levelcounter (`self.LevelCounter`))
  (`/Engine/EditorBlueprintResources/StandardMacros.IsValid` _levelcounter
    (:`Is Valid`
      (`self.Wave Control` _levelcounter null null self))))

(event `GO`
  (bind _actor_store (`self.Actor_Store`))
  (bind _spline (`self.Spline`))
  (`|ExecutionSequence`
    (:`then_0`
      ;[1 1 1] q
      (`KismetSystemLibrary.Delay` (`self.Building Displau Delaytime`))
      (bind _index (`self.Loop With Delay` (`KismetArrayLibrary.Array_LastIndex` _actor_store) :!label _label)
        (:`Loop Body`
          (`SceneComponent.SetVisibility` (`.Actor_6_A2B9A9E848577EC93019A394DA4F74C4` (break `/Game/Asset/Blueprints/Struct/Str_SplineActor` (`|GetArrayItem` _actor_store _index))) true false)
          (`KismetSystemLibrary.Delay` (`self.Building Displau Delaytime`))
          (goto _label :!via `Next Step In`))))
    (:`then_1`
      (`KismetSystemLibrary.K2_SetTimer` null "UpdateMove" 0.017 true))
    (:`then_2`
      (if (`self.Is Main Road`)
        (bind _returnvalue (`|SpawnActorFromClass` (`self.TransformActor`) (`KismetMathLibrary.Conv_VectorToTransform` (`SplineComponent.GetLocationAtSplinePoint` _spline 0 "World")) "Undefined" "OverrideRootScale" (`GameplayStatics.GetPlayerController` 0) (`KismetMathLibrary.MakeVector` 0.0 (* (/ (`SplineComponent.GetSplineLength` _spline) (`self.TotalTime`)) -0.0167)) null))
        (`/Game/Asset/Blueprints/EnviromentSwitch/EnviromentSwitchEffect.Go` _returnvalue)))))

(event `self.ReceiveTick`
  (params (DeltaSeconds :type "Float (single-precision)"))
  (`/Engine/EditorBlueprintResources/StandardMacros.Gate` true :!label _label_2
    (:`Exit`
      (`SceneComponent.K2_AddWorldOffset` (`self.DefaultSceneRoot`) (`KismetMathLibrary.MakeVector` 0.0 (* (* (/ 0.017 (`self.TotalTime`)) (`SplineComponent.GetSplineLength` (`self.Spline`))) -1.0)) false false)
      (`KismetSystemLibrary.Delay` 10.0)
      (`self.K2_DestroyActor`))))

(event `BYEBYE`
  (`|ExecutionSequence`
    (:`then_0`
      (`KismetSystemLibrary.K2_ClearTimer` null "UpdateMove"))
    (:`then_1`
      (goto _label_2 :!via `Open`))))

(fn `UpdateMove`
  (locals (LocalTime :type "Float (double-precision)"))
  (bind _spline (`self.Spline`))
  (bind _returnvalue (`SplineComponent.GetSplineLength` (`self.Spline`)))
  (for (_array_element _array_index) (`self.Actor_Store`)
    (bind (_actor _time) (break `/Game/Asset/Blueprints/Struct/Str_SplineActor` _array_element))
    (bind _returnvalue_2 (+ _time (/ 0.017 (`self.TotalTime`))))
    (if (>= _returnvalue_2 1.0)
      (set `local.LocalTime` 0.0)
      (else
        (set `local.LocalTime` _returnvalue_2)))
    (`/Engine/EditorBlueprintResources/StandardMacros.IsValid` _actor
      (:`Is Valid`
        (`KismetArrayLibrary.Array_Set` (`self.Actor_Store`) _array_index (make `/Game/Asset/Blueprints/Struct/Str_SplineActor` _actor (`local.LocalTime`)))
        (if (`self.+?`)
          (bind _returnvalue_3 (`CurveFloat.GetFloatValue` (`self.Curve`) _returnvalue_2))
          (bind _returnvalue_4 (* _returnvalue_3 _returnvalue))
          (`SceneComponent.K2_SetWorldLocation` _actor (`SplineComponent.GetLocationAtDistanceAlongSpline` _spline _returnvalue_4 "World") false false)
          (else
            (`SceneComponent.K2_SetWorldLocation` _actor (`SplineComponent.GetLocationAtDistanceAlongSpline` _spline (* (- 1.0 _returnvalue_3) _returnvalue) "World") false false)))
        (`SceneComponent.K2_SetWorldRotation` _actor (`KismetMathLibrary.MakeRotator` (.roll (`SplineComponent.GetRotationAtDistanceAlongSpline` _spline _returnvalue_4 "World")) (.pitch (`SplineComponent.GetRotationAtDistanceAlongSpline` _spline _returnvalue_4 "World")) (+ (.yaw (`SplineComponent.GetRotationAtDistanceAlongSpline` _spline _returnvalue_4 "World")) (`self.TURN`))) false false)))))

(fn `UserConstructionScript`
  (bind _amount (`self.Amount`))
  (bind _spline (`self.Spline`))
  (`KismetArrayLibrary.Array_Clear` (`self.Actor_Store`))
  (for _index (range _amount)
    (bind _returnvalue (/ (`KismetMathLibrary.Conv_IntToDouble` _index) (`KismetMathLibrary.Conv_IntToDouble` _amount)))
    (bind _returnvalue_2 (* _returnvalue (`SplineComponent.GetSplineLength` _spline)))
    (bind _returnvalue_3 (`AddComponent|NODE_AddChildActorComponent-4` :`RelativeTransform` (`KismetMathLibrary.MakeTransform` (`SplineComponent.GetLocationAtDistanceAlongSpline` _spline _returnvalue_2 "Local") (`SplineComponent.GetRotationAtDistanceAlongSpline` _spline _returnvalue_2 "Local"))))
    (`SceneComponent.SetVisibility` _returnvalue_3 (`self.Visible`) false)
    (`ChildActorComponent.SetChildActorClass` _returnvalue_3 (`self.Move_budy`))
    (`KismetArrayLibrary.Array_Add` (`self.Actor_Store`) (make `/Game/Asset/Blueprints/Struct/Str_SplineActor` _returnvalue_3 _returnvalue))))