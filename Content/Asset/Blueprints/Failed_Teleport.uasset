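; Placed actor that repositions the player at level start when the game instance's PreLevelFail flag is set.
; On BeginPlay it reads the flag from bp_Gameinstance and, if true, moves the ThirdPersonCharacter to its Arrow component's world location and rotation.
; The world-space values are applied through relative location and rotation setters, and the flag is not cleared here.
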(event `self.ReceiveBeginPlay`
  (bind _arrow (`self.Arrow`))
  (bind _asbp_gameinstance (cast `/Game/Asset/Blueprints/bp_Gameinstance` (`GameplayStatics.GetGameInstance`)))
  (if (`/Game/Asset/Blueprints/bp_Gameinstance.PreLevelFail?` _asbp_gameinstance)
    (bind _asthird_person_character (cast `/Game/DynamicLocomotion/Blueprints/ThirdPersonCharacter` (`GameplayStatics.GetPlayerPawn` 0)))
    (`self.K2_SetActorRelativeLocation` _asthird_person_character (`SceneComponent.K2_GetComponentLocation` _arrow) false false)
    (`self.K2_SetActorRelativeRotation` _asthird_person_character (`SceneComponent.K2_GetComponentRotation` _arrow) false false)))

(fn `UserConstructionScript`)