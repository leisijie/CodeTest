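; Test follower actor that moves itself to the player pawn and then sticks to its location.
; Shortly after BeginPlay, a timeline pulls the root toward the player with VInterpTo, using its MOVE track as both delta time and interp speed.
; A delay started from the timeline update sets Follow, after which Tick snaps the root to the player's location every frame.
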(event `self.ReceiveActorBeginOverlap`
  (params (OtherActor :type "Actor Object Reference")))

(event `self.ReceiveBeginPlay`
  (`KismetSystemLibrary.Delay` 2.0)
  (`self.MOVE`))

(event `MOVE`
  (bind (_direction _move) (`Timeline|Timeline_0` :`NewTime` 10.0)
    (:`Update`
      (`SceneComponent.K2_SetWorldLocation` (`self.DefaultSceneRoot`) (`KismetMathLibrary.VInterpTo` (`SceneComponent.K2_GetComponentLocation` (`self.DefaultSceneRoot`)) (`self.K2_GetActorLocation` (`GameplayStatics.GetPlayerPawn` 0)) _move _move) false false)
      (`KismetSystemLibrary.Delay` 2.0)
      (set `self.Follow` true))))

(event `self.ReceiveTick`
  (params (DeltaSeconds :type "Float (single-precision)"))
  (if (`self.Follow`)
    (`SceneComponent.K2_SetWorldLocation` (`self.DefaultSceneRoot`) (`self.K2_GetActorLocation` (`GameplayStatics.GetPlayerPawn` 0)) false false)))

(fn `UserConstructionScript`)