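; Grapple launcher that fires a cabled LagaanBody in four directions to steal guns from weakened enemies and upgrade the player's.
; Aim opens a Tick gate that follows the controller's FireDirection and box-traces to place a target marker.
; Start fires on a hit, using Timeline lerps to send the body out and back.
; A copy of an unlooted gun rides back, feeds GunUpgrade for the aimed direction, then is destroyed.
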(event `self.ReceiveTick`
  (params (DeltaSeconds :type "Float (single-precision)"))
  (bind _lagaan_body (`self.Lagaan_Body`))
  (bind _plane (`self.Plane`))
  (bind _returnvalue (`SceneComponent.K2_GetComponentLocation` (`self.DefaultSceneRoot`)))
  (`/Engine/EditorBlueprintResources/StandardMacros.Gate` true :!label _label
    (:`Exit`
      (if (not (`self.IsFiring`))
        (bind _asbp_player_controller (cast `/Game/Asset/Blueprints/BP_PlayerController` (`GameplayStatics.GetPlayerController` 0)))
        (switch `/Game/Asset/Blueprints/Enum/Enum_GunDirection` (`/Game/Asset/Blueprints/BP_PlayerController.FireDirection` _asbp_player_controller)
          (:`NewEnumerator0`
            (set `self.FireDirection` (1.0 0.0 0.0))
            (`SceneComponent.K2_SetWorldRotation` _lagaan_body (struct :`Yaw` -90.0) false false))
          (:`NewEnumerator1`
            (set `self.FireDirection` (-1.0 0.0 0.0))
            (`SceneComponent.K2_SetWorldRotation` _lagaan_body (struct :`Yaw` 90.0) false false))
          (:`NewEnumerator2`
            (set `self.FireDirection` (0.0 -1.0 0.0))
            (`SceneComponent.K2_SetWorldRotation` _lagaan_body (struct :`Yaw` 180.0) false false))
          (:`NewEnumerator3`
            (set `self.FireDirection` (0.0 1.0 0.0))
            (`SceneComponent.K2_SetWorldRotation` :`self` _lagaan_body)))
        (bind (_outhit _returnvalue_2) (`KismetSystemLibrary.BoxTraceSingle` _returnvalue (+ _returnvalue (* (`self.FireDirection`) 3000.0)) (100.0 100.0 100.0) (struct) "TraceTypeQuery4"))
        (if _returnvalue_2
          (`SceneComponent.SetVisibility` _plane true false)
          (`SceneComponent.K2_SetWorldLocation` _plane (`self.K2_GetActorLocation` (`.HitActor` (`GameplayStatics.BreakHitResult` _outhit))) false false)
          (else
            (`SceneComponent.SetVisibility` _plane false false)))))))

(event `Aim`
  (goto _label :!via `Open`))

(event `self.ReceiveBeginPlay`
  (`SceneComponent.SetWorldScale3D` (`self.DefaultSceneRoot`) (1.0 1.0 1.0))
  (`SceneComponent.K2_DetachFromComponent` (`self.Plane`) "KeepWorld" "KeepWorld" "KeepWorld" true))

(event `Start`
  (bind _returnvalue (`SceneComponent.K2_GetComponentLocation` (`self.DefaultSceneRoot`)))
  (`|ExecutionSequence`
    (:`then_0`
      (`SceneComponent.SetVisibility` (`self.Plane`) false false)
      (goto _label :!via `Close`))
    (:`then_1`
      (if (not (`self.IsFiring`))
        (set `self.IsFiring` true)
        ;[1 1 1] Aim Fire
        (bind (_outhit _returnvalue_2) (`KismetSystemLibrary.BoxTraceSingle` _returnvalue (+ _returnvalue (* (`self.FireDirection`) 3000.0)) (100.0 100.0 100.0) (struct) "TraceTypeQuery4"))
        (if _returnvalue_2
          (set `self.Hitlocation` (`.Location` (`GameplayStatics.BreakHitResult` _outhit)))
          (`self.FireGrab`)
          (`SceneComponent.SetVisibility` (`self.Lagaan_Body`) true false)
          (`SceneComponent.SetVisibility` (`self.Cable`) true false)
          (else
            (set `self.IsFiring` false)))))))

(event `FireGrab`
  (bind _lagaan_body (`self.Lagaan_Body`))
  (`GameplayStatics.SpawnEmitterAtLocation` "/Game/BallisticsVFX/Particles/Impacts/DynamicImpacts/Lava/Lava_Debris.Lava_Debris" (`SceneComponent.K2_GetComponentLocation` (`self.DefaultSceneRoot`)) (`KismetMathLibrary.Conv_VectorToRotator` (`self.FireDirection`)) (3.0 3.0 3.0))
  ;[1 1 1] Visible
  (`SceneComponent.SetVisibility` (`self.Lagaan_Body`) true false)
  (bind _asbp_player_controller (cast `/Game/Asset/Blueprints/BP_PlayerController` (`GameplayStatics.GetPlayerController` 0)))
  ;[1 1 1] Fire
  (set `self.AimDir` (`/Game/Asset/Blueprints/BP_PlayerController.FireDirection` _asbp_player_controller))
  (bind (_direction _move) (`Timeline|Timeline_0` :!via `PlayFromStart`)
    (:`Update`
      (`SceneComponent.K2_SetWorldLocation` (`self.Lagaan_Body`) (+ (* (`SceneComponent.K2_GetComponentLocation` (`self.DefaultSceneRoot`)) (- 1.0 _move)) (* (`self.Hitlocation`) _move)) false false))
    (:`Finished`
      (`GameplayStatics.SpawnEmitterAttached` "/Game/BallisticsVFX/Laggonburst.Laggonburst" _lagaan_body "None" (0.0 0.0 0.0) (`SceneComponent.K2_GetComponentRotation` _lagaan_body))
      (bind (_bblockinghit _binitialoverlap _time _distance _location _impactpoint _normal _impactnormal _physmat _hitactor _hitcomponent) (`GameplayStatics.BreakHitResult` (stale `Start` _outhit)))
      ;[1 1 1] Attach
      (`SceneComponent.K2_AttachToComponent` _lagaan_body _hitcomponent "None" "KeepWorld" "KeepWorld" "KeepWorld" true)
      (`KismetSystemLibrary.Delay` (`self.Wait`))
      (`self.Getback`)
      ;[1 1 1] CheckWeakAndLoot
      (`/Engine/EditorBlueprintResources/StandardMacros.IsValid` _hitactor
        (:`Is Valid`
          (bind _asbp_enemy (cast `/Game/Asset/Blueprints/Character/BP_Enemy` (`self.GetParentActor` (`self.GetParentActor` _hitactor))))
          (if (`/Game/Asset/Blueprints/Character/BP_Enemy.BeWeak` _asbp_enemy)
            (bind _asbp_gun_base (cast `/Game/Asset/Blueprints/Gun/BP_GunBase` _hitactor))
            (if (not (`/Game/Asset/Blueprints/Gun/BP_GunBase.BeLoot` _asbp_gun_base))
              (set `/Game/Asset/Blueprints/Gun/BP_GunBase.BeLoot` true _asbp_gun_base)
              (bind _returnvalue (`|SpawnActorFromClass` (`GameplayStatics.GetObjectClass` _hitactor) (`KismetMathLibrary.Conv_VectorToTransform` (`SceneComponent.K2_GetComponentLocation` (`self.Lagaan_Body`))) "AlwaysSpawn" "OverrideRootScale" null null))
              (set `self.CaughtStuff` _returnvalue)
              (`self.K2_AttachToComponent` _returnvalue (`self.Lagaan_Body`) "None" "KeepWorld" "KeepWorld" "KeepWorld" true))))))))

(event `Getback`
  (bind _caughtstuff (`self.CaughtStuff`))
  (`GameplayStatics.SpawnEmitterAtLocation` "/Game/BallisticsVFX/Laggonburst.Laggonburst" (`SceneComponent.K2_GetComponentLocation` (`self.Lagaan_Body`)))
  ;[1 1 1] Getback
  (bind (_direction _move) (`Timeline|Timeline_1` :!via `PlayFromStart`)
    (:`Update`
      (`SceneComponent.K2_SetWorldLocation` (`self.Lagaan_Body`) (+ (* (`self.Hitlocation`) (- 1.0 _move)) (* (`SceneComponent.K2_GetComponentLocation` (`self.DefaultSceneRoot`)) _move)) false false))
    (:`Finished`
      ;[1 1 1] byebye
      (`SceneComponent.K2_AttachToComponent` (`self.Lagaan_Body`) (`self.DefaultSceneRoot`) "None" "KeepWorld" "SnapToTarget" "KeepWorld" true)
      (set `self.IsFiring` false)
      (`SceneComponent.SetVisibility` (`self.Lagaan_Body`) false false)
      (`SceneComponent.SetVisibility` (`self.Cable`) false false)
      ;[1 1 1] GunUpgrade
      (`/Engine/EditorBlueprintResources/StandardMacros.IsValid` _caughtstuff
        (:`Is Valid`
          (bind _asbp_player_controller (cast `/Game/Asset/Blueprints/BP_PlayerController` (`GameplayStatics.GetPlayerController` 0)))
          (`/Game/Asset/Blueprints/Character/BP_PlayerCharacter.GunUpgrade` (`/Game/Asset/Blueprints/BP_PlayerController.MainCharacter` _asbp_player_controller) (`self.AimDir`) (`|GetArrayItem` (`Actor.Tags` _caughtstuff)))
          (`/Engine/EditorBlueprintResources/StandardMacros.IsValid` (`self.CaughtStuff`)
            (:`Is Valid`
              (`self.K2_DestroyActor` (`self.CaughtStuff`)))))))))

(fn `UserConstructionScript`)