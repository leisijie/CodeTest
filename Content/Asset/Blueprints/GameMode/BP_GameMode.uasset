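; Game mode Blueprint that manages a multi-slot save system, indexed by a master AllSaveData object in the "AllGameData" slot.
; BeginPlay loads or creates that index.
; SaveNew writes a timestamp-named SaveGameTest slot and SaveRepeat overwrites a given one, both updating the index list.
; Load finds an entry by UserIndex and loads its slot, but SetDataDetail and LoadData are empty stubs, so no game state is transferred yet.
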(event `self.ReceiveBeginPlay`
  (bind _returnvalue (`GameplayStatics.LoadGameFromSlot` "AllGameData"))
  (bind _asall_save_data (cast `/Game/Asset/Blueprints/AllSaveData` _returnvalue)
    (:`then`
      (set `self.AllSaveData` _asall_save_data))
    (:`CastFailed`
      (bind _returnvalue_2 (`GameplayStatics.CreateSaveGameObject` "/Game/Asset/Blueprints/AllSaveData.AllSaveData_C"))
      (bind _output_get (set `self.AllSaveData` _returnvalue_2))
      (`GameplayStatics.SaveGameToSlot` _output_get "AllGameData"))))

(event `SaveNew`
  (`self.Save Game Data New`))

(event `Save Repeat`
  (params (saveDataName1 :type String) (DataIndex1 :type Integer))
  (`self.Save Game Data Repeat` saveDataName1 DataIndex1))

(event `Load`
  (params (Index :type Integer))
  (bind _returnvalue (`GameplayStatics.LoadGameFromSlot` "AllGameData"))
  (bind _asall_save_data (cast `/Game/Asset/Blueprints/AllSaveData` _returnvalue))
  (for _array_element (`/Game/Asset/Blueprints/AllSaveData.GameSaveDataList` _asall_save_data)
    (bind (_savetime _slotname _userindex) (break `/Game/Asset/Blueprints/SaveDataStructure` _array_element))
    (if (== _userindex Index)
      (bind _returnvalue_2 (`GameplayStatics.LoadGameFromSlot` _slotname _userindex))
      (bind _assave_game_test (cast `/Game/Asset/Blueprints/SaveGameTest` _returnvalue_2))
      (`self.LoadData` _assave_game_test))))

(fn `LoadData`
  (params (GameData :type "/Game/Asset/Blueprints/SaveGameTest Object Reference"))
  (return))

(fn `Save Game Data New`
  (locals (saveDataName :type String) (DataIndex :type Integer :default 0) (SaveDate :type "/Game/Asset/Blueprints/SaveGameTest Object Reference"))
  (bind _dataindex (`local.DataIndex`))
  (bind _savedataname (`local.saveDataName`))
  (bind (_year _month _day _hour _minute _second) (`KismetMathLibrary.BreakDateTime` (`KismetMathLibrary.Now`)))
  (bind _returnvalue (`GameplayStatics.CreateSaveGameObject` "/Game/Asset/Blueprints/SaveGameTest.SaveGameTest_C"))
  (bind _savegamedata1 (`self.SetDataDetail` _returnvalue))
  (bind _output_get (set `local.SaveDate` _savegamedata1))
  (bind _output_get_2 (set `local.saveDataName` (`KismetStringLibrary.Concat_StrStr` (`KismetStringLibrary.Conv_IntToString` _year) "/" (`KismetStringLibrary.Conv_IntToString` _month) "/" (`KismetStringLibrary.Conv_IntToString` _day) "/" (`KismetStringLibrary.Conv_IntToString` _hour) "/" (`KismetStringLibrary.Conv_IntToString` _minute) "/" (`KismetStringLibrary.Conv_IntToString` _second))))
  (bind _output_get_3 (set `local.DataIndex` (`KismetArrayLibrary.Array_Length` (`/Game/Asset/Blueprints/AllSaveData.GameSaveDataList` (`self.AllSaveData`)))))
  (`GameplayStatics.SaveGameToSlot` _output_get _output_get_2 _output_get_3)
  (`KismetArrayLibrary.Array_Set` (`/Game/Asset/Blueprints/AllSaveData.GameSaveDataList` (`self.AllSaveData`)) _dataindex (make `/Game/Asset/Blueprints/SaveDataStructure` (`KismetStringLibrary.Concat_StrStr` "第" (`KismetStringLibrary.Conv_IntToString` _dataindex) " 时间：" _savedataname) _savedataname _dataindex) true)
  (`GameplayStatics.SaveGameToSlot` (`self.AllSaveData`) "AllGameData"))

(fn `Save Game Data Repeat`
  (params (saveDataName1 :type String) (DataIndex1 :type Integer))
  (locals (saveDataName :type String) (DataIndex :type Integer :default 0) (SaveData :type "/Game/Asset/Blueprints/SaveGameTest Object Reference"))
  (bind _dataindex (`local.DataIndex`))
  (bind _savedataname (`local.saveDataName`))
  (bind _returnvalue (`GameplayStatics.CreateSaveGameObject` "/Game/Asset/Blueprints/SaveGameTest.SaveGameTest_C"))
  (bind _savegamedata1 (`self.SetDataDetail` _returnvalue))
  (bind _output_get (set `local.SaveData` _savegamedata1))
  (bind _output_get_2 (set `local.saveDataName` saveDataName1))
  (bind _output_get_3 (set `local.DataIndex` DataIndex1))
  (`GameplayStatics.SaveGameToSlot` _output_get _output_get_2 _output_get_3)
  (`KismetArrayLibrary.Array_Set` (`/Game/Asset/Blueprints/AllSaveData.GameSaveDataList` (`self.AllSaveData`)) _dataindex (make `/Game/Asset/Blueprints/SaveDataStructure` (`KismetStringLibrary.Concat_StrStr` "第" (`KismetStringLibrary.Conv_IntToString` _dataindex) " 时间：" _savedataname) _savedataname _dataindex) true)
  (`GameplayStatics.SaveGameToSlot` (`self.AllSaveData`) "AllGameData"))

(fn `SetDataDetail`
  (params (SaveGameData :type "/Game/Asset/Blueprints/SaveGameTest Object Reference"))
  (returns (SaveGameData1 :type "/Game/Asset/Blueprints/SaveGameTest Object Reference"))
  (return SaveGameData))

(fn `UserConstructionScript`)