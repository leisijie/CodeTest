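; Charge gun that builds a laser while firing, then hits overlapping enemies with the accumulated charge.
; Each GunFire raises ChargeNumber and spends a round, while a Tick gate shows and lengthens a Cube along Y until RoundCheck reaches 2 and flags Overcharge.
; FireLaser reloads through BP_PlayerController, passes ChargeNumber to each BP_Enemy overlapping the Cube, then resets the beam.
; FireOff triggers FireLaser and stops growth.
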(event `self.ReceiveBeginPlay`
  (`parent.ReceiveBeginPlay`)
  (set `self.Round Check` (`self.MaxRound`))
  (bind _output_get (set `self.BasScale` (`SceneComponent.K2_GetComponentScale` (`self.Cube`))))
  (set `self.Scale` _output_get))

(event `self.ReceiveTick`
  (params (DeltaSeconds :type "Float (single-precision)"))
  (bind _cube (`self.Cube`))
  (`/Engine/EditorBlueprintResources/StandardMacros.Gate` true :!label _label
    (:`Exit`
      (`|ExecutionSequence`
        (:`then_0`
          (`/Engine/EditorBlueprintResources/StandardMacros.DoOnce` false :!label _label_2
            (:`Completed`
              (`SceneComponent.SetVisibility` _cube true false))))
        (:`then_1`
          (bind _output_get (set `self.Scale` (`KismetMathLibrary.MakeVector` (.x (`self.Scale`)) (+ (.y (`self.Scale`)) 0.05) (.z (`self.Scale`)))))
          (`SceneComponent.SetWorldScale3D` _cube _output_get))))))

(event `Reset Detect`
  (set `self.ChargeNumber` 0)
  (set `self.Scale` (`self.BasScale`))
  (`SceneComponent.SetVisibility` (`self.Cube`) false false)
  (`|ExecutionSequence`
    (:`then_0`
      (goto _label :!via `Close`))
    (:`then_1`
      (goto _label_2 :!via `Reset`))))

(event `ChargeStart`
  (if (!= (`self.Round Check`) 2)
    (`|ExecutionSequence`
      (:`then_0`
        (goto _label :!via `Open`))
      (:`then_1`
        (`/Engine/EditorBlueprintResources/StandardMacros.Gate` false :!label _label_3
          (:`Exit`
            (set `self.ChargeNumber` (+ (`self.ChargeNumber`) 1))
            (set `self.Round Check` (- (`self.Round Check`) 1))))))
    (else
      (`|ExecutionSequence`
        (:`then_0`
          (goto _label :!via `Close`))
        (:`then_1`
          (set `self.Overcharge` true))))))

(event `FireLaser`
  (bind _cube (`self.Cube`))
  (`|ExecutionSequence`
    (:`then_0`
      (goto _label_3 :!via `Open`))
    (:`then_1`
      (set `self.Round Check` (`self.MaxRound`))
      (set `self.Overcharge` false)
      (bind _asbp_player_controller (cast `/Game/Asset/Blueprints/BP_PlayerController` (`GameplayStatics.GetPlayerController` 0)))
      (`/Game/Asset/Blueprints/BP_PlayerController.Reload` _asbp_player_controller))
    (:`then_2`
      (bind (_outactors _returnvalue) (`KismetSystemLibrary.ComponentOverlapActors` _cube (`SceneComponent.K2_GetComponentToWorld` _cube) (`|MakeArray` "ObjectTypeQuery14" :!type "EObjectTypeQuery Enum")))
      (if _returnvalue
        (for _array_element _outactors
          (bind _asbp_enemy (cast `/Game/Asset/Blueprints/Enemy/BP_Enemy` (`self.GetParentActor` _array_element)))
          (`/Game/Asset/Blueprints/Enemy/BP_Enemy.BeHit` _asbp_enemy (`self.ChargeNumber`))))
      (`self.Reset Detect`))))

(event `self.FireOff`
  (`|ExecutionSequence`
    (:`then_0`
      (goto _label_3 :!via `Close`))
    (:`then_1`
      (`self.FireLaser`))
    (:`then_2`
      (goto _label :!via `Close`))))

(fn `GunFire`
  (params (BePlayer :type Boolean))
  (`self.ChargeStart`)
  (`parent.GunFire` BePlayer))

(fn `UserConstructionScript`
  (`parent.UserConstructionScript`))