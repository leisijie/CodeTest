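; Base Blueprint for a self-aiming gun that tracks and fires at the player's main character, found through BP_PlayerController.
; Each Tick it compares the 2D forward vector from GunMesh to ForwardPoint with the direction to the player.
; Outside the AngularDistance tolerance it turns on yaw only with RInterpTo at AngularVelocity.
; Within tolerance it stops turning and calls GunFire when off cooldown, which a named timer resets after CDTime.
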(event `self.ReceiveBeginPlay`
  (`parent.ReceiveBeginPlay`)
  (bind _asbp_player_controller (cast `/Game/Asset/Blueprints/BP_PlayerController` (`GameplayStatics.GetPlayerController` 0)))
  (set `self.PlayerContorller` _asbp_player_controller))

(event `self.ReceiveTick`
  (params (DeltaSeconds :type "Float (single-precision)"))
  (if (`self.CheckRange`)
    (if (`self.CanFire`)
      (`self.GunFire` false)
      (`self.StartColdDown`))
    (else
      (`self.InterpToPlayer` DeltaSeconds))))

(fn `ColdDown`
  (set `self.CanFire` true))

(fn `UserConstructionScript`
  (`parent.UserConstructionScript`))