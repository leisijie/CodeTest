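; Wave controller actor that runs one stage of a level within a linked chain of waves, with the last showing Victory.
; Activation starts enemy splines after a delay, environment splines and audio.
; The wave ends when polling finds no enemies, time expires or EndThis fires, then activates NextWave.
; A GameInstance-stored name skips preceding waves, while construction-script text and particle targets visualize the links.
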(event `Shine`
  ;[1 1 1] Shine
  (`PrimitiveComponent.SetMaterial` (`self.Cube`) 0 "/Game/Asset/Materials/M_Laser_Inst.M_Laser_Inst")
  (`PrimitiveComponent.SetMaterial` (`self.Cube1`) 0 "/Game/Asset/Materials/M_Laser_Inst.M_Laser_Inst")
  (`PrimitiveComponent.SetMaterial` (`self.TextRender`) 0 "/Game/Asset/Materials/M_Laser_Inst.M_Laser_Inst"))

(event `/Game/Asset/Blueprints/Wave_Control.Wave Control`
  (params (Enemy :type "Actor Object Reference") (`Enter Spline` :type "/Game/Asset/Blueprints/SplineStuff/Move_Actor_Enter Object Reference") (`Enviroment Spline` :type "/Game/Asset/Blueprints/EnviromentSwitch/Move_Line_Enviroment Object Reference"))
  ;[1 1 1] Set Wave
  (`|ExecutionSequence`
    (:`then_0`
      (`/Engine/EditorBlueprintResources/StandardMacros.IsValid` Enemy
        (:`Is Valid`
          (`self.Shine`)
          (`KismetArrayLibrary.Array_Add` (`self.Enemy`) Enemy)
          (`self.Start Detect`))))
    (:`then_1`
      (`/Engine/EditorBlueprintResources/StandardMacros.IsValid` `Enter Spline`
        (:`Is Valid`
          (`KismetArrayLibrary.Array_Add` (`self.EnterSpline`) `Enter Spline`))))
    (:`then_2`
      (`/Engine/EditorBlueprintResources/StandardMacros.IsValid` `Enviroment Spline`
        (:`Is Valid`
          (set `self.BuildingControl` true)
          (`KismetArrayLibrary.Array_Add` (`self.Enviroment`) `Enviroment Spline`))))))

(event `Start Detect`
  ;[1 1 1] Detect
  (`KismetSystemLibrary.K2_SetTimerDelegate` (delegate `Detecting`) 0.1 true))

(event `Detecting`
  (bind _returnvalue (`GameplayStatics.GetPlayerController` 0))
  (bind _next_wave (`self.Next Wave`))
  (bind _close_this_wave (`self.Close This Wave`))
  (bind _progresswidget (`self.ProgressWidget`))
  ;[1 1 1] Detect
  (if (== (`KismetArrayLibrary.Array_Length` (`self.Enemy`)) 0)
    (set `self.Active` false :!label _label)
    (`ActorComponent.SetActive` (`self.Audio`) false true)
    (for _array_element (`self.Enviroment`)
      (`/Game/Asset/Blueprints/EnviromentSwitch/Move_Line_Enviroment.BYEBYE` _array_element))
    (if (`self.Last?`)
      (`/Engine/EditorBlueprintResources/StandardMacros.DoOnce` false
        (:`Completed`
          ;[1 1 1] Victory
          (`WidgetLayoutLibrary.RemoveAllWidgets`)
          (`GameplayStatics.SetGlobalTimeDilation` 0.5)
          (`KismetSystemLibrary.Delay` 0.5)
          (`GameplayStatics.SetGlobalTimeDilation` 1.0)
          (bind _returnvalue_2 (`|CreateWidget` "/Game/Asset/Widget/Victory.Victory_C" _returnvalue))
          (`UserWidget.AddToPlayerScreen` _returnvalue_2 0)
          (`/Game/Asset/Widget/Victory.victory` _returnvalue_2)
          (`WidgetBlueprintLibrary.SetInputMode_UIOnlyEx` _returnvalue null)))
      (else
        (`/Engine/EditorBlueprintResources/StandardMacros.IsValid` _next_wave
          (:`Is Valid`
            (`self.Activate` _next_wave)
            (`|ExecutionSequence`
              (:`then_0`
                (if (not (`self.BuildingControl`))
                  (`/Engine/EditorBlueprintResources/StandardMacros.IsValid` _progresswidget
                    (:`Is Valid`
                      (`/Game/Asset/Widget/LevelScreen/LevelProgress.Break` _progresswidget)))))
              (:`then_1`
                (`/Engine/EditorBlueprintResources/StandardMacros.IsValid` _close_this_wave
                  (:`Is Valid`
                    (`self.EndThis` _close_this_wave))
                  (:`Is Not Valid`
                    _))
                (`self.K2_DestroyActor`)))))))))

(event `self.ReceiveBeginPlay`
  (bind _asbp_gameinstance (cast `/Game/Asset/Blueprints/bp_Gameinstance` (`GameplayStatics.GetGameInstance`)))
  (if (`KismetStringLibrary.EqualEqual_StrStr` (`/Game/Asset/Blueprints/bp_Gameinstance.StoreLevelCounter` _asbp_gameinstance) (`KismetSystemLibrary.GetDisplayName` self))
    (`self.DismisFront`))
  (`KismetSystemLibrary.Delay` 0.1)
  ;[1 1 1] Detect
  (if (`self.First?`)
    (set `self.Counter Number` 0)
    (`self.CountNumberSet`)
    (if (`self.Skip?`) :!label _label_2
      (goto _label)
      (else
        (`|ExecutionSequence`
          (:`then_0`
            (`KismetSystemLibrary.Delay` (`self.Time Befor Wave Start`))
            (for _array_element (`self.EnterSpline`)
              (`/Game/Asset/Blueprints/SplineStuff/Move_Actor_Enter.Active` _array_element)))
          (:`then_1`
            (for _array_element_2 (`self.Enviroment`)
              (`/Game/Asset/Blueprints/EnviromentSwitch/Move_Line_Enviroment.GO` _array_element_2)))
          (:`then_2`
            (`KismetSystemLibrary.Delay` (`self.Time befor end`))
            (goto _label))
          (:`then_3`
            (set `AudioComponent.Sound` (`self.sound`) (`self.Audio`))
            (`ActorComponent.SetActive` (`self.Audio`) true false)))))))

(event `EndThis`
  (goto _label))

(event `Activate`
  (set `self.Active` true)
  (goto _label_2))

(event `DismisFront`
  (bind _pre_wave (`self.Pre_wave`))
  ;[1 1 1] Dismis
  (`/Engine/EditorBlueprintResources/StandardMacros.IsValid` _pre_wave
    (:`Is Valid`
      (set `/Game/Asset/Blueprints/Level_Counter.Skip?` true _pre_wave)
      (`self.DismisFront` _pre_wave))))

(event `CountNumberSet`
  (bind _next_wave (`self.Next Wave`))
  (`TextRenderComponent.K2_SetText` (`self.TextRender`) (`KismetTextLibrary.Conv_StringToText` (`KismetStringLibrary.Concat_StrStr` (`KismetStringLibrary.Conv_IntToString` (`self.Counter Number`)) "///" (`self.Name`))))
  (`/Engine/EditorBlueprintResources/StandardMacros.IsValid` _next_wave
    (:`Is Valid`
      (set `/Game/Asset/Blueprints/Level_Counter.Counter Number` (+ (`self.Counter Number`) 1) _next_wave)
      (`self.CountNumberSet` _next_wave))))

(fn `DeleteActor`
  (params (Enemy :type "/Game/Asset/Blueprints/Enemy/BP_Enemy Object Reference"))
  (`KismetArrayLibrary.Array_RemoveItem` (`self.Enemy`) Enemy))

(fn `UserConstructionScript`
  (locals (LoName :type String))
  (set `local.LoName` (`self.Name`))
  (`ParticleSystemComponent.SetActorParameter` (`self.ParticleSystemNext`) "Target" (`self.Pre_wave`))
  (`ParticleSystemComponent.SetActorParameter` (`self.ParticleSystemEndThis`) "Target" (`self.Close This Wave`))
  (if (`self.Skip?`)
    (set `local.LoName` (`KismetStringLibrary.Concat_StrStr` "SKIP_" (`self.Name`))))
  (`TextRenderComponent.K2_SetText` (`self.TextRender`) (`KismetTextLibrary.Conv_StringToText` (`local.LoName`))))