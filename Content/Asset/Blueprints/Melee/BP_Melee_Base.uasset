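; Base melee weapon child actor of the player character, loading montages, sound and effect class from a data table.
; AttackMainFunction executes a valid target with camera effects, slow motion and timed scene captures, then starts a buff timer, otherwise playing bike and rider montages.
; CollisionDetect gathers enemies in an aim-offset sphere, which mon3 damages while spawning the weapon effect.
; The per-tick buff function is an empty stub.
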(event `self.ReceiveBeginPlay`
  (bind _asbp_gameinstance (cast `/Game/Asset/Blueprints/bp_Gameinstance` (`GameplayStatics.GetGameInstance`)))
  (bind _meleeweapon (`/Game/Asset/Blueprints/bp_Gameinstance.MeleeWeapon` _asbp_gameinstance))
  (if (not (== _meleeweapon "None"))
    (bind _returnvalue (`|GetDataTableRow` "/Game/Asset/Blueprints/DataTable/Meleeweapon_Table.Meleeweapon_Table" _meleeweapon)
      (:`then`
        (bind (_meleename _ingamename _weaponactor _description _caranmiation _chaanmiation _cd _weapon _mesh _icon _sound) (break `/Game/Asset/Blueprints/Struct/Str_Meleeweapon` _returnvalue))
        (set `self.cha` _chaanmiation)
        (set `self.moto` _caranmiation)
        (bind _asbp_player_character (cast `/Game/Asset/Blueprints/Character/BP_PlayerCharacter` (`self.GetParentActor`)))
        (set `self.Character` _asbp_player_character)
        (set `self.cd` _cd)
        (set `self.sword` _weapon)
        (set `self.sound` _sound)))))

(event `SetBuff`
  (`KismetSystemLibrary.K2_SetTimerDelegate` (delegate `EndBuff`) (`self.BuffDuration`))
  (`KismetSystemLibrary.K2_ClearAndInvalidateTimerHandle` (`self.BuffHandle`))
  (if (`self.LoopPerFrame?`)
    (bind _returnvalue (`KismetSystemLibrary.K2_SetTimer` null "ContinuedBuffFunction" 0.0167 true))
    (set `self.BuffHandle` _returnvalue)
    (else
      (bind _returnvalue_2 (`KismetSystemLibrary.K2_SetTimer` null "ContinuedBuffFunction" 1.0 true))
      (set `self.BuffHandle` _returnvalue_2))))

(event `EndBuff`
  (`KismetSystemLibrary.K2_ClearAndInvalidateTimerHandle` (`self.BuffHandle`)))

(event `Execute`
  (params (CloesetEnemy :type "/Game/Asset/Blueprints/Enemy/BP_Enemy Object Reference"))
  (bind _character (`self.Character`))
  (`/Game/Asset/Blueprints/Character/BP_PlayerCharacter.ExecuteCameraStart` _character)
  (`/Game/Asset/Blueprints/BP_PlayerController.StopControll` (`/Game/Asset/Blueprints/Character/BP_PlayerCharacter.PlayerController` _character))
  (`/Game/Asset/Blueprints/Enemy/BP_Enemy.BeHit` CloesetEnemy (`self.Damage`) (`self.K2_GetActorLocation` CloesetEnemy) (`self.Cri`) (`self.ShieldBreakPer`))
  (`|ExecutionSequence`
    (:`then_0`
      (`GameplayStatics.PlaySound2D` (`self.ExecuteSound`) 1.0 1.0 0.0 null null)
      (`KismetSystemLibrary.Delay` 0.4)
      (`/Game/Asset/Blueprints/BP_PlayerController.StartControll` (`/Game/Asset/Blueprints/Character/BP_PlayerCharacter.PlayerController` _character))
      (`/Game/Asset/Blueprints/Character/BP_PlayerCharacter.ExecuteCameraEnd` _character))
    (:`then_1`
      (`self.mon2`))))

(event `mon1`
  (bind _asbp_moto (cast `/Game/Asset/Blueprints/Car/BP_Moto` (`/Game/Asset/Blueprints/Character/BP_PlayerCharacter.Car` (`self.Character`))))
  (`|ExecutionSequence`
    (:`then_0`
      (`|PlayMontage` (`/Game/Asset/Blueprints/Car/BP_Car.Motor` _asbp_moto) (`self.moto`)
        (:`then`
          (`GameplayStatics.PlaySound2D` (`self.sound`) 0.5 1.0 0.0 null null))))
    (:`then_1`
      (`|PlayMontage` (`/Game/Asset/Blueprints/Car/BP_Moto.SkeletalMesh` _asbp_moto) (`self.cha`)
        (:`OnCompleted`
          (set `/Game/Asset/Blueprints/BP_PlayerController.IsAttacking？` false (`/Game/Asset/Blueprints/Character/BP_PlayerCharacter.PlayerController` (`self.Character`))))))))

(event `mon2`
  (bind _asbp_moto (cast `/Game/Asset/Blueprints/Car/BP_Moto` (`/Game/Asset/Blueprints/Character/BP_PlayerCharacter.Car` (`self.Character`))))
  (`|ExecutionSequence`
    (:`then_0`
      (bind _jian (`/Game/Asset/Blueprints/Car/BP_Moto.jian` _asbp_moto))
      (`SceneComponent.SetVisibility` _jian true false)
      (`|PlayMontage` (`/Game/Asset/Blueprints/Car/BP_Moto.SkeletalMesh` _asbp_moto) "/Game/Asset/Animation/cha/ani/sword/Slash_Montage.Slash_Montage"
        (:`then`
          (`PlayerCameraManager.PlayCameraShake` :`self` (`GameplayStatics.GetPlayerCameraManager` 0) :`ShakeClass` "/Game/Asset/Animation/cha/ani/sword/NewBlueprint1.NewBlueprint1_C" :`PlaySpace` "World")
          (`KismetSystemLibrary.Delay` 0.25)
          (`|ExecutionSequence`
            (:`then_0`
              (`GameplayStatics.SetGlobalTimeDilation` 0.2)
              (`KismetSystemLibrary.Delay` 0.1)
              (`GameplayStatics.SetGlobalTimeDilation` 1.0)
              (`|ExecutionSequence`
                (:`then_0`
                  (`SceneComponent.SetVisibility` _jian false false)
                  (set `/Game/Asset/Blueprints/BP_PlayerController.IsAttacking？` false (`/Game/Asset/Blueprints/Character/BP_PlayerCharacter.PlayerController` (`self.Character`))))
                (:`then_1`
                  (`Widget.RemoveFromParent` (stale _returnvalue_3))
                  (`KismetSystemLibrary.K2_ClearAndInvalidateTimerHandle` (stale _returnvalue)))))
            (:`then_1`
              (`KismetSystemLibrary.K2_ClearAndInvalidateTimerHandle` (stale _returnvalue_2))
              (bind _returnvalue (`KismetSystemLibrary.K2_SetTimer` null "CaptureTimer" 0.01 true)))))))
    (:`then_1`
      (bind _skeletalmesh (`/Game/Asset/Blueprints/Car/BP_Moto.SkeletalMesh` _asbp_moto))
      (`GameplayStatics.SpawnEmitterAttached` "/Game/VectorFieldBuilder/1/P_VFEffect12.P_VFEffect12" _skeletalmesh "lizi" (`SceneComponent.K2_GetComponentLocation` _skeletalmesh) (struct) (1.0 1.0 1.0) "KeepWorldPosition"))
    (:`then_2`
      (`KismetSystemLibrary.Delay` 0.1)
      (`|ExecutionSequence`
        (:`then_0`
          (bind _returnvalue_2 (`KismetSystemLibrary.K2_SetTimer` null "CaptureTimer" 0.05 true)))
        (:`then_1`
          (bind _returnvalue_3 (`|CreateWidget` "/Game/Asset/Blueprints/Character/me/mel.mel_C"))
          (`UserWidget.AddToViewport` _returnvalue_3 0))))))

(event `Capture`)

(event `mon3`
  (`self.SpawnEffect` (+ (* (`self.aimDirection`) (`self.DistanceToParent`)) (`self.K2_GetActorLocation` (`self.GetParentActor`))) (`KismetMathLibrary.MakeRotator` 0.0 0.0 (`KismetMathLibrary.DegAtan2` (.y (`self.aimDirection`)) (.x (`self.aimDirection`)))))
  (`self.Hit`))

(event `self.ReceiveTick`
  (params (DeltaSeconds :type "Float (single-precision)")))

(fn `AttackMainFunction`
  (params (CloesetEnemy :type "/Game/Asset/Blueprints/Enemy/BP_Enemy Object Reference"))
  (returns (`IsExecute?` :type Boolean))
  (`/Engine/EditorBlueprintResources/StandardMacros.IsValid` CloesetEnemy
    (:`Is Valid`
      (`self.Execute` CloesetEnemy)
      (`self.SetBuff`)
      (return true))
    (:`Is Not Valid`
      (`self.mon1`)
      (return false))))

(fn `CaptureTimer`
  (bind _asbp_player_character (cast `/Game/Asset/Blueprints/Character/BP_PlayerCharacter` (`GameplayStatics.GetPlayerPawn` 0)))
  (`SceneCaptureComponent2D.CaptureScene` (`/Game/Asset/Blueprints/Character/BP_PlayerCharacter.SceneCaptureComponent2D` _asbp_player_character)))

(fn `CollisionDetect`
  (params (AimDirection :type "Vector Structure"))
  (returns (EnemysInRange :type "Array of /Game/Asset/Blueprints/Enemy/BP_Enemy Object Reference"))
  (`KismetArrayLibrary.Array_Clear` (`self.EnemyInRange`))
  (set `self.aimDirection` AimDirection)
  (bind _outactors (`KismetSystemLibrary.SphereOverlapActors` (+ (* AimDirection (`self.DistanceToParent`)) (`self.K2_GetActorLocation` (`self.GetParentActor`))) (`self.Radius`) (`|MakeArray` "ObjectTypeQuery14" :!type "EObjectTypeQuery Enum")))
  (for _array_element _outactors
    (bind _asbp_enemy (cast `/Game/Asset/Blueprints/Enemy/BP_Enemy` (`self.GetParentActor` _array_element)))
    (`KismetArrayLibrary.Array_Add` (`self.EnemyInRange`) _asbp_enemy))
  (return (`self.EnemyInRange`)))

(fn `ContinuedBuffFunction`)

(fn `Hit`
  (for _array_element (`self.EnemyInRange`)
    (`/Game/Asset/Blueprints/Enemy/BP_Enemy.BeHit` _array_element (`self.Damage`) (`self.K2_GetActorLocation` _array_element) (`self.Cri`) (`self.ShieldBreakPer`))))

(fn `SpawnEffect`
  (params (Location :type "Vector Structure") (Rotation :type "Rotator Structure") (Scale :type "Vector Structure" :default (1.0 1.0 1.0)))
  (bind _returnvalue (`|SpawnActorFromClass` (`self.sword`) (`KismetMathLibrary.MakeTransform` Location (`KismetMathLibrary.MakeRotator` 0.0 0.0 (`KismetMathLibrary.DegAtan2` (.y (`self.aimDirection`)) (.x (`self.aimDirection`)))) Scale) "Undefined" "OverrideRootScale" null null))
  (`self.K2_AttachToActor` _returnvalue (`self.Character`) "None" "KeepWorld" "KeepWorld" "KeepWorld" true))

(fn `UserConstructionScript`
  (set `self.DistanceToParent` (`KismetMathLibrary.VSize` (- (`self.K2_GetActorLocation`) (`self.K2_GetActorLocation` (`self.GetParentActor`)))))
  (`SphereComponent.SetSphereRadius` (`self.Sphere`) (`self.Radius`) false)
  (bind _asbp_player_character (cast `/Game/Asset/Blueprints/Character/BP_PlayerCharacter` (`self.GetParentActor`)))
  (set `/Game/Asset/Blueprints/Character/BP_PlayerCharacter.MeleeWeapon` self _asbp_player_character))