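; Missile actor that homes in on the player pawn and destroys itself five seconds after spawning.
; Each tick it line-traces from its static mesh to the player, filtered by the Target object types, and aims using the hit location.
; It overwrites the mesh's physics velocity with forward motion plus a constant sideways component, giving a curved approach.
; The mesh's X axis is rotated to point away from the hit, so forward travel uses negative X.
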(event `self.ReceiveBeginPlay`
  (`KismetSystemLibrary.Delay` 5.0)
  (`self.K2_DestroyActor`))

(event `self.ReceiveTick`
  (params (DeltaSeconds :type "Float (single-precision)"))
  (bind _staticmesh (`self.StaticMesh`))
  (bind _returnvalue (`SceneComponent.K2_GetComponentLocation` (`self.StaticMesh`)))
  (bind _outhit (`KismetSystemLibrary.LineTraceSingleForObjects` :`Start` (`SceneComponent.K2_GetComponentLocation` (`self.StaticMesh`)) :`End` (`self.K2_GetActorLocation` (`GameplayStatics.GetPlayerPawn` 0)) :`ObjectTypes` (`self.Target`) :`bTraceComplex` true :`DrawTime` 0.2))
  (bind _returnvalue_2 (`KismetMathLibrary.Conv_VectorToRotator` (- _returnvalue (`.Location` (`GameplayStatics.BreakHitResult` _outhit)))))
  (`PrimitiveComponent.SetPhysicsLinearVelocity` _staticmesh (`KismetMathLibrary.TransformDirection` (`KismetMathLibrary.MakeTransform` _returnvalue _returnvalue_2) (`KismetMathLibrary.MakeVector` -1000.0 500.0)) false "None")
  (`SceneComponent.K2_SetWorldRotation` _staticmesh _returnvalue_2 false false))

(fn `UserConstructionScript`)