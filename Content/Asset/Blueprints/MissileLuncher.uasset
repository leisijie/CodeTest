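; Missile launcher Blueprint that repeatedly spawns Supa_Missile actors at the player character's Arrow component location.
; Tick caches that location from BP_PlayerController's MainCharacter each frame.
; When NewVar3 is invalid, a DoOnce on Tick starts an endless delay loop calling Shooot every second, without rechecking the variable.
; Shooot waits a further second, then spawns the missile using only the cached location.
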(event `Shooot`
  (`KismetSystemLibrary.Delay` 1.0)
  (`|SpawnActorFromClass` "/Game/Asset/Blueprints/Supa_Missile.Supa_Missile_C" (`KismetMathLibrary.Conv_VectorToTransform` (`self.NewVar_0`)) "Undefined" "OverrideRootScale" null null))

(event `self.ReceiveTick`
  (params (DeltaSeconds :type "Float (single-precision)"))
  (`|ExecutionSequence`
    (:`then_0`
      (`/Engine/EditorBlueprintResources/StandardMacros.IsValid` (`self.NewVar_3`)
        (:`Is Not Valid`
          (`/Engine/EditorBlueprintResources/StandardMacros.DoOnce` false
            (:`Completed`
              (`self.Shooot` :!label _label)
              (`KismetSystemLibrary.Delay` 1.0)
              (goto _label))))))
    (:`then_1`
      (bind _asbp_player_controller (cast `/Game/Asset/Blueprints/BP_PlayerController` (`GameplayStatics.GetPlayerController` 0)))
      (set `self.NewVar_0` (`SceneComponent.K2_GetComponentLocation` (`/Game/Asset/Blueprints/Character/BP_PlayerCharacter.Arrow` (`/Game/Asset/Blueprints/BP_PlayerController.MainCharacter` _asbp_player_controller)))))))

(fn `UserConstructionScript`)