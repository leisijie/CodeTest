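; Multi-enemy encounter actor that moves a group of child actors along a spline, then destroys itself after a set delay.
; The construction script spawns the chosen class as child actor components evenly spaced along the spline, storing each with a normalized time.
; Every tick, UpdateMove advances and loops those times, remapping them through a float curve to set each component's position and spline-aligned rotation, plus a yaw offset.
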(event `self.ReceiveBeginPlay`
  (`KismetSystemLibrary.Delay` (`self.BYEBYE`))
  (`self.K2_DestroyActor`))

(event `self.ReceiveTick`
  (params (DeltaSeconds :type "Float (single-precision)"))
  (`self.UpdateMove` DeltaSeconds))

(fn `UpdateMove`
  (params (deltaTime :type "Float (double-precision)"))
  (locals (LocalTime :type "Float (double-precision)"))
  (bind _spline (`self.Spline`))
  (for (_array_element _array_index) (`self.Actor_Store`)
    (bind (_actor _time) (break `/Game/Asset/Blueprints/Struct/Str_SplineActor` _array_element))
    (bind _returnvalue (+ _time (/ deltaTime (`self.TotalTime`))))
    (if (>= _returnvalue 1.0)
      (set `local.LocalTime` 0.0)
      (else
        (set `local.LocalTime` _returnvalue)))
    (`/Engine/EditorBlueprintResources/StandardMacros.IsValid` _actor
      (:`Is Valid`
        (`KismetArrayLibrary.Array_Set` (`self.Actor_Store`) _array_index (make `/Game/Asset/Blueprints/Struct/Str_SplineActor` _actor (`local.LocalTime`)))
        (bind _returnvalue_2 (* (`CurveFloat.GetFloatValue` (`self.Curve`) _returnvalue) (`SplineComponent.GetSplineLength` (`self.Spline`))))
        (`SceneComponent.K2_SetWorldLocation` _actor (`SplineComponent.GetLocationAtDistanceAlongSpline` _spline _returnvalue_2 "World") false false)
        (`SceneComponent.K2_SetWorldRotation` _actor (`KismetMathLibrary.MakeRotator` (.roll (`SplineComponent.GetRotationAtDistanceAlongSpline` _spline _returnvalue_2 "World")) (.pitch (`SplineComponent.GetRotationAtDistanceAlongSpline` _spline _returnvalue_2 "World")) (+ (.yaw (`SplineComponent.GetRotationAtDistanceAlongSpline` _spline _returnvalue_2 "World")) (`self.TURN`))) false false)))))

(fn `UserConstructionScript`
  (bind _amount (`self.Amount`))
  (bind _spline (`self.Spline`))
  (`KismetArrayLibrary.Array_Clear` (`self.Actor_Store`))
  (for _index (range _amount)
    (bind _returnvalue (/ (`KismetMathLibrary.Conv_IntToDouble` _index) (`KismetMathLibrary.Conv_IntToDouble` _amount)))
    (bind _returnvalue_2 (* _returnvalue (`SplineComponent.GetSplineLength` _spline)))
    (bind _returnvalue_3 (`AddComponent|NODE_AddChildActorComponent-4` :`RelativeTransform` (`KismetMathLibrary.MakeTransform` (`SplineComponent.GetLocationAtDistanceAlongSpline` _spline _returnvalue_2 "Local") (`SplineComponent.GetRotationAtDistanceAlongSpline` _spline _returnvalue_2 "Local"))))
    (`ChildActorComponent.SetChildActorClass` _returnvalue_3 (`self.Move_budy`))
    (`KismetArrayLibrary.Array_Add` (`self.Actor_Store`) (make `/Game/Asset/Blueprints/Struct/Str_SplineActor` _returnvalue_3 _returnvalue))))