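; Spline-based placer that builds a line of Move_Actor instances along its path.
; The construction script divides the spline length by Space and adds a child actor at each interval, aligned to the spline's local location and rotation.
; An alternative static mesh placement using MoveBudy is left disconnected, and BeginPlay does nothing.
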(event `self.ReceiveBeginPlay`)

(fn `UserConstructionScript`
  (bind _spline (`self.Spline`))
  (bind _space (`self.Space`))
  (for _index (range (+ (`.ReturnValue` (`KismetMathLibrary.FMod` (`SplineComponent.GetSplineLength` _spline) _space)) 1))
    (bind _returnvalue (* _index _space))
    (bind _returnvalue_2 (`AddComponent|NODE_AddChildActorComponent-4` :`RelativeTransform` (`KismetMathLibrary.MakeTransform` (`SplineComponent.GetLocationAtDistanceAlongSpline` _spline _returnvalue "Local") (`SplineComponent.GetRotationAtDistanceAlongSpline` _spline _returnvalue "Local"))))
    (`ChildActorComponent.SetChildActorClass` _returnvalue_2 "/Game/Asset/Blueprints/Move_Actor.Move_Actor_C")))