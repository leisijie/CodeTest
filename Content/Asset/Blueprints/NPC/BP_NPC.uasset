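; BP_NPC is a non-player character that shows speech bubbles and an interaction prompt through widget components.
; BeginPlay applies its skeletal mesh, and UISpeak puts text in a new TalkBubble, which a two-second looping timer clears before cancelling itself.
; CloseNPC and LeaveNPC drive the prompt widget and CLOSE flag, while PressBUttom plays the press and removes it after a brief delay.
; Speaking, Greeting and GoodBye are empty events.
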(event `self.ReceiveBeginPlay`
  (`SkinnedMeshComponent.SetSkinnedAssetAndUpdate` (`self.SkeletalMesh`) (`self.NPC`) true))

(event `UISpeak`
  (params (Word :type String))
  (`|ExecutionSequence`
    (:`then_0`
      (bind _returnvalue (`|CreateWidget` "/Game/Asset/Widget/TalkBubble.TalkBubble_C" (`GameplayStatics.GetPlayerController` 0)))
      (set `self.SpeakBubble` _returnvalue)
      (`WidgetComponent.SetWidget` (`self.Bubble`) _returnvalue)
      (`/Game/Asset/Widget/TalkBubble.Get Player String` _returnvalue Word))
    (:`then_1`
      (bind _returnvalue_2 (`KismetSystemLibrary.K2_SetTimerDelegate` (delegate `ECHO`) 2.0 true)))))

(event `Speaking`)

(event `Clear`
  (bind _speakbubble (`self.SpeakBubble`))
  (if (not (`/Game/Asset/Widget/TalkBubble.Clear?` _speakbubble))
    (`/Game/Asset/Widget/TalkBubble.Clear` _speakbubble)))

(event `Greeting`)

(event `GoodBye`)

(event `ECHO`
  (`self.Clear`)
  (`KismetSystemLibrary.K2_ClearAndInvalidateTimerHandle` (stale `UISpeak` _returnvalue_2)))

(event `PressBUttom`
  (bind _presss (`self.Presss`))
  (`/Engine/EditorBlueprintResources/StandardMacros.IsValid` _presss
    (:`Is Valid`
      (`/Game/Asset/Widget/NPC_Interact.PressX` _presss)
      (`KismetSystemLibrary.Delay` 0.25)
      (`WidgetComponent.SetWidget` (`self.Press`) null))))

(event `CloseNPC`
  (bind _returnvalue (`|CreateWidget` "/Game/Asset/Widget/NPC_Interact.NPC_Interact_C" (`GameplayStatics.GetPlayerController` 0)))
  (`WidgetComponent.SetWidget` (`self.Press`) _returnvalue)
  (set `self.Presss` _returnvalue)
  (`/Game/Asset/Widget/NPC_Interact.Come` (`self.Presss`))
  (set `self.CLOSE` true))

(event `LeaveNPC`
  (bind _presss (`self.Presss`))
  (`/Engine/EditorBlueprintResources/StandardMacros.IsValid` _presss
    (:`Is Valid`
      (`/Game/Asset/Widget/NPC_Interact.Left` _presss))
    (:`Is Not Valid`
      _))
  (set `self.CLOSE` false))

(fn `UserConstructionScript`)