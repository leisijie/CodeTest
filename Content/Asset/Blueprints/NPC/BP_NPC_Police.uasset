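; BP_NPC_Police is the police officer NPC, a child Blueprint that sets the officer's animations for conversation events.
; BeginPlay defers to the parent, while Speaking loops the talking animation, Greeting plays it once and GoodBye returns to a looping breathing idle.
; Disconnected nodes that would load common NPC lines and progress-keyed speech from data tables remain in the graph but never run.
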(event `self.ReceiveBeginPlay`
  (`parent.ReceiveBeginPlay`))

(event `self.Speaking`
  (`SkeletalMeshComponent.PlayAnimation` (`self.SkeletalMesh`) "/Game/Asset/Animation/NPC/Police_Talking_Anim_mixamo_com.Police_Talking_Anim_mixamo_com" true))

(event `self.Greeting`
  (`SkeletalMeshComponent.PlayAnimation` (`self.SkeletalMesh`) "/Game/Asset/Animation/NPC/Police_Talking_Anim_mixamo_com.Police_Talking_Anim_mixamo_com" false))

(event `self.GoodBye`
  (`SkeletalMeshComponent.PlayAnimation` (`self.SkeletalMesh`) "/Game/Asset/Animation/NPC/Police_Breathing_Idle_Anim_mixamo_com.Police_Breathing_Idle_Anim_mixamo_com" true))

(fn `UserConstructionScript`
  (`parent.UserConstructionScript`))