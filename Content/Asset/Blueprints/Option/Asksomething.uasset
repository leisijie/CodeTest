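; Interaction trigger that runs NPC conversations and can also show an announcement UI or switch levels after a blackout.
; BeginPlay creates the Dialogue widget and copies speech text from the assigned NPC.
; Overlapping DetectArea drives greetings, farewells and a looping timer that checks player distance.
; When close, Interact steps through conversation lines, then opens the question menu, with DoOnce and Gate nodes controlling one-time steps.
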(event `/Game/Asset/Blueprints/Interaction.PlayerInterraction`
  ;[1 0.5369 0.386] Player Control
  (`self.Interact`))

(event `self.ReceiveBeginPlay`
  (bind _npc (`self.NPC`))
  ;[1 0.5369 0.386] Begin
  (`KismetSystemLibrary.Delay` 0.2)
  (bind _returnvalue (`|CreateWidget` "/Game/Asset/Blueprints/Option/Dialogue.Dialogue_C"))
  (bind _output_get (set `self.Dialogue` _returnvalue))
  (set `/Game/Asset/Blueprints/Option/Dialogue.Owner` self _output_get)
  (`/Engine/EditorBlueprintResources/StandardMacros.IsValid` _npc
    (:`Is Valid`
      (set `/Game/Asset/Blueprints/NPC/BP_NPC.AskOwner` self _npc)
      (`/Game/Asset/Blueprints/Option/Dialogue.BeginSet` (`self.Dialogue`) (`self.NPC`))
      (`self.SetSpeachText`))))

(event `ResetADD`
  (bind _npc (`self.NPC`))
  (bind _npc_2 (`self.NPC`))
  (bind _dialogue (`self.Dialogue`))
  (`|ExecutionSequence`
    (:`then_0`
      (goto _label_2 :!via `Reset`))
    (:`then_1`
      (goto _label_3 :!via `Reset`))))

(event `Interact`
  (bind _npc (`self.NPC`))
  (bind _npc_2 (`self.NPC`))
  (bind _npc_3 (`self.NPC`))
  (bind _npc_4 (`self.NPC`))
  (bind _npc_5 (`self.NPC`))
  (bind _dialogue (`self.Dialogue`))
  (bind _level_name (`self.level Name`))
  (`|ExecutionSequence`
    (:`then_0`
      (if (`self.CloseEnough？`)
        ;[1 1 1] IS Done?
        (if (== (`self.Which To Speak`) (`KismetArrayLibrary.Array_Length` (`self.Conversation`)))
          (set `self.IsFinished` true))
        (if (`self.IsFinished`)
          (`|ExecutionSequence`
            (:`then_0`
              ;[1 1 1] Done
              (`/Engine/EditorBlueprintResources/StandardMacros.DoOnce` false
                (:`Completed`
                  (`/Game/Asset/Blueprints/Option/Dialogue.Clear` (`self.Dialogue`))
                  (`/Engine/EditorBlueprintResources/StandardMacros.IsValid` _npc_3
                    (:`Is Valid`
                      (`/Game/Asset/Blueprints/NPC/BP_NPC.UISpeak` _npc_3 (`KismetTextLibrary.Conv_TextToString` (`|GetArrayItem` (`self.AfterDone`))))
                      (`/Game/Asset/Blueprints/NPC/BP_NPC.CloseNPC` (`self.NPC`)))))))
            (:`then_1`
              (`/Engine/EditorBlueprintResources/StandardMacros.Gate` true :!label _label
                (:`Exit`
                  (`|ExecutionSequence`
                    (:`then_0`
                      ;[1 1 1] ReSpeak
                      (`/Engine/EditorBlueprintResources/StandardMacros.DoOnce` false :!label _label_2
                        (:`Completed`
                          (`/Game/Asset/Blueprints/Option/Dialogue.Clear` _dialogue)
                          (`UserWidget.AddToViewport` _dialogue 0)
                          (`/Engine/EditorBlueprintResources/StandardMacros.IsValid` _npc_4
                            (:`Is Valid`
                              (`/Game/Asset/Blueprints/NPC/BP_NPC.Clear` _npc_4))))))
                    (:`then_1`
                      ;[1 1 1] Question
                      (`/Game/Asset/Blueprints/Option/Dialogue.QuestionBegin` (`self.Dialogue`) (`self.StartQuestion`) (`self.PlayerAsk`) (`self.NPCAnser`)))
                    (:`then_2`
                      (`/Engine/EditorBlueprintResources/StandardMacros.IsValid` _npc_5
                        (:`Is Valid`
                          (`/Game/Asset/Blueprints/NPC/BP_NPC.Speaking` _npc_5)
                          (`/Game/Asset/Blueprints/NPC/BP_NPC.PressBUttom` _npc_5))))))))
            (:`then_2`
              (goto _label :!via `Open`)))
          (else
            (`|ExecutionSequence`
              (:`then_0`
                ;[1 1 1] Speak
                (`/Engine/EditorBlueprintResources/StandardMacros.DoOnce` false :!label _label_3
                  (:`Completed`
                    (`UserWidget.AddToViewport` (`self.Dialogue`) 0)
                    (`/Engine/EditorBlueprintResources/StandardMacros.IsValid` _npc
                      (:`Is Valid`
                        (`/Game/Asset/Blueprints/NPC/BP_NPC.Clear` _npc))))))
              (:`then_1`
                ;[1 1 1] conversation
                (`/Game/Asset/Blueprints/Option/Dialogue.Say` (`self.Dialogue`) (`|GetArrayItem` (`self.Conversation`) (`self.Which To Speak`)))
                (set `self.Which To Speak` (+ (`self.Which To Speak`) 1)))
              (:`then_2`
                (`/Engine/EditorBlueprintResources/StandardMacros.IsValid` _npc_2
                  (:`Is Valid`
                    (`/Game/Asset/Blueprints/NPC/BP_NPC.Speaking` _npc_2)
                    (`/Game/Asset/Blueprints/NPC/BP_NPC.PressBUttom` _npc_2)))))))))
    (:`then_1`
      ;[1 0.8806 0.41 1 20] SwitchLevel
      (if (`self.SwitchLevel`)
        (if (not (== _level_name "None"))
          (bind _returnvalue (`|CreateWidget` "/Game/Asset/Widget/Switch_Blackout.Switch_Blackout_C" (`GameplayStatics.GetPlayerController` 0)))
          (`UserWidget.AddToViewport` _returnvalue 0)
          (`KismetSystemLibrary.Delay` 0.5)
          (`GameplayStatics.OpenLevel` _level_name))))))

(event `self.DetectArea.OnComponentBeginOverlap`
  (params (OverlappedComponent :type "PrimitiveComponent Object Reference") (OtherActor :type "Actor Object Reference") (OtherComp :type "PrimitiveComponent Object Reference") (OtherBodyIndex :type Integer) (bFromSweep :type Boolean) (SweepResult :type "HitResult Structure (by ref)"))
  (bind _npc (`self.NPC`))
  (bind _anythingelse (`self.AnythingElse`))
  (bind _npc_2 (`self.NPC`))
  (bind _npc_3 (`self.NPC`))
  (bind _memory (`self.Memory`))
  ;[1 1 1 1 50] INTER
  (set `self.Player` OtherActor)
  (set `self.PlayerHere` true)
  (`|ExecutionSequence`
    (:`then_1`
      (if (`self.UIAnnounce`)
        ;[1 1 1] UI Only
        (bind _returnvalue (`|CreateWidget` "/Game/Asset/Blueprints/Option/TopUI.TopUI_C" (`GameplayStatics.GetPlayerController` 0)))
        (set `self.UIwidget` _returnvalue)
        (set `/Game/Asset/Blueprints/Option/TopUI.Owner` self _returnvalue)
        (`WidgetComponent.SetWidget` (`self.Widget`) _returnvalue)
        (`/Game/Asset/Blueprints/Option/TopUI.Get Player String` _returnvalue (`self.Player`) (`self.UI`) (`self.SwitchLevel`))
        (else
          ;[1 1 1] Hello
          (if (`self.IsFinished`)
            (`/Engine/EditorBlueprintResources/StandardMacros.IsValid` _npc
              (:`Is Valid`
                (`/Game/Asset/Blueprints/NPC/BP_NPC.UISpeak` _npc (`KismetTextLibrary.Conv_TextToString` (`|GetArrayItem` _anythingelse (`KismetMathLibrary.RandomInteger` (`KismetArrayLibrary.Array_Length` _anythingelse)))))
                (if true
                  _)))
            (else
              (`|ExecutionSequence`
                (:`then_0`
                  (`/Engine/EditorBlueprintResources/StandardMacros.IsValid` _npc_3
                    (:`Is Valid`
                      (`/Game/Asset/Blueprints/NPC/BP_NPC.UISpeak` _npc_3 (`KismetTextLibrary.Conv_TextToString` (`|GetArrayItem` _memory (`KismetMathLibrary.RandomInteger` (`KismetArrayLibrary.Array_Length` _memory))))))))
                (:`then_1`
                  (`/Engine/EditorBlueprintResources/StandardMacros.DoOnce` false
                    (:`Completed`
                      (`/Engine/EditorBlueprintResources/StandardMacros.IsValid` _npc_2
                        (:`Is Valid`
                          (`/Game/Asset/Blueprints/NPC/BP_NPC.UISpeak` _npc_2 (`KismetTextLibrary.Conv_TextToString` (`self.Meet`))))))))))))))
    (:`then_2`
      (`/Engine/EditorBlueprintResources/StandardMacros.IsValid` (`self.NPC`)
        (:`Is Valid`
          (`/Game/Asset/Blueprints/NPC/BP_NPC.Greeting` (`self.NPC`))
          (bind _returnvalue_2 (`KismetSystemLibrary.K2_SetTimer` null "DetectLength" 0.05 true)))))))

(event `CloseEnough`
  (bind _npc (`self.NPC`))
  ;[1 1 1 1 37] DistanceDetect
  (`|ExecutionSequence`
    (:`then_0`
      (`/Engine/EditorBlueprintResources/StandardMacros.DoOnce` false :!label _label_4
        (:`Completed`
          (`/Game/Asset/Blueprints/NPC/BP_NPC.CloseNPC` _npc)
          (set `self.CloseEnough？` true))))
    (:`then_1`
      (goto _label_5 :!via `Reset`))))

(event `TooFar`
  ;[1 1 1 1 37] DistanceDetect
  (`|ExecutionSequence`
    (:`then_0`
      (goto _label_4 :!via `Reset`))
    (:`then_1`
      (`/Engine/EditorBlueprintResources/StandardMacros.DoOnce` false :!label _label_5
        (:`Completed`
          (`/Game/Asset/Blueprints/NPC/BP_NPC.LeaveNPC` (`self.NPC`))
          (set `self.CloseEnough？` false))))))

(event `self.DetectArea.OnComponentEndOverlap`
  (params (OverlappedComponent :type "PrimitiveComponent Object Reference") (OtherActor :type "Actor Object Reference") (OtherComp :type "PrimitiveComponent Object Reference") (OtherBodyIndex :type Integer))
  (bind _uiwidget (`self.UIwidget`))
  (bind _npc (`self.NPC`))
  (bind _wait (`self.Wait`))
  (bind _afterdone (`self.AfterDone`))
  (bind _npc_2 (`self.NPC`))
  (bind _npc_3 (`self.NPC`))
  ;[1 1 1] Bye~
  (set `self.PlayerHere` false)
  (`/Engine/EditorBlueprintResources/StandardMacros.IsValid` _npc_3
    (:`Is Valid`
      (`|ExecutionSequence`
        (:`then_0`
          (`/Game/Asset/Blueprints/NPC/BP_NPC.Clear` _npc_3)
          (`KismetSystemLibrary.K2_ClearAndInvalidateTimerHandle` (stale `self.DetectArea.OnComponentBeginOverlap` _returnvalue_2))
          (`/Engine/EditorBlueprintResources/StandardMacros.IsValid` _uiwidget :!label _label_6
            (:`Is Valid`
              (`/Game/Asset/Blueprints/Option/TopUI.Clear` _uiwidget))
            (:`Is Not Valid`
              (`/Game/Asset/Blueprints/Option/Dialogue.Clear` (`self.Dialogue`))
              (`self.ResetADD`))))
        (:`then_1`
          (`/Game/Asset/Blueprints/NPC/BP_NPC.GoodBye` (`self.NPC`))
          (if (`self.IsFinished`)
            ;[1 1 1] GoodLuck
            (`/Engine/EditorBlueprintResources/StandardMacros.IsValid` _npc_2
              (:`Is Valid`
                (`/Game/Asset/Blueprints/NPC/BP_NPC.UISpeak` _npc_2 (`KismetTextLibrary.Conv_TextToString` (`|GetArrayItem` _afterdone (`KismetMathLibrary.RandomInteger` (`KismetArrayLibrary.Array_Length` _afterdone)))))))
            (else
              ;[1 1 1] HEY WAIT
              (`/Engine/EditorBlueprintResources/StandardMacros.IsValid` _npc
                (:`Is Valid`
                  (`/Game/Asset/Blueprints/NPC/BP_NPC.UISpeak` _npc (`KismetTextLibrary.Conv_TextToString` (`|GetArrayItem` _wait (`KismetMathLibrary.RandomInteger` (`KismetArrayLibrary.Array_Length` _wait))))))))))))
    (:`Is Not Valid`
      (goto _label_6))))

(fn `DetectLength`
  (if (< (`self.GetDistanceTo` (`self.NPC`) (`GameplayStatics.GetPlayerCharacter` 0)) 300.0)
    (`self.CloseEnough`)
    (else
      (`self.TooFar`))))

(fn `SetSpeachText`
  (bind _npc (`self.NPC`))
  (set `self.Meet` (`/Game/Asset/Blueprints/NPC/BP_NPC.Meet` _npc))
  (set `self.Memory` (`/Game/Asset/Blueprints/NPC/BP_NPC.ReMeet` _npc))
  (set `self.Conversation` (`/Game/Asset/Blueprints/NPC/BP_NPC.Conversation` _npc))
  (set `self.Wait` (`/Game/Asset/Blueprints/NPC/BP_NPC.AskForComeBack` _npc))
  (set `self.AnythingElse` (`/Game/Asset/Blueprints/NPC/BP_NPC.Anythingelse` _npc))
  (set `self.AfterDone` (`/Game/Asset/Blueprints/NPC/BP_NPC.AfterDone` _npc))
  (set `self.StartQuestion` (`/Game/Asset/Blueprints/NPC/BP_NPC.StartQuestion` _npc))
  (set `self.PlayerAsk` (`/Game/Asset/Blueprints/NPC/BP_NPC.PlayerAsk` _npc))
  (set `self.NPCAnser` (`/Game/Asset/Blueprints/NPC/BP_NPC.NPCAnswer` _npc))
  (return))

(fn `UserConstructionScript`)