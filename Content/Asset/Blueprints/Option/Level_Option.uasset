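; Level_Option is a trigger actor that opens the Main_MapContainer UI when an actor overlaps its Trigger component.
; On overlap it blends the player's view to itself, disables input on the overlapping actor, then creates the widget and shows it with UI-only input focus.
; Ending the overlap only removes the widget; view target, actor input and input mode are not restored here.
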(event `self.trigger.OnComponentBeginOverlap`
  (params (OverlappedComponent :type "PrimitiveComponent Object Reference") (OtherActor :type "Actor Object Reference") (OtherComp :type "PrimitiveComponent Object Reference") (OtherBodyIndex :type Integer) (bFromSweep :type Boolean) (SweepResult :type "HitResult Structure (by ref)"))
  (bind _returnvalue (`GameplayStatics.GetPlayerController` 0))
  (`PlayerController.SetViewTargetWithBlend` _returnvalue self 0.5 "VTBlend_Linear" 0.0 false)
  (bind _returnvalue_2 (`|CreateWidget` "/Game/Asset/Widget/Map/Main_MapContainer.Main_MapContainer_C" _returnvalue))
  (set `self.MainMapUI` _returnvalue_2)
  (`self.DisableInput` OtherActor _returnvalue)
  (`WidgetBlueprintLibrary.SetInputMode_UIOnlyEx` _returnvalue _returnvalue_2)
  (`UserWidget.AddToViewport` _returnvalue_2 0))

(event `self.trigger.OnComponentEndOverlap`
  (params (OverlappedComponent :type "PrimitiveComponent Object Reference") (OtherActor :type "Actor Object Reference") (OtherComp :type "PrimitiveComponent Object Reference") (OtherBodyIndex :type Integer))
  (`Widget.RemoveFromParent` (`self.MainMapUI`)))

(fn `UserConstructionScript`)