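; Map switch point actor that opens a map menu when an actor overlaps its trigger and sets up travel to a level.
; The overlap clears widgets, blends the camera to itself, disables the overlapping actor's input and shows Main_MapContainer in UI-only mode, passing it both actors.
; OpenLevelTime looks up a row name in Map_Level_Table and hands the level name and switch flag to OpenLevel.
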(event `self.trigger.OnComponentBeginOverlap`
  (params (OverlappedComponent :type "PrimitiveComponent Object Reference") (OtherActor :type "Actor Object Reference") (OtherComp :type "PrimitiveComponent Object Reference") (OtherBodyIndex :type Integer) (bFromSweep :type Boolean) (SweepResult :type "HitResult Structure (by ref)"))
  (bind _returnvalue (`GameplayStatics.GetPlayerController` 0))
  (`WidgetLayoutLibrary.RemoveAllWidgets`)
  (`PlayerController.SetViewTargetWithBlend` _returnvalue self 1.0 "VTBlend_Cubic" 0.0 false)
  (bind _returnvalue_2 (`|CreateWidget` "/Game/Asset/Widget/Map/Main_MapContainer.Main_MapContainer_C" _returnvalue))
  (set `self.MainMapUI` _returnvalue_2)
  (`self.DisableInput` OtherActor _returnvalue)
  (`WidgetBlueprintLibrary.SetInputMode_UIOnlyEx` _returnvalue _returnvalue_2)
  (`UserWidget.AddToViewport` _returnvalue_2 0)
  (set `/Game/Asset/Widget/Map/Main_MapContainer.Player` OtherActor _returnvalue_2)
  (set `/Game/Asset/Widget/Map/Main_MapContainer.Owner` self _returnvalue_2))

(event `OpenLevelTime`
  (params (Name :type Name))
  (bind _openlevel (`self.OpenLevel`))
  (bind _returnvalue (`|GetDataTableRow` "/Game/Asset/Blueprints/DataTable/Map_Level_Table.Map_Level_Table" Name)
    (:`then`
      (set `/Game/Asset/Blueprints/Option/Asksomething.SwitchLevel` true _openlevel)
      (set `/Game/Asset/Blueprints/Option/Asksomething.level Name` (`.OpenLevelName_28_3F0F4BB047A384856C0552B6A864941F` (break `/Game/Asset/Blueprints/Struct/Map_Str` _returnvalue)) _openlevel))))

(fn `UserConstructionScript`)