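; MapSwitchOption1 is an interactable option actor that shows a "mysterious" prompt and opens an input screen.
; Overlapping its Trigger creates a TopUI in its Widget component and passes it the player and prompt text; leaving clears it.
; PlayerInterraction adds an Input widget to the viewport and switches to UI-only input.
; GetLevel is empty, and the file itself performs no map switch.
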(event `self.trigger.OnComponentBeginOverlap`
  (params (OverlappedComponent :type "PrimitiveComponent Object Reference") (OtherActor :type "Actor Object Reference") (OtherComp :type "PrimitiveComponent Object Reference") (OtherBodyIndex :type Integer) (bFromSweep :type Boolean) (SweepResult :type "HitResult Structure (by ref)"))
  (set `self.player` OtherActor)
  (bind _returnvalue (`|CreateWidget` "/Game/Asset/Blueprints/Option/TopUI.TopUI_C" (`GameplayStatics.GetPlayerController` 0)))
  (bind _output_get (set `self.TOPUI` _returnvalue))
  (`WidgetComponent.SetWidget` (`self.Widget`) _output_get)
  (`/Game/Asset/Blueprints/Option/TopUI.Get Player String` _output_get (`self.player`) "神秘，太神秘了" true))

(event `self.trigger.OnComponentEndOverlap`
  (params (OverlappedComponent :type "PrimitiveComponent Object Reference") (OtherActor :type "Actor Object Reference") (OtherComp :type "PrimitiveComponent Object Reference") (OtherBodyIndex :type Integer))
  (bind _topui (`self.TOPUI`))
  (`/Engine/EditorBlueprintResources/StandardMacros.IsValid` _topui
    (:`Is Valid`
      (`/Game/Asset/Blueprints/Option/TopUI.Clear` _topui))))

(event `/Game/Asset/Blueprints/Interaction.PlayerInterraction`
  (bind _returnvalue (`GameplayStatics.GetPlayerController` 0))
  (bind _returnvalue_2 (`|CreateWidget` "/Game/Asset/Blueprints/Option/input.input_C" _returnvalue))
  (`WidgetBlueprintLibrary.SetInputMode_UIOnlyEx` _returnvalue _returnvalue_2)
  (`UserWidget.AddToViewport` _returnvalue_2 0))

(fn `Get Level`)

(fn `UserConstructionScript`)