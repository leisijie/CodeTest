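; Interactable loadout station where the player inspects and selects weapons, trinkets and a melee weapon.
; Overlap shows a prompt; interacting blends the view to the station, swaps the player for a display actor, starts the platform and opens the A_Select_main UI.
; Timelines lerp between weapon and trinket camera transforms.
; Finish, gated by a DoOnce re-armed on each start, saves choices to the game instance, readies the platform and restores player control.
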(event `/Game/Asset/Blueprints/Interaction.PlayerInterraction`
  (`self.StartOption`))

(event `self.Box.OnComponentBeginOverlap`
  (params (OverlappedComponent :type "PrimitiveComponent Object Reference") (OtherActor :type "Actor Object Reference") (OtherComp :type "PrimitiveComponent Object Reference") (OtherBodyIndex :type Integer) (bFromSweep :type Boolean) (SweepResult :type "HitResult Structure (by ref)"))
  (set `self.Player` OtherActor)
  (bind _returnvalue (`|CreateWidget` "/Game/Asset/Blueprints/Option/TopUI.TopUI_C" (`GameplayStatics.GetPlayerController` 0)))
  (bind _output_get (set `self.TopUI` _returnvalue))
  (`WidgetComponent.SetWidget` (`self.Widget1`) _output_get)
  (`/Game/Asset/Blueprints/Option/TopUI.Get Player String` _output_get (`self.player`) "检查武器" true))

(event `self.Box.OnComponentEndOverlap`
  (params (OverlappedComponent :type "PrimitiveComponent Object Reference") (OtherActor :type "Actor Object Reference") (OtherComp :type "PrimitiveComponent Object Reference") (OtherBodyIndex :type Integer))
  (bind _topui (`self.TopUI`))
  (`/Engine/EditorBlueprintResources/StandardMacros.IsValid` _topui
    (:`Is Valid`
      (`/Game/Asset/Blueprints/Option/TopUI.Clear` _topui))))

(event `self.ReceiveBeginPlay`
  ;[1 1 1] BeginPlay CAR
  (`self.SetActorHiddenInGame` (`self.Show`) true)
  (`ActorComponent.SetActive` (`self.Camera_weapon`) false false)
  (`ActorComponent.SetActive` (`self.Camera_Trinket`) false false))

(event `StartOption`
  (bind _returnvalue (`GameplayStatics.GetPlayerController` 0))
  (bind _returnvalue_2 (`GameplayStatics.GetPlayerController` 0))
  (bind _topui (`self.TopUI`))
  (bind _player (`self.Player`))
  (bind _carplateform (`self.CarPlateform`))
  (bind _carplateform_2 (`self.CarPlateform`))
  ;[0.8234 0.7067 1] Start
  (`|ExecutionSequence`
    (:`then_0`
      (`/Engine/EditorBlueprintResources/StandardMacros.IsValid` _topui
        (:`Is Valid`
          (`/Game/Asset/Blueprints/Option/TopUI.Clear` _topui))
        (:`Is Not Valid`
          _))
      (`PlayerController.SetViewTargetWithBlend` (`GameplayStatics.GetPlayerController` 0) self 1.0 "VTBlend_Cubic" 0.0 false)
      (`|ExecutionSequence`
        (:`then_0`
          (bind (_direction _move) (`Timeline|Timeline_1` :!via `PlayFromStart`)
            (:`Update`
              (`SceneComponent.K2_SetWorldLocationAndRotation` (`self.000`) (.location (`KismetMathLibrary.TLerp` (`SceneComponent.K2_GetComponentToWorld` (`self.000`)) (`SceneComponent.K2_GetComponentToWorld` (`self.Camera_weapon`)) _move)) (.rotation (`KismetMathLibrary.TLerp` (`SceneComponent.K2_GetComponentToWorld` (`self.000`)) (`SceneComponent.K2_GetComponentToWorld` (`self.Camera_weapon`)) _move)) true false))
            (:`Finished`
              ;[1 1 1] Add Widget
              (bind _returnvalue_3 (`|CreateWidget` "/Game/Asset/Widget/SwitchWidget/A_Select_main.A_Select_main_C" _returnvalue))
              (set `self.Widget` _returnvalue_3)
              (set `/Game/Asset/Widget/SwitchWidget/A_Select_main.Owner` self _returnvalue_3)
              (`self.DisableInput` (`self.Player`) _returnvalue)
              (`WidgetBlueprintLibrary.SetInputMode_UIOnlyEx` _returnvalue _returnvalue_3)
              (`/Game/Asset/Widget/SwitchWidget/A_Select_main.Get Car` _returnvalue_3 (`self.CAR`))
              (`UserWidget.AddToViewport` _returnvalue_3 0))))
        (:`then_1`
          (`KismetSystemLibrary.Delay` 0.45)
          (`self.SetActorHiddenInGame` (`self.Show`) false)
          (`self.SetActorHiddenInGame` (`self.Player`) true))
        (:`then_2`
          (goto _label :!via `Reset`))))
    (:`then_1`
      (`/Engine/EditorBlueprintResources/StandardMacros.IsValid` _carplateform
        (:`Is Valid`
          (`/Game/Asset/Blueprints/CarPlatform.Start` _carplateform))))))

(event `Cacu Widget`
  ;[1 1 1] Finish
  (`/Game/Asset/Widget/SwitchWidget/A_Select_main.Get Setting` (`self.Widget`)))

(event `Finish`
  (params (l_Weapon :type Name) (R_Weapon :type Name) (Trinkets :type "Array of Name") (Melee :type Name))
  (bind _returnvalue (`GameplayStatics.GetPlayerController` 0))
  (bind _player (`self.Player`))
  (bind _carplateform (`self.CarPlateform`))
  ;[1 1 1] Finish
  (`/Engine/EditorBlueprintResources/StandardMacros.DoOnce` false :!label _label
    (:`Completed`
      (bind _asbp_gameinstance (cast `/Game/Asset/Blueprints/bp_Gameinstance` (`GameplayStatics.GetGameInstance`)))
      (set `/Game/Asset/Blueprints/bp_Gameinstance.L_Weapon` l_Weapon _asbp_gameinstance)
      (set `/Game/Asset/Blueprints/bp_Gameinstance.R_Weapon` R_Weapon _asbp_gameinstance)
      (set `/Game/Asset/Blueprints/bp_Gameinstance.Trinkets` Trinkets _asbp_gameinstance)
      (set `/Game/Asset/Blueprints/bp_Gameinstance.MeleeWeapon` Melee _asbp_gameinstance)
      (`|ExecutionSequence`
        (:`then_0`
          ;;[1 1 1] Leave Area
          (`/Engine/EditorBlueprintResources/StandardMacros.IsValid` _carplateform
            (:`Is Valid`
              (`/Game/Asset/Blueprints/CarPlatform.GetREady` _carplateform))))
        (:`then_1`
          (`KismetSystemLibrary.Delay` 1.0)
          (`WidgetBlueprintLibrary.SetInputMode_GameOnly` _returnvalue)
          (`self.EnableInput` _player _returnvalue)
          (`PlayerController.SetViewTargetWithBlend` _returnvalue _player 0.0 "VTBlend_Linear" 0.0 false)
          (`self.SetActorHiddenInGame` (`self.Show`) true)
          (`self.SetActorHiddenInGame` (`self.Player`) false))))))

(event `SwitchCameraTrinket`
  ;[1 0.7901 0.1603] MainWidggetSwitchControl
  (`/Game/Asset/Widget/SwitchWidget/A_Select_main.OpenTrinkets` (`self.Widget`))
  (set `self.switchING` true)
  (bind (_direction _move) (`Timeline|MoveCamera` :!via `PlayFromStart`)
    (:`Update`
      (`SceneComponent.K2_SetWorldLocationAndRotation` (`self.000`) (.location (`KismetMathLibrary.TLerp` (`SceneComponent.K2_GetComponentToWorld` (`self.000`)) (`SceneComponent.K2_GetComponentToWorld` (`self.Camera_Trinket`)) _move)) (.rotation (`KismetMathLibrary.TLerp` (`SceneComponent.K2_GetComponentToWorld` (`self.000`)) (`SceneComponent.K2_GetComponentToWorld` (`self.Camera_Trinket`)) _move)) true false))
    (:`Finished`
      (set `self.switchING` false))))

(event `SwitchCameraWeapon`
  ;[1 0.7901 0.1603] MainWidggetSwitchControl
  (`/Game/Asset/Widget/SwitchWidget/A_Select_main.openWeapons` (`self.Widget`))
  (set `self.switchING` true)
  (bind (_direction _move) (`Timeline|Timeline_0` :!via `PlayFromStart`)
    (:`Update`
      (`SceneComponent.K2_SetWorldLocationAndRotation` (`self.000`) (.location (`KismetMathLibrary.TLerp` (`SceneComponent.K2_GetComponentToWorld` (`self.000`)) (`SceneComponent.K2_GetComponentToWorld` (`self.Camera_weapon`)) _move)) (.rotation (`KismetMathLibrary.TLerp` (`SceneComponent.K2_GetComponentToWorld` (`self.000`)) (`SceneComponent.K2_GetComponentToWorld` (`self.Camera_weapon`)) _move)) true false))
    (:`Finished`
      (set `self.switchING` false))))

(fn `UserConstructionScript`)