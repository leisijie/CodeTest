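; Player bullet that damages enemy drivers through the cars they occupy.
; BeginPlay launches its box along the forward vector with physics velocity, while a looping timer tallies distance and destroys it past max range.
; Hits branch on the target's first tag: enemy and car hits apply damage with shield break, impact effect and scorch decal; others just destroy it.
; Critical boost and reported crit flag come from separate random-roll calls.
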(event `self.ReceiveBeginPlay`
  (`ParticleSystemComponent.SetTemplate` (`self.ParticleSystem`) (`self.ParticleSys`))
  (`self.K2_SetActorRotation` (`KismetMathLibrary.Conv_VectorToRotator` (`self.ForwardVector`)))
  (`PrimitiveComponent.SetPhysicsLinearVelocity` (`self.Box`) (* (`self.ForwardVector`) (`self.Speed`)) false "None")
  (bind _returnvalue (`KismetSystemLibrary.K2_SetTimerDelegate` (delegate `Move`) 0.0167 true))
  (set `self.TimerHandle` _returnvalue))

(event `Move`
  (bind _output_get (set `self.Distance` (+ (* (`GameplayStatics.GetWorldDeltaSeconds`) (`self.Speed`)) (`self.Distance`))))
  (if (> _output_get (`self.MaxDistance`))
    (`self.DestorySelf`)))

(event `self.ReceiveHit`
  (params (MyComp :type "PrimitiveComponent Object Reference") (Other :type "Actor Object Reference") (OtherComp :type "PrimitiveComponent Object Reference") (bSelfMoved :type Boolean) (HitLocation :type "Vector Structure") (HitNormal :type "Vector Structure") (NormalImpulse :type "Vector Structure") (Hit :type "HitResult Structure (by ref)"))
  (bind _tags (`Actor.Tags` Other))
  (if (`KismetArrayLibrary.Array_IsValidIndex` _tags)
    (switch `name` (`|GetArrayItem` _tags)
      (:`Default`
        (`self.HitObstacle` :!label _label))
      (:`Enemy`
        (`self.HitEnemy` Other HitLocation)
        (`GameplayStatics.SpawnEmitterAtLocation` "/Game/BallisticsVFX/Particles/ImpactsVROptimal/DynamicImpacts/Lava/Lava_impact_Dyn.Lava_impact_Dyn" HitLocation (struct) (3.0 3.0 3.0) :!label _label_2)
        (`GameplayStatics.SpawnDecalAttached` "/Game/BallisticsVFX/Decals/Decals_Scorch.Decals_Scorch" (30.0 50.0 50.0) OtherComp "None" HitLocation (struct :`Yaw` 90.0) "KeepWorldPosition" 6.0)
        (`self.DestorySelf`))
      (:`Car`
        (`self.HitEnemyCar` Other HitLocation)
        (goto _label_2))
      (:`Obstacle`
        (goto _label)))
    (else
      (`self.HitObstacle`))))

(fn `HitEnemy`
  (params (Actor :type "Actor Object Reference") (HitLocation :type "Vector Structure"))
  (bind _asbp_car (cast `/Game/Asset/Blueprints/Car/BP_Car` Actor))
  (bind _asbp_enemy (cast `/Game/Asset/Blueprints/Enemy/BP_Enemy` (`/Game/Asset/Blueprints/Car/BP_Car.Driver` _asbp_car)))
  (bind (_damage_out _cri_) (`self.Damage Check` (`self.Damage`))
    (:`Out`
      (`/Game/Asset/Blueprints/Enemy/BP_Enemy.BeHit` _asbp_enemy _damage_out HitLocation _cri_ (`self.Break Shield Per`)))))

(fn `HitEnemyCar`
  (params (Car :type "Actor Object Reference") (HitLocation :type "Vector Structure"))
  (bind _asbp_car (cast `/Game/Asset/Blueprints/Car/BP_Car` Car))
  (`self.HitEnemy` (`self.GetAttachParentActor` _asbp_car) HitLocation))

(fn `HitObstacle`
  (`self.K2_DestroyActor`))

(fn `UserConstructionScript`)