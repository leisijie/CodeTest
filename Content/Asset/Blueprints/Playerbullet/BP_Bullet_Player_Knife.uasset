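; Player knife projectile that sticks into the enemy or car it hits, then explodes after a short delay.
; It launches its Box along ForwardVector at Speed, self-destroying after a timeout unless attached.
; Tag-based hits call HitEnemy, HitEnemyCar or HitObstacle; enemy and car hits attach the knife and trigger DelayExplode, which damages Sphere-overlapped BP_Enemy parent actors with boosted damage.
; A looping timer tracks distance, but exceeding MaxDistance does nothing.
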(event `self.ReceiveBeginPlay`
  (bind _particlesys (`self.ParticleSys`))
  (`|ExecutionSequence`
    (:`then_0`
      (`self.K2_SetActorRotation` (`KismetMathLibrary.Conv_VectorToRotator` (`self.ForwardVector`)))
      (`PrimitiveComponent.SetPhysicsLinearVelocity` (`self.Box`) (* (`self.ForwardVector`) (`self.Speed`)) false "None")
      (bind _returnvalue (`KismetSystemLibrary.K2_SetTimerDelegate` (delegate `CustomEvent`) 0.0167 true))
      (set `self.TimerHandle` _returnvalue)
      (`KismetSystemLibrary.Delay` 2.0)
      (if (not (`self.Attach?`))
        (`self.K2_DestroyActor`)))
    (:`then_1`
      (if (!= _particlesys null)
        (`ParticleSystemComponent.SetTemplate` (`self.ParticleSystem`) _particlesys)))))

(event `CustomEvent`
  (bind _output_get (set `self.Distance` (+ (* (`GameplayStatics.GetWorldDeltaSeconds`) (`self.Speed`)) (`self.Distance`))))
  (if (> _output_get (`self.MaxDistance`))
    _))

(event `self.ReceiveHit`
  (params (MyComp :type "PrimitiveComponent Object Reference") (Other :type "Actor Object Reference") (OtherComp :type "PrimitiveComponent Object Reference") (bSelfMoved :type Boolean) (HitLocation :type "Vector Structure") (HitNormal :type "Vector Structure") (NormalImpulse :type "Vector Structure") (Hit :type "HitResult Structure (by ref)"))
  (bind _tags (`Actor.Tags` Other))
  (if (`KismetArrayLibrary.Array_IsValidIndex` _tags)
    (switch `name` (`|GetArrayItem` _tags)
      (:`Default`
        (`self.HitObstacle` :!label _label))
      (:`Enemy`
        (`self.HitEnemy` Other HitLocation)
        (`GameplayStatics.SpawnEmitterAtLocation` "/Game/Asset/Particles/P_bullethit.P_bullethit" HitLocation (`KismetMathLibrary.RotatorFromAxisAndAngle` HitNormal) :!label _label_2)
        (`self.K2_AttachToComponent` self OtherComp "None" "KeepWorld" "KeepWorld" "KeepWorld" true)
        (set `self.Attach?` true)
        (`KismetSystemLibrary.Delay` 2.0)
        (`self.DelayExplode`))
      (:`Car`
        (`self.HitEnemyCar` Other HitLocation)
        (goto _label_2))
      (:`Obstacle`
        (goto _label)))
    (else
      (`self.HitObstacle`))))

(event `DelayExplode`
  (bind _sphere (`self.Sphere`))
  (bind _returnvalue (`SceneComponent.K2_GetComponentLocation` (`self.ParticleSystem`)))
  (bind (_outactors _returnvalue_2) (`KismetSystemLibrary.ComponentOverlapActors` _sphere (`SceneComponent.K2_GetComponentToWorld` _sphere) (`|MakeArray` "ObjectTypeQuery14" :!type "EObjectTypeQuery Enum")))
  (if _returnvalue_2
    (for _array_element _outactors
      (bind _asbp_enemy (cast `/Game/Asset/Blueprints/Enemy/BP_Enemy` (`self.GetParentActor` _array_element))
        (:`then`
          (`/Engine/EditorBlueprintResources/StandardMacros.IsValid` _asbp_enemy
            (:`Is Valid`
              (`/Game/Asset/Blueprints/Enemy/BP_Enemy.BeHit` _asbp_enemy (+ (`self.Damage`) 20) _returnvalue false 1.0)
              (`GameplayStatics.SpawnEmitterAtLocation` "/Game/Asset/Particles/P_bulletAfterBurst.P_bulletAfterBurst" _returnvalue (struct) (1.5 1.5 1.5)))
            (:`Is Not Valid`
              _)))
        (:`CastFailed`
          _))
      (`KismetSystemLibrary.Delay` 0.1 :!label _label_3)
      (`self.K2_DestroyActor`))
    (else
      (goto _label_3))))

(fn `UserConstructionScript`
  (`parent.UserConstructionScript`))