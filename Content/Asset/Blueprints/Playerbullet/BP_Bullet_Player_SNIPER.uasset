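; BP_Bullet_Player_SNIPER is the player's sniper projectile, which damages BP_Enemy targets.
; After a short delay it aligns to its forward vector, launches Box by physics velocity, sets its particle template and self-destructs shortly after.
; A looping timer polls Sphere overlaps and calls BeHit on overlapped actors' parent enemies with crit and shield-break data, spawning impact effects without destroying the bullet.
; A second timer accumulates travel distance, but exceeding MaxDistance does nothing.
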(event `self.ReceiveBeginPlay`
  (bind _particlesys (`self.ParticleSys`))
  (`KismetSystemLibrary.Delay` 0.18)
  (`|ExecutionSequence`
    (:`then_0`
      (`self.K2_SetActorRotation` (`KismetMathLibrary.Conv_VectorToRotator` (`self.ForwardVector`)))
      (`PrimitiveComponent.SetPhysicsLinearVelocity` (`self.Box`) (* (`self.ForwardVector`) (`self.Speed`)) false "None")
      (bind _returnvalue (`KismetSystemLibrary.K2_SetTimerDelegate` (delegate `CustomEvent`) 0.0167 true))
      (set `self.TimerHandle` _returnvalue)
      (`KismetSystemLibrary.Delay` 1.0)
      (`self.K2_DestroyActor`))
    (:`then_1`
      (if (!= _particlesys null)
        (`ParticleSystemComponent.SetTemplate` (`self.ParticleSystem`) _particlesys)))
    (:`then_2`
      (`KismetSystemLibrary.K2_SetTimer` null "HIT_Enemy" 0.02 true))))

(event `CustomEvent`
  (bind _output_get (set `self.Distance` (+ (* (`GameplayStatics.GetWorldDeltaSeconds`) (`self.Speed`)) (`self.Distance`))))
  (if (> _output_get (`self.MaxDistance`))
    _))

(fn `HIT_Enemy`
  (bind _sphere (`self.Sphere`))
  (bind _returnvalue (`SceneComponent.K2_GetComponentLocation` (`self.ParticleSystem`)))
  (bind (_outactors _returnvalue_2) (`KismetSystemLibrary.ComponentOverlapActors` _sphere (`SceneComponent.K2_GetComponentToWorld` _sphere) (`|MakeArray` "ObjectTypeQuery14" :!type "EObjectTypeQuery Enum")))
  (if _returnvalue_2
    (for _array_element _outactors
      (bind _asbp_enemy (cast `/Game/Asset/Blueprints/Enemy/BP_Enemy` (`self.GetParentActor` _array_element)))
      (`/Engine/EditorBlueprintResources/StandardMacros.IsValid` _asbp_enemy
        (:`Is Valid`
          (`/Game/Asset/Blueprints/Enemy/BP_Enemy.BeHit` _asbp_enemy (`self.Damage`) _returnvalue (`self.Cri?`) (`self.Break Shield Per`))
          (`GameplayStatics.SpawnEmitterAtLocation` "/Game/Asset/Particles/P_bullethit.P_bullethit" _returnvalue (struct) (2.0 2.0 2.0)))))))

(fn `UserConstructionScript`
  (`parent.UserConstructionScript`))