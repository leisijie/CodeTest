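; BP_Crash_Player is a player attack actor that deals a one-shot area hit to enemies, then destroys itself.
; On BeginPlay it queries actors overlapping its Cube component and casts each one's parent actor to BP_Enemy, so it expects child-actor hit targets.
; Each enemy receives BeHit with damage, crit and shield-break values, plus a large shield impact effect at the particle component's location.
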(event `self.ReceiveBeginPlay`
  (bind _cube (`self.Cube`))
  (bind _returnvalue (`SceneComponent.K2_GetComponentLocation` (`self.ParticleSystem`)))
  (`parent.ReceiveBeginPlay`)
  (bind _outactors (`KismetSystemLibrary.ComponentOverlapActors` _cube (`SceneComponent.K2_GetComponentToWorld` _cube) (`|MakeArray` "ObjectTypeQuery14" :!type "EObjectTypeQuery Enum")))
  (if true
    (for _array_element _outactors
      (bind _asbp_enemy (cast `/Game/Asset/Blueprints/Enemy/BP_Enemy` (`self.GetParentActor` _array_element)))
      (`/Game/Asset/Blueprints/Enemy/BP_Enemy.BeHit` _asbp_enemy (`self.Damage`) _returnvalue (`self.Cri?`) (`self.Break Shield Per`))
      (`GameplayStatics.SpawnEmitterAtLocation` "/Game/BallisticsVFX/Particles/Impacts/LegacyFX/Small-Medium-Large/EnergyShield/EnergyShield_impact_Large.EnergyShield_impact_Large" _returnvalue (struct) (2.0 2.0 2.0))))
  (`self.K2_DestroyActor`))

(fn `UserConstructionScript`
  (`parent.UserConstructionScript`))