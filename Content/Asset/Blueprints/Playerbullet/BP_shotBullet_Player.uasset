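; BP_shotBullet_Player is a short-lived player shot that damages enemies inside a growing or shrinking area, destroying itself after half a second.
; A timeline scales the mesh in X and Y, running a component overlap check on every update.
; Line traces toward each enemy supply hit locations for BeHit, alongside crit-rolled damage and shield-break value.
; The handled-enemy ignore list clears after each overlap pass, so hits can repeat across updates.
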(event `self.ReceiveBeginPlay`
  (bind _damage (`self.Damage`))
  (bind _staticmesh (`self.StaticMesh`))
  (`parent.ReceiveBeginPlay`)
  (`|ExecutionSequence`
    (:`then_0`
      (`KismetSystemLibrary.Delay` 0.5)
      (`self.K2_DestroyActor`))
    (:`then_1`
      (bind (_direction _newtrack_0) (`Timeline|Timeline_0`)
        (:`Update`
          (`SceneComponent.SetWorldScale3D` (`self.StaticMesh`) (`KismetMathLibrary.MakeVector` (* (.x (`self.scale`)) _newtrack_0) (* (.y (`self.scale`)) _newtrack_0) (.z (`self.scale`))))
          (bind (_outactors _returnvalue) (`KismetSystemLibrary.ComponentOverlapActors` _staticmesh (`SceneComponent.K2_GetComponentToWorld` _staticmesh) (`|MakeArray` "ObjectTypeQuery14" :!type "EObjectTypeQuery Enum")))
          (if _returnvalue
            (for _array_element _outactors
              (bind _asbp_enemy (cast `/Game/Asset/Blueprints/Enemy/BP_Enemy` (`self.GetParentActor` _array_element)))
              (bind _outhit (`KismetSystemLibrary.LineTraceSingleForObjects` (`SceneComponent.K2_GetComponentLocation` (`self.Box`)) (`SceneComponent.K2_GetComponentLocation` (`/Game/Asset/Blueprints/Enemy/BP_Enemy.CarActor` _asbp_enemy)) (`|MakeArray` "ObjectTypeQuery14" :!type "EObjectTypeQuery Enum") false (`self.RemoveEnemy`)))
              (`KismetArrayLibrary.Array_Add` (`self.RemoveEnemy`) _asbp_enemy)
              (if (`KismetMathLibrary.RandomBoolWithWeight` (`self.Credit Hit Per`))
                (set `self.Store Damage` (`KismetMathLibrary.FTrunc` (* _damage (`self.Credit Boost Per`))))
                (set `self.Cri?` true)
                (else
                  (set `self.Store Damage` _damage)
                  (set `self.Cri?` false)))
              (`/Game/Asset/Blueprints/Enemy/BP_Enemy.BeHit` _asbp_enemy (`self.Store Damage`) (`.Location` (`GameplayStatics.BreakHitResult` _outhit)) (`self.Cri?`) (`self.Break Shield Per`)))
            (`KismetArrayLibrary.Array_Clear` (`self.RemoveEnemy`))))))))

(fn `UserConstructionScript`
  (`parent.UserConstructionScript`))