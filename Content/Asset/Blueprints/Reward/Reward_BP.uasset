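; Reward actor that builds a row of shield pack cubes and removes itself after a short idle period.
; Each Active call, including one on BeginPlay, counts a pack, plays a timeline nudging the child actor along Y, then spawns a cube at the root attached to it.
; Active also resets a looping Delay clock; once Tick sees it pass its limit, the cubes and actor are destroyed.
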(event `self.ReceiveBeginPlay`
  (`|ExecutionSequence`
    (:`then_0`
      ;[1 1 1] Clock
      (set `self.TickTock` 0)
      (bind _output_get (set `self.TickTock` (+ (`self.TickTock`) 1) :!label _label))
      (`KismetSystemLibrary.Delay` 0.1)
      (goto _label))
    (:`then_1`
      (`self.Active`))))

(event `Reset`
  ;[1 1 1] Reset
  (set `self.TickTock` 0))

(event `Active`
  ;[1 1 1] Active
  (bind _output_get (set `self.ShieldPack_Number` (+ (`self.ShieldPack_Number`) 1)))
  (`self.ADD ONE SHIELD`)
  (`self.Reset`))

(event `self.ReceiveTick`
  (params (DeltaSeconds :type "Float (single-precision)"))
  ;[1 1 1] Detect
  (if (> (`self.ShieldPack_Number`) 0)
    (if (not (<= (`self.TickTock`) 6))
      (`/Engine/EditorBlueprintResources/StandardMacros.DoOnce` false
        (:`Completed`
          (`self.BYEBYE`))))))

(event `ADD ONE SHIELD`
  (bind _returnvalue (`SceneComponent.K2_GetComponentLocation` (`self.ChildActor`)))
  ;[1 1 1] Leader, Move!
  (bind (_direction _move) (`Timeline|Timeline_1`)
    (:`Update`
      (`SceneComponent.K2_SetWorldLocation` (`self.ChildActor`) (`KismetMathLibrary.VInterpTo` _returnvalue (`KismetMathLibrary.MakeVector` (.x _returnvalue) (+ (.y _returnvalue) 50.0) (.z _returnvalue)) _move _move) false false))
    (:`Finished`
      ;[1 1 1] Spawn
      (bind _returnvalue_2 (`|SpawnActorFromClass` "/Game/Asset/Blueprints/Reward/Reward_Cube_BP.Reward_Cube_BP_C" (`KismetMathLibrary.Conv_VectorToTransform` (`SceneComponent.K2_GetComponentLocation` (`self.DefaultSceneRoot`))) "Undefined" "OverrideRootScale" null null))
      (`KismetArrayLibrary.Array_Add` (`self.Reward`) _returnvalue_2)
      (`SceneComponent.K2_AttachToComponent` (`Actor.RootComponent` _returnvalue_2) (`self.ChildActor`) "None" "KeepWorld" "KeepWorld" "KeepWorld" true))))

(event `BYEBYE`
  ;[1 1 1] Byebye
  (for _array_element (`self.Reward`)
    (`/Engine/EditorBlueprintResources/StandardMacros.IsValid` _array_element
      (:`Is Valid`
        (`self.K2_DestroyActor` _array_element)
        (`self.K2_DestroyActor`)))))

(fn `UserConstructionScript`)