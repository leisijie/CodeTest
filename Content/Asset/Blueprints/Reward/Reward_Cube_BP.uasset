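; Reward cube Blueprint whose MoveBack event slides its root along world +Y.
; Each timeline update uses VInterpTo toward a point slightly ahead of the current location, with one track feeding both delta time and interp speed.
; An unconnected debug line trace along local Y and a DoOnce that would call MoveBack never run, so nothing here triggers the movement.
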(event `self.ReceiveTick`
  (params (DeltaSeconds :type "Float (single-precision)")))

(event `Move Back`
  (bind _returnvalue (`SceneComponent.K2_GetComponentLocation` (`self.DefaultSceneRoot`)))
  (bind (_direction _newtrack_0) (`Timeline|Timeline_0`)
    (:`Update`
      (`SceneComponent.K2_SetWorldLocation` (`self.DefaultSceneRoot`) (`KismetMathLibrary.VInterpTo` _returnvalue (`KismetMathLibrary.MakeVector` (.x _returnvalue) (+ (.y _returnvalue) 50.0) (.z _returnvalue)) _newtrack_0 _newtrack_0) false false))))

(fn `UserConstructionScript`)