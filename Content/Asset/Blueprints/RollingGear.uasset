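; RollingGear is an actor Blueprint that continuously spins a gear static mesh.
; BeginPlay starts a looping timer that calls Rolling roughly 60 times a second, in place of Tick.
; Rolling adds a local yaw rotation of Speed per call, with a branch choosing negative or positive direction, so Speed is per step rather than per second.
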(event `self.ReceiveBeginPlay`
  (`KismetSystemLibrary.K2_SetTimer` null "Rolling" 0.017 true))

(fn `Rolling`
  (bind _staticmesh (`self.StaticMesh`))
  (if (`self.+_`)
    (`SceneComponent.K2_AddLocalRotation` _staticmesh (`KismetMathLibrary.MakeRotator` 0.0 0.0 (* (`self.Speed`) -1.0)) false false)
    (else
      (`SceneComponent.K2_AddLocalRotation` _staticmesh (`KismetMathLibrary.MakeRotator` 0.0 0.0 (* (`self.Speed`) 1.0)) false false))))

(fn `UserConstructionScript`)