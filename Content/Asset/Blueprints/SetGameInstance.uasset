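; Trigger actor that records named progress or a reward in the game instance when its Cube is overlapped, then reloads the current level.
; The Event flag selects between calling NewProgress and JustReward on bp_Gameinstance with ProgressName.
; Both branches share a short delay before reopening the level by name.
; The construction script shows ProgressName on the TextRender as a label.
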(event `self.Cube.OnComponentBeginOverlap`
  (params (OverlappedComponent :type "PrimitiveComponent Object Reference") (OtherActor :type "Actor Object Reference") (OtherComp :type "PrimitiveComponent Object Reference") (OtherBodyIndex :type Integer) (bFromSweep :type Boolean) (SweepResult :type "HitResult Structure (by ref)"))
  (if (`self.Event?`)
    (bind _asbp_gameinstance (cast `/Game/Asset/Blueprints/bp_Gameinstance` (`GameplayStatics.GetGameInstance`)))
    (`/Game/Asset/Blueprints/bp_Gameinstance.NewProgress` _asbp_gameinstance (`self.ProgressName`))
    (else
      (bind _asbp_gameinstance_2 (cast `/Game/Asset/Blueprints/bp_Gameinstance` (`GameplayStatics.GetGameInstance`)))
      (`/Game/Asset/Blueprints/bp_Gameinstance.JustReward` _asbp_gameinstance_2 (`self.ProgressName`))))
  (`KismetSystemLibrary.Delay` 0.5)
  (bind _returnvalue (`GameplayStatics.GetCurrentLevelName` true))
  (`GameplayStatics.OpenLevel` (`KismetStringLibrary.Conv_StringToName` _returnvalue)))

(fn `UserConstructionScript`
  (`TextRenderComponent.K2_SetText` (`self.TextRender`) (`KismetTextLibrary.Conv_NameToText` (`self.ProgressName`))))