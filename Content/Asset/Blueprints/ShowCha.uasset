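; Display character actor that previews the weapons chosen in the left and right input boxes of its referenced widget.
; Its custom event Aniiiiii plays a one-shot gun-drawing animation, then looks up each slot's name in WeaponTable to set the Gun2 (left box) and Gun1 (right box) skeletal meshes.
; An empty slot clears that gun's mesh, and nothing runs on BeginPlay or Tick.
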(event `/Game/Asset/Animation/cha/ani.aniiiiii`
  (params (NewParam :type Boolean))
  (bind _wight (`self.wight`))
  (bind _gun2 (`self.gun2`))
  (bind _gun1 (`self.gun1`))
  (bind _name (`/Game/Asset/Widget/SwitchWidget/Inputbox.name` (`/Game/Asset/Widget/SwitchWidget/WeaponSelect_main.Inputbox_R` _wight)))
  (bind _name_2 (`/Game/Asset/Widget/SwitchWidget/Inputbox.name` (`/Game/Asset/Widget/SwitchWidget/WeaponSelect_main.Inputbox_L` _wight)))
  (`SkeletalMeshComponent.PlayAnimation` (`self.SkeletalMesh`) "/Game/Asset/Animation/cha/ani/Drawing_Gun.Drawing_Gun" false)
  (`|ExecutionSequence`
    (:`then_0`
      (if (== _name_2 "None")
        (`SkinnedMeshComponent.SetSkinnedAssetAndUpdate` _gun2 null false)
        (else
          (bind _returnvalue (`|GetDataTableRow` "/Game/Asset/Blueprints/DataTable/WeaponTable.WeaponTable" _name_2)
            (:`then`
              (`SkinnedMeshComponent.SetSkinnedAssetAndUpdate` _gun2 (`.mesh_22_936B7FBF41D2504430B5EBA05C8D0698` (break `/Game/Asset/Blueprints/Struct/WeaponIconAndClass` _returnvalue)) false))))))
    (:`then_1`
      (if (== _name "None")
        (`SkinnedMeshComponent.SetSkinnedAssetAndUpdate` _gun1 null false)
        (else
          (bind _returnvalue_2 (`|GetDataTableRow` "/Game/Asset/Blueprints/DataTable/WeaponTable.WeaponTable" _name)
            (:`then`
              (`SkinnedMeshComponent.SetSkinnedAssetAndUpdate` _gun1 (`.mesh_22_936B7FBF41D2504430B5EBA05C8D0698` (break `/Game/Asset/Blueprints/Struct/WeaponIconAndClass` _returnvalue_2)) false))))))))

(event `self.ReceiveBeginPlay`)

(fn `UserConstructionScript`)