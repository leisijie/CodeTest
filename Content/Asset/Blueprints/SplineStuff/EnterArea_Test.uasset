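; Test actor that builds spline mesh segments along its Spline one at a time after BeginPlay.
; A custom Loop & Delay macro steps through the point indices, pausing briefly between segments.
; Each step adds a spline mesh component to Splinestuff and shapes it from the previous and current points' world-space locations and tangents.
; The Construction Script is empty, with an instant for-loop version left disconnected.
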(event `self.ReceiveBeginPlay`
  (bind _spline (`self.Spline`))
  (bind _index (`self.Loop & Delay` 0 (- (`SplineComponent.GetNumberOfSplinePoints` (`self.Spline`)) 1) :!label _label)
    (:`Loop Body`
      (bind _returnvalue (`AddComponent|NODE_AddSplineMeshComponent-7` :`bManualAttachment` true))
      (`KismetArrayLibrary.Array_Add` (`self.Splinestuff`) _returnvalue)
      (`SceneComponent.K2_AttachToComponent` (`self.DefaultSceneRoot`) null "None" "KeepRelative" "KeepRelative" "KeepRelative" true)
      (bind (_location _tangent) (`SplineComponent.GetLocationAndTangentAtSplinePoint` _spline (- _index 1) "World"))
      (bind (_location_2 _tangent_2) (`SplineComponent.GetLocationAndTangentAtSplinePoint` _spline _index "World"))
      (`SplineMeshComponent.SetStartAndEnd` _returnvalue _location _tangent _location_2 _tangent_2 true)
      (`KismetSystemLibrary.Delay` 0.2)
      (goto _label :!via `Next Step`))))

(fn `UserConstructionScript`)