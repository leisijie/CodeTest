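; Spline path actor that, once its PreviousONE predecessor is gone and a delay passes, spawns an ActorWantToEnter and moves it along the spline.
; It builds spline meshes segment by segment with a March_End marker at the end, then removes them progressively, timed by the move rate.
; A MOVE timeline drives location and rotation, optionally registering the actor with LevelCounter.
; The path self-destructs on arrival, also destroying the actor when SHOW is set.
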(event `EnterArea`
  (bind _spline_0 (`self.Spline_0`))
  (bind _spline_space (`self.Spline space`))
  (bind _spline_0_2 (`self.Spline_0`))
  (bind _returnvalue (`SplineComponent.GetSplineLength` _spline_0))
  ;[1 1 1] Enter Area
  (bind _output_get (set `self.Spline Mesh Amount` (- (`KismetMathLibrary.FTrunc` (/ _returnvalue (`self.Spline space`))) 1)))
  (bind _index (`self.Delay With Loop Break` 0 _output_get :!label _label)
    (:`Loop Body`
      (bind _returnvalue_2 (`AddComponent|NODE_AddSplineMeshComponent-7` :`bManualAttachment` true))
      (`KismetArrayLibrary.Array_Add` (`self.Spline_Stuff`) _returnvalue_2)
      (`SceneComponent.K2_AttachToComponent` (`self.Spline_0`) null "None" "KeepWorld" "KeepWorld" "KeepWorld" true)
      (bind _returnvalue_3 (* _index _spline_space))
      (bind _returnvalue_4 (* (+ _index 1) _spline_space))
      (`SplineMeshComponent.SetStartAndEnd` _returnvalue_2 (`SplineComponent.GetLocationAtDistanceAlongSpline` _spline_0_2 _returnvalue_3 "World") (`SplineComponent.GetTangentAtDistanceAlongSpline` _spline_0_2 _returnvalue_3 "World") (`SplineComponent.GetLocationAtDistanceAlongSpline` _spline_0_2 _returnvalue_4 "World") (`SplineComponent.GetTangentAtDistanceAlongSpline` _spline_0_2 _returnvalue_4 "World") true)
      (`KismetSystemLibrary.Delay` 0.05)
      (goto _label :!via `Next Step`))
    (:`Complete`
      (bind _returnvalue_5 (`|SpawnActorFromClass` "/Game/Asset/Blueprints/SplineStuff/March_End.March_End_C" (`KismetMathLibrary.Conv_VectorToTransform` (`SplineComponent.GetLocationAtDistanceAlongSpline` _spline_0 _returnvalue "World")) "Undefined" "OverrideRootScale" null null))
      (set `self.Target` _returnvalue_5))))

(event `Destroy Spline`
  (bind _target (`self.Target`))
  ;[1 1 1] ByeSpline
  (set `self.SplinDestroyWaitTime` (/ (/ 10.0 (`self.New Rate`)) (+ (`KismetMathLibrary.Conv_IntToDouble` (`self.Spline Mesh Amount`)) 1.0)))
  (bind _index (`self.Delay With Loop Break` 0 (`self.Spline Mesh Amount`) :!label _label_2)
    (:`Loop Body`
      (bind _output (`|GetArrayItem` (`self.Spline_Stuff`) _index))
      (`/Engine/EditorBlueprintResources/StandardMacros.IsValid` _output
        (:`Is Valid`
          (`ActorComponent.K2_DestroyComponent` _output)
          (`KismetSystemLibrary.Delay` (`self.SplinDestroyWaitTime`))
          (goto _label_2 :!via `Next Step`))))
    (:`Complete`
      (`/Engine/EditorBlueprintResources/StandardMacros.IsValid` _target
        (:`Is Valid`
          (`self.K2_DestroyActor` _target))))))

(event `GOGOGO`
  (bind _level_counter (`self.Level_Counter`))
  (bind _move_budy (`self.Move_budy`))
  (bind _spline_0 (`self.Spline_0`))
  ;[1 1 1] Set actor
  (bind _returnvalue (`|SpawnActorFromClass` (`self.Actor_Want_To_Enter`) (`KismetMathLibrary.Conv_VectorToTransform` (`SceneComponent.K2_GetComponentLocation` (`self.Spline_0`))) "AlwaysSpawn" "OverrideRootScale" null (`self.Level_Counter`) null))
  (bind _output_get (set `self.Move_budy` _returnvalue))
  (if (`self.SHOW?`)
    ;[1 1 1] Move to the grave
    (bind (_direction _move) (`Timeline|MOVE` :!label _label_3)
      (:`Update`
        (`/Engine/EditorBlueprintResources/StandardMacros.IsValid` _move_budy
          (:`Is Valid`
            (bind _asbp_enemy (cast `/Game/Asset/Blueprints/Character/BP_Enemy` _move_budy)
              (:`then`
                (bind _returnvalue_2 (* _move (`SplineComponent.GetSplineLength` (`self.Spline_0`))))
                (bind _returnvalue_3 (`SplineComponent.GetLocationAtDistanceAlongSpline` _spline_0 _returnvalue_2 "World"))
                (bind (_sweephitresult _returnvalue_4) (`self.K2_SetActorLocation` (`self.GetAttachParentActor` _asbp_enemy) _returnvalue_3 true false))
                (`KismetSystemLibrary.PrintString` (`KismetStringLibrary.Conv_BoolToString` _returnvalue_4))
                (if (not (`self.Land?`))
                  (bind _returnvalue_5 (`KismetMathLibrary.MakeRotator` (.roll (`SplineComponent.GetRotationAtDistanceAlongSpline` _spline_0 _returnvalue_2 "World")) (.pitch (`SplineComponent.GetRotationAtDistanceAlongSpline` _spline_0 _returnvalue_2 "World")) (+ (.yaw (`SplineComponent.GetRotationAtDistanceAlongSpline` _spline_0 _returnvalue_2 "World")) (`self.Turn`))))
                  (`self.K2_SetActorRotation` _returnvalue_5))
                (`TimelineComponent.SetPlayRate` (`self.MOVE`) (`self.New Rate`)))
              (:`CastFailed`
                (`self.K2_SetActorLocation` _asbp_enemy _returnvalue_3 true false)
                (if (not (`self.Land?`))
                  (`self.K2_SetActorRotation` _returnvalue_5))
                (`TimelineComponent.SetPlayRate` (`self.MOVE`) (`self.New Rate`))))))))
    (else
      (`/Engine/EditorBlueprintResources/StandardMacros.IsValid` _level_counter
        (:`Is Valid`
          (`/Game/Asset/Blueprints/Level_Counter.Wave Control` _level_counter _output_get)
          (goto _label_3 :!via `PlayFromStart`))
        (:`Is Not Valid`
          (goto _label_3))))))

(event `self.ReceiveTick`
  (params (DeltaSeconds :type "Float (single-precision)"))
  (bind _spline_0 (`self.Spline_0`))
  (`|ExecutionSequence`
    (:`then_0`
      (`/Engine/EditorBlueprintResources/StandardMacros.IsValid` (`self.PreviousONE`)
        (:`Is Not Valid`
          (`/Engine/EditorBlueprintResources/StandardMacros.DoOnce` false
            (:`Completed`
              (`KismetSystemLibrary.Delay` (`self.Delay`))
              (set `self.On my way` true)
              (`|ExecutionSequence`
                (:`then_0`
                  (`self.GOGOGO`))
                (:`then_1`
                  (`self.EnterArea`))
                (:`then_2`
                  (`self.Destroy Spline`))))))))
    (:`then_1`
      (if (`self.On my way`)
        (`/Engine/EditorBlueprintResources/StandardMacros.IsValid` (`self.Move_budy`)
          (:`Is Valid`
            ;[1 1 1] END?
            (if (`KismetMathLibrary.EqualExactly_VectorVector` (`self.K2_GetActorLocation` (`self.Move_budy`)) (`SplineComponent.GetLocationAtDistanceAlongSpline` _spline_0 (`SplineComponent.GetSplineLength` _spline_0) "World"))
              (if (`self.SHOW?`)
                (`self.K2_DestroyActor` (`self.Move_budy`)))
              (`self.K2_DestroyActor` :!label _label_4)))
          (:`Is Not Valid`
            (goto _label_4)))))))

(fn `UserConstructionScript`)