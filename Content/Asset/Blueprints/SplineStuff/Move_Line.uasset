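; Spline mover actor that spawns an actor of a configurable class and moves it along its spline.
; On BeginPlay it spawns and stores the actor, then plays the MOVE timeline.
; Each update maps the timeline value to a distance along the spline and sets the actor's world location and rotation, adding a yaw offset from Turn.
; The timeline's play rate is reapplied from NewRate every update.
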(event `self.ReceiveBeginPlay`
  (bind _spline_0 (`self.Spline_0`))
  (bind _rootcomponent (`Actor.RootComponent` (`self.Move_budy`)))
  (bind _returnvalue (`|SpawnActorFromClass` (`self.Actor Want To Move`) (`SceneComponent.K2_GetComponentToWorld` (`self.Spline_0`)) "Undefined" "OverrideRootScale" null null))
  (set `self.Move_budy` _returnvalue)
  (bind (_direction _move) (`Timeline|MOVE` :`NewTime` 10.0)
    (:`Update`
      (bind _returnvalue_2 (* _move (`SplineComponent.GetSplineLength` (`self.Spline_0`))))
      (`SceneComponent.K2_SetWorldLocation` _rootcomponent (`SplineComponent.GetLocationAtDistanceAlongSpline` _spline_0 _returnvalue_2 "World") false false)
      (`SceneComponent.K2_SetWorldRotation` _rootcomponent (`KismetMathLibrary.MakeRotator` (.roll (`SplineComponent.GetRotationAtDistanceAlongSpline` _spline_0 _returnvalue_2 "World")) (.pitch (`SplineComponent.GetRotationAtDistanceAlongSpline` _spline_0 _returnvalue_2 "World")) (+ (.yaw (`SplineComponent.GetRotationAtDistanceAlongSpline` _spline_0 _returnvalue_2 "World")) (`self.Turn`))) false false)
      (`TimelineComponent.SetPlayRate` (`self.MOVE`) (`self.New Rate`)))))

(fn `UserConstructionScript`)