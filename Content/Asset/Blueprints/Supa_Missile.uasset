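; Missile actor that flies its mesh along a spline and explodes at the far end.
; On BeginPlay the MOVE timeline drives the mesh by spline distance while the path is drawn as spline mesh segments, added one at a time through a delayed loop macro.
; Once the path completes, a March_End actor spawns at the endpoint as Target.
; When the timeline finishes, it spawns an explosion and destroys both Target and itself.
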(event `EnterArea`
  (bind _spline_0 (`self.Spline_0`))
  (bind _spline_space (`self.Spline space`))
  (bind _spline_0_2 (`self.Spline_0`))
  (bind _returnvalue (`SplineComponent.GetSplineLength` _spline_0))
  ;[1 1 1] Enter Area
  (bind _output_get (set `self.Spline Mesh Amount` (- (`KismetMathLibrary.FTrunc` (/ _returnvalue (`self.Spline space`))) 1)))
  (bind _index (`self.Delay With Loop Break` 0 _output_get :!label _label)
    (:`Loop Body`
      (bind _returnvalue_2 (`AddComponent|NODE_AddSplineMeshComponent-7` :`bManualAttachment` true))
      (`KismetArrayLibrary.Array_Add` (`self.Spline_Stuff`) _returnvalue_2)
      (`SceneComponent.K2_AttachToComponent` (`self.Spline_0`) null "None" "KeepWorld" "KeepWorld" "KeepWorld" true)
      (bind _returnvalue_3 (* _index _spline_space))
      (bind _returnvalue_4 (* (+ _index 1) _spline_space))
      (`SplineMeshComponent.SetStartAndEnd` _returnvalue_2 (`SplineComponent.GetLocationAtDistanceAlongSpline` _spline_0_2 _returnvalue_3 "World") (`SplineComponent.GetTangentAtDistanceAlongSpline` _spline_0_2 _returnvalue_3 "World") (`SplineComponent.GetLocationAtDistanceAlongSpline` _spline_0_2 _returnvalue_4 "World") (`SplineComponent.GetTangentAtDistanceAlongSpline` _spline_0_2 _returnvalue_4 "World") true)
      (`KismetSystemLibrary.Delay` 0.05)
      (goto _label :!via `Next Step`))
    (:`Complete`
      (bind _returnvalue_5 (`|SpawnActorFromClass` "/Game/Asset/Blueprints/SplineStuff/March_End.March_End_C" (`KismetMathLibrary.Conv_VectorToTransform` (`SplineComponent.GetLocationAtDistanceAlongSpline` _spline_0 _returnvalue "World")) "Undefined" "OverrideRootScale" null null))
      (set `self.Target` _returnvalue_5))))

(event `self.ReceiveBeginPlay`
  (`|ExecutionSequence`
    (:`then_0`
      (`self.GOGOGO`))
    (:`then_1`
      (`self.EnterArea`))))

(event `GOGOGO`
  (bind _spline_0 (`self.Spline_0`))
  (bind (_direction _move) (`Timeline|MOVE`)
    (:`Update`
      (`SceneComponent.K2_SetWorldLocation` (`self.StaticMesh`) (`SplineComponent.GetLocationAtDistanceAlongSpline` (`self.Spline_0`) (* _move (`SplineComponent.GetSplineLength` (`self.Spline_0`))) "World") false false)
      (`TimelineComponent.SetPlayRate` (`self.MOVE`) (`self.New Rate`)))
    (:`Finished`
      (`GameplayStatics.SpawnEmitterAtLocation` "/Game/BallisticsVFX/Particles/Explosive/Explosion_Frag_small.Explosion_Frag_small" (.location (`KismetMathLibrary.Conv_VectorToTransform` (`SplineComponent.GetLocationAtDistanceAlongSpline` _spline_0 (`SplineComponent.GetSplineLength` _spline_0) "World"))) (struct) (5.0 5.0 5.0))
      (`self.K2_DestroyActor` (`self.Target`))
      (`self.K2_DestroyActor`))))

(fn `UserConstructionScript`)