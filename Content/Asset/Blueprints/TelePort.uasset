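; Two-way teleporter actor that moves the ThirdPersonCharacter between a start point and a target point.
; Overlapping Box sends the player to TargetLo and overlapping Box1 sends them back to StartLo, copying that point's location and rotation.
; Each trip shows a BlackOut widget via Shutdown and waits its AniTime before moving the character.
; Two flags block the opposite box during a trip so arrival does not immediately trigger a return.
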(event `self.Box.OnComponentBeginOverlap`
  (params (OverlappedComponent :type "PrimitiveComponent Object Reference") (OtherActor :type "Actor Object Reference") (OtherComp :type "PrimitiveComponent Object Reference") (OtherBodyIndex :type Integer) (bFromSweep :type Boolean) (SweepResult :type "HitResult Structure (by ref)"))
  (bind _player (`self.player`))
  (bind _targetlo (`self.TargetLo`))
  ;[1 1 1] TotTarget
  (if (not (`self.GetBack Active`))
    (bind _asthird_person_character (cast `/Game/DynamicLocomotion/Blueprints/ThirdPersonCharacter` OtherActor))
    (set `self.player` _asthird_person_character)
    (set `self.ToTarget Actice` true)
    (bind _returnvalue (`|CreateWidget` "/Game/Asset/Widget/BlackOut.BlackOut_C" (`GameplayStatics.GetPlayerController` 0)))
    (`UserWidget.AddToViewport` _returnvalue 0)
    (`/Game/Asset/Widget/BlackOut.Shutdown` _returnvalue (`self.blackTime`) (`self.player`))
    (`KismetSystemLibrary.Delay` (`/Game/Asset/Widget/BlackOut.AniTime` _returnvalue))
    (`self.K2_SetActorRelativeLocation` _player (`SceneComponent.K2_GetComponentLocation` _targetlo) false false)
    (`self.K2_SetActorRelativeRotation` _player (`SceneComponent.K2_GetComponentRotation` _targetlo) false false)
    (set `self.ToTarget Actice` false)))

(event `self.Box.OnComponentEndOverlap`
  (params (OverlappedComponent :type "PrimitiveComponent Object Reference") (OtherActor :type "Actor Object Reference") (OtherComp :type "PrimitiveComponent Object Reference") (OtherBodyIndex :type Integer))
  ;[1 1 1] TotTarget
)

(event `self.Box1.OnComponentBeginOverlap`
  (params (OverlappedComponent :type "PrimitiveComponent Object Reference") (OtherActor :type "Actor Object Reference") (OtherComp :type "PrimitiveComponent Object Reference") (OtherBodyIndex :type Integer) (bFromSweep :type Boolean) (SweepResult :type "HitResult Structure (by ref)"))
  (bind _player (`self.player`))
  (bind _startlo (`self.StartLo`))
  (if (not (`self.ToTarget Actice`))
    (bind _asthird_person_character (cast `/Game/DynamicLocomotion/Blueprints/ThirdPersonCharacter` OtherActor))
    (set `self.player` _asthird_person_character)
    (set `self.GetBack Active` true)
    (bind _returnvalue (`|CreateWidget` "/Game/Asset/Widget/BlackOut.BlackOut_C" (`GameplayStatics.GetPlayerController` 0)))
    (`UserWidget.AddToViewport` _returnvalue 0)
    (`/Game/Asset/Widget/BlackOut.Shutdown` _returnvalue (`self.blackTime`) (`self.player`))
    (`KismetSystemLibrary.Delay` (`/Game/Asset/Widget/BlackOut.AniTime` _returnvalue))
    (`self.K2_SetActorRelativeLocation` _player (`SceneComponent.K2_GetComponentLocation` _startlo) false false)
    (`self.K2_SetActorRelativeRotation` _player (`SceneComponent.K2_GetComponentRotation` _startlo) false false)
    (set `self.GetBack Active` false)))

(event `self.Box1.OnComponentEndOverlap`
  (params (OverlappedComponent :type "PrimitiveComponent Object Reference") (OtherActor :type "Actor Object Reference") (OtherComp :type "PrimitiveComponent Object Reference") (OtherBodyIndex :type Integer)))

(fn `UserConstructionScript`)