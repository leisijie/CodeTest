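; Vacuum is an actor that bursts into reward particles and gets pulled into the player before destroying itself.
; After a short delay on BeginPlay, it attaches emitters at random numbered mesh sockets and plays an explode-shrink animation.
; A timeline repeatedly blends its current location toward the player's live position, then destroys it on finish.
; As the pull starts, it also spawns a Vacuum actor at its transform.
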(event `self.ReceiveBeginPlay`
  (bind _skeletalmesh (`self.SkeletalMesh`))
  (bind _returnvalue (`KismetStringLibrary.Conv_StringToName` (`KismetStringLibrary.Conv_IntToString` (`KismetMathLibrary.RandomInteger` 17))))
  (bind _asbp_player_character (cast `/Game/Asset/Blueprints/Character/BP_PlayerCharacter` (`GameplayStatics.GetPlayerPawn` 0)))
  (`KismetSystemLibrary.Delay` 1.2)
  (`|ExecutionSequence`
    (:`then_0`
      (for _ (range 11)
        (`GameplayStatics.SpawnEmitterAttached` "/Game/Asset/Animation/Spark/Reward_part.Reward_part" _skeletalmesh _returnvalue (`SceneComponent.GetSocketLocation` _skeletalmesh _returnvalue) (struct) (100.0 100.0 100.0) "KeepWorldPosition" false))
      (`SkeletalMeshComponent.PlayAnimation` (`self.SkeletalMesh`) "/Game/Asset/Animation/Spark/Exposion_Shrink_Anim.Exposion_Shrink_Anim" false)
      (bind (_direction _move) (`Timeline|Timeline_0`)
        (:`Update`
          (`SceneComponent.K2_SetWorldLocation` (`self.DefaultSceneRoot`) (+ (* (`SceneComponent.K2_GetComponentLocation` (`self.DefaultSceneRoot`)) (- 1.0 _move)) (* (`self.K2_GetActorLocation` _asbp_player_character) _move)) false false))
        (:`Finished`
          (`self.K2_DestroyActor`))))
    (:`then_1`
      (`|SpawnActorFromClass` "Vacuum_C" (`SceneComponent.K2_GetComponentToWorld` (`self.DefaultSceneRoot`)) "Undefined" "OverrideRootScale" null null))))

(fn `UserConstructionScript`)