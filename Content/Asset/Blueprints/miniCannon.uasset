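; Mini cannon Blueprint that continuously turns its Cannon component to face the player pawn.
; Each Tick it builds a rotation from the direction between the cannon and player 0, offsetting roll and yaw by -90 degrees.
; RInterpTo smooths the turn before it is applied as world rotation.
; The file contains no firing logic.
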(event `self.ReceiveTick`
  (params (DeltaSeconds :type "Float (single-precision)"))
  (`SceneComponent.K2_SetWorldRotation` (`self.Cannon`) (`KismetMathLibrary.RInterpTo` (`SceneComponent.K2_GetComponentRotation` (`self.Cannon`)) (`KismetMathLibrary.MakeRotator` (- (.roll (`KismetMathLibrary.Conv_VectorToRotator` (- (`self.K2_GetActorLocation` (`GameplayStatics.GetPlayerPawn` 0)) (`SceneComponent.K2_GetComponentLocation` (`self.Cannon`))))) 90.0) (.pitch (`KismetMathLibrary.Conv_VectorToRotator` (- (`self.K2_GetActorLocation` (`GameplayStatics.GetPlayerPawn` 0)) (`SceneComponent.K2_GetComponentLocation` (`self.Cannon`))))) (- (.yaw (`KismetMathLibrary.Conv_VectorToRotator` (- (`self.K2_GetActorLocation` (`GameplayStatics.GetPlayerPawn` 0)) (`SceneComponent.K2_GetComponentLocation` (`self.Cannon`))))) 90.0)) DeltaSeconds 10.0) false false))

(fn `UserConstructionScript`)